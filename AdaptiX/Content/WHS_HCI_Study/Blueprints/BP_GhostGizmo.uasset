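; Ghost gizmo for a VR Jaco robot-arm study, previewing gripper motion along a chosen adaptive axis.
; Each tick it integrates the axis delta over segments to draw beams with one or two arrows per direction, with a separate arc for gripper-only motion.
; Single-arrow mode also moves the pawn's GripperMover, to which GhostJaco connects.
; Realtime mode uses cosine similarity to suppress Wizard suggestions close to the current axis.
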(event EventBeginPlay
  ;[1 1 1] Basic setup
  (CallFunction|SetPlayerPawn)
  (CallFunction|SetArrowMaterial)
  (CallFunction|SetJaco))

(event EventTick
  (params (DeltaSeconds :type Float%20%28single-precision%29))
  (if (and (not (Variables|Default|GetResetting)) (!= (Variables|Default|GetJaco) 0))
    _
    (else
      _))
  (bind _returnvalue (Actor|GetActorOfClass "/Game/Blueprints/BP_JacoArm/GhostJaco.GhostJaco_C"))
  (Default|ConnecttoMotionController _returnvalue (Variables|/Game/WHS_HCI_Study/Blueprints/BP_WHS_VR_Pawn.BP_WHS_VR_Pawn_C|GetGripperMover (Variables|Default|GetPlayerPawn)) false false false)
  ;[1 1 1] Setup for creating gizmos
  (CallFunction|SetChosenAxisDelta 1)
  (Utilities|ResetBeams
    (:Completed
      (|Hidegizmos,ifadaptiveaxisisempty)
      (switch Utilities|FlowControl|Switch|SwitchonVisualisationType (Variables|Default|GetVisualisation%20Type)
        (:NewEnumerator0
          (|GizmoVisualisationwith1Arrow))
        (:NewEnumerator1
          (Utilities|GizmoVisualisationwith2Arrows))))))

(event EventOnReset
  (Variables|Default|SetResetting true)
  (Utilities|FlowControl|Delay 0.1)
  (Variables|Default|SetResetting false)
  ;[1 1 1] Basic setup
  (CallFunction|SetPlayerPawn)
  (CallFunction|SetArrowMaterial)
  (CallFunction|SetJaco))

(fn ConstructionScript)

(fn FollowPlayer
  (Transformation|SetWorldTransform (Variables|Default|GetDefaultSceneRoot) (Transformation|GetWorldTransform (Variables|/Game/WHS_HCI_Study/Blueprints/BP_WHS_VR_Pawn.BP_WHS_VR_Pawn_C|GetGripperMover (Variables|Default|GetPlayerPawn))) false false))

(fn SetPlayerPawn
  (bind _asbp_whs_vr_pawn (Utilities|Casting|CastToBP_WHS_VR_Pawn (Game|Player|GetPlayerPawn 0))
    (:then
      (bind _output_get (Variables|Default|SetPlayerPawn _asbp_whs_vr_pawn))
      (Transformation|AttachComponentToComponent (Variables|/Game/WHS_HCI_Study/Blueprints/BP_WHS_VR_Pawn.BP_WHS_VR_Pawn_C|GetGripperMover _output_get) "None" "SnapToTarget" "SnapToTarget" "SnapToTarget" true))
    (:CastFailed
      (Development|PrintString "Player not VR Pawn"))))

(fn UpdateLinesandArrows(DoubleArrows)
  (params (Arrow%201 :type Static%20Mesh%20Component%20Object%20Reference) (Arrow%202 :type Static%20Mesh%20Component%20Object%20Reference) (Beam :type Particle%20System%20Component%20Object%20Reference) (Reverse :type Boolean))
  (if Reverse
    (LocalVariables|SetDirectional%20Multiplier -1)
    (else
      (LocalVariables|SetDirectional%20Multiplier 1)))
  ;[1 1 1] Reset gripper center and gripper state and move them to their starting transforms calling the advancement function
  (CallFunction|SetChosenAxisDelta (LocalVariables|GetDirectional%20Multiplier))
  (Transformation|SetWorldTransform (Variables|Default|GetNextGripperCenter) (Transformation|GetWorldTransform (Variables|Default|GetDefaultSceneRoot)) false false)
  (Variables|Default|SetNextGripperState (- 1.0 (Variables|/Game/Blueprints/BP_JacoArm/Jaco.Jaco_C|GetFinger1State (Variables|Default|GetJaco))))
  (CallFunction|AdvanceGripperCentersandStates)
  (Variables|Default|SetPrevLineTangent (Math|Vector|Normalize (.location (Variables|Default|GetChosenAxisDelta))))
  (bind _index (Utilities|FlowControl|ForLoopwithBreak 0 (Variables|Default|GetGizmoSegmentCount))
    (:LoopBody
      (CallFunction|AdvanceGripperCentersandStates)
      (CallFunction|CreateGizmoLinesOffset _index Beam))
    (:Completed
      (CallFunction|PositionDoubleArrows Arrow%201 Arrow%202 (LocalVariables|GetDirectional%20Multiplier)))))

(fn SetArrowMaterial
  (bind _forwardbeam (Variables|Default|GetForwardBeam))
  (bind _adaptiveaxisindex_offset (Variables|Default|GetAdaptiveAxisIndex_offset))
  (Rendering|Material|SetMaterial (Variables|Default|GetForwardArrow1) 0 (Variables|Default|GetArrowMaterial))
  (if (and (== (|(a%2) (Math|Conversions|ToFloat(Integer) _adaptiveaxisindex_offset)) 0.0) (!= _adaptiveaxisindex_offset 6))
    (Effects|Components|ParticleSystem|SetColorParameter _forwardbeam "BeamColor" "(R=0.000000,G=1.000000,B=1.000000,A=1.000000)")
    (else
      (Effects|Components|ParticleSystem|SetColorParameter _forwardbeam "BeamColor" "(R=0.000000,G=0.000000,B=0.330000,A=1.000000)"))))

(fn DrawGizmoLineOffset
  (params (BeamEmitterIndex :type Integer) (Index :type Integer) (Oriented%20Prev%20Gripper%20State :type Float%20%28single-precision%29) (Oriented%20Current%20Gripper%20State :type Float%20%28single-precision%29) (Prev%20Line%20Tangent :type Vector) (Current%20Line%20Tangent :type Vector) (Beam :type Particle%20System%20Component%20Object%20Reference))
  (bind _arrowoffset (Variables|Default|GetArrowOffset))
  (bind _prevgrippercenter (Variables|Default|GetPrevGripperCenter))
  (bind _currentgrippercenter (Variables|Default|GetCurrentGripperCenter))
  (bind _returnvalue (Transformation|GetWorldTransform _prevgrippercenter))
  (bind _returnvalue_2 (Transformation|GetWorldTransform _currentgrippercenter))
  (Class|ParticleSystemComponent|SetBeamSourcePoint Beam BeamEmitterIndex (+ (.location _returnvalue) (Math|Vector|RotateVector (Math|Vector|MakeVector (.x _arrowoffset) (* Oriented%20Prev%20Gripper%20State (.y _arrowoffset)) (.z _arrowoffset)) (.rotation _returnvalue))) Index)
  (Class|ParticleSystemComponent|SetBeamSourceTangent Beam BeamEmitterIndex Prev%20Line%20Tangent Index)
  (Class|ParticleSystemComponent|SetBeamTargetPoint Beam BeamEmitterIndex (+ (.location _returnvalue_2) (Math|Vector|RotateVector (Math|Vector|MakeVector (.x _arrowoffset) (* Oriented%20Current%20Gripper%20State (.y _arrowoffset)) (.z _arrowoffset)) (.rotation _returnvalue_2))) Index)
  (Class|ParticleSystemComponent|SetBeamTargetTangent Beam BeamEmitterIndex Current%20Line%20Tangent Index))

(fn PositionDoubleArrows
  (params (Arrow%201 :type Static%20Mesh%20Component%20Object%20Reference) (Arrow%202 :type Static%20Mesh%20Component%20Object%20Reference) (Directional%20Multiplier :type Integer))
  (bind _arrowoffset (Variables|Default|GetArrowOffset))
  (bind _prevgripperstate (Variables|Default|GetPrevGripperState))
  (bind _currentgripperstate (Variables|Default|GetCurrentGripperState))
  (bind _returnvalue (* (.y _arrowoffset) _currentgripperstate))
  (bind _returnvalue_2 (* _prevgripperstate (.y _arrowoffset)))
  (CallFunction|SetArrowTransform Arrow%201 (Math|Vector|MakeVector (.x _arrowoffset) _returnvalue_2 (.z _arrowoffset)) (Math|Vector|MakeVector (.x _arrowoffset) _returnvalue (.z _arrowoffset)) Directional%20Multiplier)
  (CallFunction|SetArrowTransform Arrow%202 (Math|Vector|MakeVector (.x _arrowoffset) (* -1 _returnvalue_2) (.z _arrowoffset)) (Math|Vector|MakeVector (.x _arrowoffset) (* -1 _returnvalue) (.z _arrowoffset)) Directional%20Multiplier))

(fn SetJaco
  (bind _returnvalue (Actor|GetActorOfClass "/Game/Blueprints/BP_JacoArm/Jaco.Jaco_C"))
  (Variables|Default|SetJaco _returnvalue))

(fn SetChosenAxisDelta
  (params (Directional%20Multiplier :type Integer))
  (bind _playerpawn (Variables|Default|GetPlayerPawn))
  (bind _playerpawn_2 (Variables|Default|GetPlayerPawn))
  (bind _playerpawn_3 (Variables|Default|GetPlayerPawn))
  (bind _playerpawn_4 (Variables|Default|GetPlayerPawn))
  (bind _adaptiveaxisindex_offset (Variables|Default|GetAdaptiveAxisIndex_offset))
  (bind _playerpawn_5 (Variables|Default|GetPlayerPawn))
  (bind _playerpawn_6 (Variables|Default|GetPlayerPawn))
  (bind _wizard (Variables|/Game/WHS_HCI_Study/Blueprints/BP_WHS_VR_Pawn.BP_WHS_VR_Pawn_C|GetWizard _playerpawn))
  (bind _adaptiveset (Variables|/Game/WHS_HCI_Study/Blueprints/BP_WHS_VR_Pawn.BP_WHS_VR_Pawn_C|GetAdaptiveSet _playerpawn_4))
  (bind _adaptiveset_2 (Variables|/Game/WHS_HCI_Study/Blueprints/BP_WHS_VR_Pawn.BP_WHS_VR_Pawn_C|GetAdaptiveSet _playerpawn_6))
  (bind _wizard_2 (Variables|/Game/WHS_HCI_Study/Blueprints/BP_WHS_VR_Pawn.BP_WHS_VR_Pawn_C|GetWizard _playerpawn_3))
  (bind _direction_0 (Utilities|Struct|BreakAdaptiveSet _adaptiveset_2))
  (bind (_direction_0_2 _direction_1 _direction_2 _direction_3 _direction_4 _direction_5 _direction_6) (Utilities|Struct|BreakAdaptiveSet _adaptiveset))
  (bind _axis_1 (Default|CalculateAxis1 _wizard))
  (bind _axis_1_2 (Default|CalculateAxis1 _wizard_2))
  (bind (_location _rotation _gripper) (Utilities|Struct|BreakAdaptiveAxis _direction_0))
  (bind _array (Utilities|Array|MakeArray _direction_0_2 _direction_1 _direction_2 _direction_3 _direction_4 _direction_5 _direction_6 ""))
  (bind _output (Utilities|Array|Get(acopy) _array _adaptiveaxisindex_offset))
  (if (Math|Boolean|ANDBoolean (Variables|/Game/WHS_HCI_Study/Blueprints/BP_WHS_VR_Pawn.BP_WHS_VR_Pawn_C|GetRealtimeVisu _playerpawn_5) (Variables|/Game/WHS_HCI_Study/Blueprints/BP_AxisWizard.BP_AxisWizard_C|GetEnabled (Variables|/Game/WHS_HCI_Study/Blueprints/BP_WHS_VR_Pawn.BP_WHS_VR_Pawn_C|GetWizard _playerpawn_5)) (== (Variables|Default|GetAdaptiveAxisIndex_offset) 1))
    (if (and (not (Math|Float|NearlyEqual(Float) (|(((((((a*b)+(c*d))+(e*f))+(g*h))+(i*j))+(k*l))+(m*n)) (.x _location) (.x (.location _axis_1_2)) (.y _location) (.y (.location _axis_1_2)) (.z _location) (.z (.location _axis_1_2)) (.roll _rotation) (.roll (.rotation _axis_1_2)) (.pitch _rotation) (.pitch (.rotation _axis_1_2)) (.yaw _rotation) (.yaw (.rotation _axis_1_2)) _gripper (.gripper _axis_1_2)) (* (Math|Float|Sqrt (|((((((a²+b²)+c²)+d²)+e²)+f²)+g²) (.x _location) (.y _location) (.z _location) (.roll _rotation) (.pitch _rotation) (.yaw _rotation) _gripper)) (Math|Float|Sqrt (|((((((a²+b²)+c²)+d²)+e²)+f²)+g²) (.x (.location _axis_1_2)) (.y (.location _axis_1_2)) (.z (.location _axis_1_2)) (.roll (.rotation _axis_1_2)) (.pitch (.rotation _axis_1_2)) (.yaw (.rotation _axis_1_2)) (.gripper _axis_1_2)))) (Variables|Default|GetRealtimeThreshold))) (not (Variables|/Game/WHS_HCI_Study/Blueprints/BP_WHS_VR_Pawn.BP_WHS_VR_Pawn_C|GetStopInput _playerpawn_5)))
      (bind _returnvalue (Actor|GetActorOfClass "/Game/Blueprints/BP_JacoArm/GhostJaco.GhostJaco_C"))
      (Rendering|SetActorHiddenInGame _returnvalue true)
      (LocalVariables|SetAxisDeltaLocation "0, 0, 0")
      (LocalVariables|SetAxisDeltaRotation "0, 0, 0")
      (LocalVariables|SetAxisDeltaGripper 0.0)
      (else
        (bind _returnvalue_2 (Actor|GetActorOfClass "/Game/Blueprints/BP_JacoArm/GhostJaco.GhostJaco_C"))
        (Rendering|SetActorHiddenInGame _returnvalue_2 false)
        (LocalVariables|SetAxisDeltaLocation (.location _axis_1))
        (LocalVariables|SetAxisDeltaRotation (.rotation _axis_1))
        (LocalVariables|SetAxisDeltaGripper (.gripper _axis_1))))
    (else
      (LocalVariables|SetAxisDeltaLocation (.location _output))
      (LocalVariables|SetAxisDeltaRotation (.rotation _output))
      (LocalVariables|SetAxisDeltaGripper (.gripper _output))))
  (Variables|Default|SetChosenAxisDelta (Utilities|Struct|MakeAdaptiveAxis (* (* (LocalVariables|GetAxisDeltaLocation) (Variables|/Game/WHS_HCI_Study/Blueprints/BP_WHS_VR_Pawn.BP_WHS_VR_Pawn_C|GetVel_Trans _playerpawn_2)) Directional%20Multiplier) (* (* (LocalVariables|GetAxisDeltaRotation) (Variables|/Game/WHS_HCI_Study/Blueprints/BP_WHS_VR_Pawn.BP_WHS_VR_Pawn_C|GetVel_Rot _playerpawn_2)) Directional%20Multiplier) (* Directional%20Multiplier (* (Math|Float|Clamp(Float) (LocalVariables|GetAxisDeltaGripper) -1.0) (Variables|/Game/Blueprints/BP_JacoArm/Jaco.Jaco_C|GetFingerVelocity (Variables|Default|GetJaco))))))
  (return))

(fn AdvanceGripperCentersandStates
  (bind _chosenaxisdelta (Variables|Default|GetChosenAxisDelta))
  ;[1 1 1] Advance gripper center points
  (Transformation|SetWorldTransform (Variables|Default|GetPrevGripperCenter) (Transformation|GetWorldTransform (Variables|Default|GetCurrentGripperCenter)) false false)
  (Transformation|SetWorldTransform (Variables|Default|GetCurrentGripperCenter) (Transformation|GetWorldTransform (Variables|Default|GetNextGripperCenter)) false false)
  (Class|SceneComponent|AddLocalTransform (Variables|Default|GetNextGripperCenter) (Math|Transform|MakeTransform (.location _chosenaxisdelta) (.rotation _chosenaxisdelta) "1,1,1") false false)
  ;[1 1 1] Advance gripper state (= gripper spacing)
  (Variables|Default|SetPrevGripperState (Variables|Default|GetCurrentGripperState))
  (Variables|Default|SetCurrentGripperState (Variables|Default|GetNextGripperState))
  (Variables|Default|SetNextGripperState (Math|Float|Clamp(Float) (- (Variables|Default|GetNextGripperState) (.gripper (Variables|Default|GetChosenAxisDelta))) (Variables|Default|GetMinimal%20Gripper%20State))))

(fn SetArrowTransform
  (params (Arrow%20Component :type Scene%20Component%20Object%20Reference) (Last%20Gripper%20Offset :type Vector) (Current%20Gripper%20Offset :type Vector) (Directional%20Multiplier :type Integer))
  (bind _use_directional_arrows (Variables|Default|GetUse_Directional_Arrows))
  (bind _prevgrippercenter (Variables|Default|GetPrevGripperCenter))
  (bind _currentgrippercenter (Variables|Default|GetCurrentGripperCenter))
  (bind _returnvalue (Transformation|GetWorldTransform _currentgrippercenter))
  (bind _returnvalue_2 (Transformation|GetWorldTransform _prevgrippercenter))
  (bind _returnvalue_3 (select _use_directional_arrows Directional%20Multiplier 1))
  (bind _returnvalue_4 (* _returnvalue_3 0.03))
  (bind _returnvalue_5 (Math|Vector|RotateVector Current%20Gripper%20Offset (.rotation _returnvalue)))
  (bind _returnvalue_6 (+ _returnvalue_5 (.location _returnvalue)))
  (Transformation|SetWorldTransform Arrow%20Component (Math|Transform|MakeTransform _returnvalue_6 (Math|Rotator|MakeRotfromZ (- _returnvalue_6 (+ (.location _returnvalue_2) (Math|Vector|RotateVector Last%20Gripper%20Offset (.rotation _returnvalue_2))))) (Math|Vector|MakeVector _returnvalue_4 _returnvalue_4 _returnvalue_4)) false false))

(fn CreateGizmoLinesOffset
  (params (Index :type Integer) (Beam :type Particle%20System%20Component%20Object%20Reference))
  (bind _prevgrippercenter (Variables|Default|GetPrevGripperCenter))
  (bind _nextgrippercenter (Variables|Default|GetNextGripperCenter))
  (bind _currentgripperstate (Variables|Default|GetCurrentGripperState))
  (bind _prevgripperstate (Variables|Default|GetPrevGripperState))
  (bind _returnvalue (Transformation|GetWorldLocation _prevgrippercenter))
  (bind _returnvalue_2 (Transformation|GetWorldLocation _nextgrippercenter))
  (bind _returnvalue_3 (- _returnvalue_2 _returnvalue))
  ;[1 1 1] Draw line on one side...
  (CallFunction|DrawGizmoLineOffset 0 Index _prevgripperstate _currentgripperstate (Variables|Default|GetPrevLineTangent) _returnvalue_3 Beam)
  ;[1 1 1] ... and on the other side
  (CallFunction|DrawGizmoLineOffset 1 Index (* -1 _prevgripperstate) (* -1 _currentgripperstate) (Variables|Default|GetPrevLineTangent) _returnvalue_3 Beam)
  (Variables|Default|SetPrevLineTangent _returnvalue_3))

(fn UpdateGizmosandArrowsGripperOnly
  (bind _gizmosegmentcount (Variables|Default|GetGizmoSegmentCount))
  (Rendering|SetVisibility (Variables|Default|GetBackwardBeam) false false)
  (CallFunction|AdvanceGripperLocation 0 _gizmosegmentcount)
  (for _index (range 0 _gizmosegmentcount)
    (CallFunction|AdvanceGripperLocation _index _gizmosegmentcount)
    (if (== _index 0)
      (CallFunction|SetGripperArrowTransform))
    (CallFunction|CreateGripperGizmoLines _index))
  (CallFunction|SetGripperArrowTransform))

(fn AdvanceGripperLocation
  (params (CurrentIndex :type Integer) (LastIndex :type Integer))
  (bind _defaultsceneroot (Variables|Default|GetDefaultSceneRoot))
  (Variables|Default|SetPrevGripperLocation (Variables|Default|GetCurrentGripperLocation))
  (Variables|Default|SetCurrentGripperLocation (+ (Transformation|GetWorldLocation (Variables|Default|GetDefaultSceneRoot)) (Math|Vector|RotateVectorAroundAxis (* (Math|Vector|GetForwardVector _defaultsceneroot) (.y (Variables|Default|GetArrowOffset))) (Math|Float|Lerp (Variables|Default|GetGripperArrowSpread) (* (Variables|Default|GetMinimal%20Gripper%20State) (Variables|Default|GetGripperArrowSpread)) (/ (Math|Conversions|ToFloat(Integer) CurrentIndex) (Math|Conversions|ToFloat(Integer) LastIndex))) (Math|Vector|GetUpVector _defaultsceneroot)))))

(fn CreateGripperGizmoLines
  (params (Index :type Integer))
  (bind _defaultsceneroot (Variables|Default|GetDefaultSceneRoot))
  (bind _returnvalue (Math|Vector|GetRightVector _defaultsceneroot))
  (bind _returnvalue_2 (Transformation|GetWorldLocation _defaultsceneroot))
  (bind _returnvalue_3 (Class|KismetMathLibrary|MakePlanefromPointandNormal _returnvalue_2 _returnvalue))
  (Class|ParticleSystemComponent|SetBeamSourcePoint (Variables|Default|GetForwardBeam) 0 (Variables|Default|GetPrevGripperLocation) Index)
  (Class|ParticleSystemComponent|SetBeamTargetPoint (Variables|Default|GetForwardBeam) 0 (Variables|Default|GetCurrentGripperLocation) Index)
  (Class|ParticleSystemComponent|SetBeamSourcePoint (Variables|Default|GetForwardBeam) 1 (Class|KismetMathLibrary|VectorMirrorbyPlane (Variables|Default|GetPrevGripperLocation) _returnvalue_3) Index)
  (Class|ParticleSystemComponent|SetBeamTargetPoint (Variables|Default|GetForwardBeam) 1 (Class|KismetMathLibrary|VectorMirrorbyPlane (Variables|Default|GetCurrentGripperLocation) _returnvalue_3) Index))

(fn SetGripperArrowTransform
  (bind _defaultsceneroot (Variables|Default|GetDefaultSceneRoot))
  (bind _prevgripperlocation (Variables|Default|GetPrevGripperLocation))
  (bind _currentgripperlocation (Variables|Default|GetCurrentGripperLocation))
  (bind _returnvalue (Math|Vector|GetRightVector _defaultsceneroot))
  (bind _returnvalue_2 (Transformation|GetWorldLocation _defaultsceneroot))
  (bind _returnvalue_3 (Class|KismetMathLibrary|MakePlanefromPointandNormal _returnvalue_2 _returnvalue))
  (bind _returnvalue_4 (Class|KismetMathLibrary|VectorMirrorbyPlane _currentgripperlocation _returnvalue_3))
  (Transformation|SetWorldTransform (Variables|Default|GetForwardArrow1) (Math|Transform|MakeTransform _currentgripperlocation (Math|Rotator|MakeRotfromZ (- _currentgripperlocation _prevgripperlocation)) "0.030000,0.030000,0.030000") false false)
  (Transformation|SetWorldTransform (Variables|Default|GetForwardArrow2) (Math|Transform|MakeTransform _returnvalue_4 (Math|Rotator|MakeRotfromZ (- _returnvalue_4 (Class|KismetMathLibrary|VectorMirrorbyPlane _prevgripperlocation _returnvalue_3))) "0.030000,0.030000,0.030000") false false))

(fn UpdateLinesandArrows(SingleArrow)
  (params (Arrow :type Static%20Mesh%20Component%20Object%20Reference) (Beam :type Particle%20System%20Component%20Object%20Reference) (Reverse :type Boolean))
  (bind _forwardarrow1 (Variables|Default|GetForwardArrow1))
  (bind _returnvalue (Transformation|GetWorldTransform _forwardarrow1))
  (if Reverse
    (LocalVariables|SetDirectional%20Multiplier -1)
    (else
      (LocalVariables|SetDirectional%20Multiplier 1)))
  ;[1 1 1] Reset gripper center and gripper state and move them to their starting transforms calling the advancement function
  (CallFunction|SetChosenAxisDelta (LocalVariables|GetDirectional%20Multiplier))
  (Transformation|SetWorldTransform (Variables|Default|GetNextGripperCenter) (Transformation|GetWorldTransform (Variables|Default|GetDefaultSceneRoot)) false false)
  (Variables|Default|SetNextGripperState (- 1.0 (Variables|/Game/Blueprints/BP_JacoArm/Jaco.Jaco_C|GetFinger1State (Variables|Default|GetJaco))))
  (CallFunction|AdvanceGripperCentersandStates)
  (Variables|Default|SetPrevLineTangent (Math|Vector|Normalize (.location (Variables|Default|GetChosenAxisDelta))))
  (bind _index (Utilities|FlowControl|ForLoopwithBreak 0 (Variables|Default|GetGizmoSegmentCount))
    (:LoopBody
      (CallFunction|AdvanceGripperCentersandStates)
      (Utilities|CreateGizmoLine _index Beam))
    (:Completed
      (Utilities|PositionSingleArrow Arrow (LocalVariables|GetDirectional%20Multiplier))
      (if (== Arrow _forwardarrow1)
        (Transformation|SetWorldLocationAndRotation (Variables|/Game/WHS_HCI_Study/Blueprints/BP_WHS_VR_Pawn.BP_WHS_VR_Pawn_C|GetGripperMover (Variables|Default|GetPlayerPawn)) (.location _returnvalue) (.rotation _returnvalue) false false)))))