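; BP_AxisWizard generates adaptive control axes for the Jaco robot arm in a VR study, steering the gripper toward pick-and-place targets.
; Tick targets the nearest box spawn volume, or the drop target while grasping, and recomputes axes once inputs go idle.
; Axis 1 blends hover-aware translation, rotation and gripper into one normalized vector.
; Perpendicular, direct-translation, rotation-only and gripper-only axes complete the set passed to the VR pawn.
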(event `self.K2_OnReset`
  (set `self.Resetting` true)
  (`KismetSystemLibrary.Delay` 0.1)
  (set `self.Resetting` false)
  (`self.SetPlayerPawn` :!label _label)
  (`self.SetJaco`)
  (bind _asbp_gm_study (cast `/Game/WHS_HCI_Study/Blueprints/BP_GM_Study` (`GameplayStatics.GetGameMode`)))
  (set `self.GM_Study` _asbp_gm_study))

(event `self.ReceiveBeginPlay`
  (goto _label))

(event `self.ReceiveTick`
  (params (DeltaSeconds :type "Float (single-precision)"))
  (if (and (`self.Enabled`) (not (`self.Resetting`)))
    ;[1 1 1] Find Closest Spawn Area and check if the Gripper is moving.
    (`self.FindClosestSpawnArea`)
    (if (and (<= (`KismetMathLibrary.Abs` (`self.AdaptiveInputAxis0`)) 0.2) (<= (`KismetMathLibrary.Abs` (`self.AdaptiveInputAxis1`)) 0.2))
      (if (not (and (`self.Mode Switched`) (!= (`/Game/WHS_HCI_Study/Blueprints/BP_GM_Study.Mode Switches` (`self.GM_Study`)) -1)))
        (set `self.Mode Switched` true)
        (`self.DoModeSwitch`))
      (else
        (set `self.Mode Switched` false)))))

(fn `Calculate Axis 1`
  (returns (`Axis 1` :type "/Game/Structs/AdaptiveAxis Structure"))
  (bind (_new_axis_1_translation _new_axis_1_rotation) (`self.Calculate Axis 1 Rotation` (`self.Calculate Axis 1 Translation`)))
  (bind (_new_axis_1_translation_2 _new_axis_1_rotation_2 _new_axis_1_gripper) (`self.Calculate Axis 1 Gripper` _new_axis_1_translation _new_axis_1_rotation))
  (bind _normalized_axis (`self.NormalizeAxis` (make `/Game/Structs/AdaptiveAxis` _new_axis_1_translation_2 _new_axis_1_rotation_2 _new_axis_1_gripper)))
  (return _normalized_axis))

(fn `Calculate Axis 1 Gripper`
  (params (`Axis 1 Translation` :type "Vector Structure") (`Axis 1 Rotation` :type "Rotator Structure"))
  (returns (`New Axis 1 Translation` :type "Vector Structure") (`New Axis 1 Rotation` :type "Rotator Structure") (`New Axis 1 Gripper` :type "Float (double-precision)"))
  (if (and (`self.IsCloseToCurrentTarget` 15.0) (not (`self.GripperIsClosed`)))
    (if (`self.GripperGraspsObject`)
      (return (* `Axis 1 Translation` -1.0) `Axis 1 Rotation` -1.0)
      (elif (`self.IsCloseToCurrentTarget` 10.0)
        (return (0.0 0.0 0.0) (struct) 1.0)
        (else
          (return `Axis 1 Translation` `Axis 1 Rotation` 1.0))))
    (elif (and (not (`self.GripperIsFullyOpen`)) (not (`self.GripperGraspsObject`)))
      (return `Axis 1 Translation` `Axis 1 Rotation` -1.0)
      (else
        (return `Axis 1 Translation` `Axis 1 Rotation` 0.0)))))

(fn `Calculate Axis 1 Rotation`
  (params (`Axis 1 Translation` :type "Vector Structure"))
  (returns (`New Axis 1 Translation` :type "Vector Structure") (`New Axis 1 Rotation` :type "Rotator Structure"))
  (bind (_returnvalue_roll _returnvalue_pitch _returnvalue_yaw) (`KismetMathLibrary.BreakRotator` (`KismetMathLibrary.MakeRotFromX` `Axis 1 Translation`)))
  (bind _gripper_mover_transform_location (`KismetMathLibrary.BreakTransform` (`self.GetGripperMoverTransform`)))
  (bind _current_target_transform_location (`KismetMathLibrary.BreakTransform` (`self.GetCurrentTargetTransform`)))
  (if (not (`self.TargetIsDirectlyInfront`))
    (if (not (and (not (< (`KismetMathLibrary.Vector_Distance` (`KismetMathLibrary.MakeVector` (.x _current_target_transform_location) (.y _current_target_transform_location)) (`KismetMathLibrary.MakeVector` (.x _gripper_mover_transform_location) (.y _gripper_mover_transform_location))) (`self.Minimal Hover Distance`))) (`self.GripperGraspsObject`) (> (+ (.z _current_target_transform_location) (`self.Hover Height`)) (.z _gripper_mover_transform_location))))
      (return `Axis 1 Translation` (* (`KismetMathLibrary.MakeRotator` (* (.roll (.rotation (`self.GetGripperMoverTransform`))) -1.0) _returnvalue_pitch _returnvalue_yaw) 0.01))
      (else
        _)))
  (return `Axis 1 Translation`))

(fn `Calculate Axis 1 Translation`
  (returns (`Axis 1 Translation` :type "Vector Structure"))
  (locals (`New Translation` :type "Vector Structure"))
  (bind (_gripper_mover_transform_location _gripper_mover_transform_rotation) (`KismetMathLibrary.BreakTransform` (`self.GetGripperMoverTransform`)))
  (bind _gripper_mover_transform_location_2 (`KismetMathLibrary.BreakTransform` (`self.GetGripperMoverTransform`)))
  (bind _current_target_transform_location (`KismetMathLibrary.BreakTransform` (`self.GetCurrentTargetTransform`)))
  (bind _hover_height (`self.Hover Height`))
  (bind _returnvalue (< (`KismetMathLibrary.Vector_Distance` (`KismetMathLibrary.MakeVector` (.x _current_target_transform_location) (.y _current_target_transform_location)) (`KismetMathLibrary.MakeVector` (.x _gripper_mover_transform_location_2) (.y _gripper_mover_transform_location_2))) (`self.Minimal Hover Distance`)))
  (bind _returnvalue_2 (* (`KismetMathLibrary.LessLess_VectorRotator` (`KismetMathLibrary.Normal` (`KismetMathLibrary.SelectVector` (+ (0.0 0.0 0.0) (`KismetMathLibrary.MakeVector` 0.0 0.0 _hover_height)) (- (`KismetMathLibrary.SelectVector` _current_target_transform_location (+ _current_target_transform_location (`KismetMathLibrary.MakeVector` 0.0 0.0 (`self.Hover Height`))) _returnvalue) _gripper_mover_transform_location_2) (and (not _returnvalue) (`self.GripperGraspsObject`) (> (+ _hover_height (.z _current_target_transform_location)) (.z _gripper_mover_transform_location_2))))) _gripper_mover_transform_rotation) (`/Game/WHS_HCI_Study/Blueprints/BP_WHS_VR_Pawn.Vel_Trans` (`self.Player Pawn`))))
  (if (!= (`self.Prev Object Grasped`) (`self.GripperGraspsObject`))
    (set `local.New Translation` (+ _returnvalue_2 (0.0 0.0 1.0)))
    (if (> (.z (.location (`self.GetGripperMoverTransform`))) (`self.Hover Height`))
      (set `self.Prev Object Grasped` (`self.GripperGraspsObject`) :!label _label))
    (else
      (set `local.New Translation` _returnvalue_2)
      (goto _label)))
  (return (`local.New Translation`)))

(fn `Calculate Axis 2`
  (params (`Axis 1` :type "/Game/Structs/AdaptiveAxis Structure"))
  (returns (`Axis 2` :type "/Game/Structs/AdaptiveAxis Structure"))
  (return (make `/Game/Structs/AdaptiveAxis` (`KismetMathLibrary.RotateAngleAxis` `Axis 1_location_18_DE814FB141141771F423A9BE579C8632` 90.0 (0.0 1.0 0.0)) `Axis 1_rotation_19_FFE889E94E9766A894E731A12272FCE9`)))

(fn `Calculate Axis 3`
  (returns (`Axis 3` :type "/Game/Structs/AdaptiveAxis Structure"))
  (bind _normalized_axis (`self.NormalizeAxis` (make `/Game/Structs/AdaptiveAxis` (`self.Calculate Axis 3 Translation`))))
  (return _normalized_axis))

(fn `Calculate Axis 3 Translation`
  (returns (ReturnValue :type "Vector Structure"))
  (bind (_gripper_mover_transform_location _gripper_mover_transform_rotation) (`KismetMathLibrary.BreakTransform` (`self.GetGripperMoverTransform`)))
  (return (`KismetMathLibrary.LessLess_VectorRotator` (`self.GetLookAtTargetNormal`) _gripper_mover_transform_rotation)))

(fn `Calculate Axis 4`
  (returns (`Axis 4` :type "/Game/Structs/AdaptiveAxis Structure"))
  (return (make `/Game/Structs/AdaptiveAxis` (0.0 0.0 0.0) (`self.Calculate Axis 4 Rotation`))))

(fn `Calculate Axis 4 Rotation`
  (returns (`New Axis 4 Rotation` :type "Rotator Structure"))
  (return (* (`self.NormalizeRotatorAsVector` (`KismetMathLibrary.MakeRotFromX` (`self.GetLookAtTargetNormal`))) 3.14)))

(fn `Calculate Axis 5`
  (returns (`Axis 5` :type "/Game/Structs/AdaptiveAxis Structure"))
  (return (make `/Game/Structs/AdaptiveAxis` (0.0 0.0 0.0) (struct) (`KismetMathLibrary.SelectFloat` -1.0 1.0 (`self.GripperGraspsObject`)))))

(fn `Calculate Axis 6`
  (returns (`Axis 6` :type "/Game/Structs/AdaptiveAxis Structure"))
  (return))

(fn `Calculate Axis 7`
  (returns (`Axis 7` :type "/Game/Structs/AdaptiveAxis Structure"))
  (return (make `/Game/Structs/AdaptiveAxis` (0.0 0.0 0.0) (struct) 1.0)))

(fn `FindClosestSpawnArea`
  (bind _gripper_mover_transform_location (`KismetMathLibrary.BreakTransform` (`self.GetGripperMoverTransform`)))
  (set `self.PreviousClosestDistance` 1.1553255867809792e+19)
  (if (`self.GripperGraspsObject`)
    (set `self.ClosestSpawnArea` (`/Game/WHS_HCI_Study/Blueprints/BP_Spawn_Volumes.TargetBoxSpawnVolume` (`self.SpawnVolumes`)))
    (bind _returnvalue (`KismetMathLibrary.Vector_Distance` (`SceneComponent.K2_GetComponentLocation` (`StaticMeshActor.StaticMeshComponent` (`/Game/Blueprints/BP_SpawnAreas/BP_Dep_Mesh_SpawnArea.P_Static Mesh Actor Ref` (stale _array_element)))) _gripper_mover_transform_location))
    (set `self.PreviousClosestDistance` _returnvalue :!label _label)
    (else
      (for _array_element (`/Game/WHS_HCI_Study/Blueprints/BP_Spawn_Volumes.BoxSpawnVolumes` (`self.SpawnVolumes`))
        (if (< _returnvalue (`self.PreviousClosestDistance`))
          (set `self.ClosestSpawnArea` _array_element)
          (goto _label))))))

(fn `GetCurrentTarget`
  (returns (`Current Target` :type "StaticMeshComponent Object Reference"))
  (return (`StaticMeshActor.StaticMeshComponent` (`/Game/Blueprints/BP_SpawnAreas/BP_Dep_Mesh_SpawnArea.P_Static Mesh Actor Ref` (`self.ClosestSpawnArea`)))))

(fn `GetCurrentTargetTransform`
  (returns (`Current Target Transform` :type "Transform Structure"))
  (return (`SceneComponent.K2_GetComponentToWorld` (`self.GetCurrentTarget`))))

(fn `GetGripperMover`
  (returns (GripperMover :type "StaticMeshComponent Object Reference"))
  (return (`/Game/WHS_HCI_Study/Blueprints/BP_WHS_VR_Pawn.GripperMover` (`self.Player Pawn`))))

(fn `GetGripperMoverTransform`
  (returns (`Gripper Mover Transform` :type "Transform Structure"))
  (return (`SceneComponent.K2_GetComponentToWorld` (`self.GetGripperMover`))))

(fn `GetLookAtTargetNormal`
  (returns (`Target Normal` :type "Vector Structure"))
  (bind _gripper_mover_transform_location (`KismetMathLibrary.BreakTransform` (`self.GetGripperMoverTransform`)))
  (bind _current_target_transform_location (`KismetMathLibrary.BreakTransform` (`self.GetCurrentTargetTransform`)))
  (return (`KismetMathLibrary.Normal` (- _current_target_transform_location _gripper_mover_transform_location))))

(fn `GripperGraspsObject`
  (returns (ReturnValue :type Boolean))
  (bind _graspedobject (`/Game/Blueprints/BP_JacoArm/Jaco.GraspedObject` (`self.Jaco`)))
  (if (`KismetSystemLibrary.IsValid` _graspedobject)
    (return (!= (`self.GetComponentByClass` _graspedobject "/Script/Engine.StaticMeshComponent") null))
    (else
      (return false))))

(fn `GripperIsClosed`
  (returns (ReturnValue :type Boolean))
  (return (>= (`/Game/Blueprints/BP_JacoArm/Jaco.Finger1State` (`self.Jaco`)) 0.75)))

(fn `GripperIsFullyOpen`
  (returns (ReturnValue :type Boolean))
  (return (<= (`/Game/Blueprints/BP_JacoArm/Jaco.Finger1State` (`self.Jaco`)) 0.0)))

(fn `IsCloseToCurrentTarget`
  (params (Distance :type "Float (double-precision)" :default 15.0))
  (returns (ReturnValue :type Boolean))
  (bind _gripper_mover_transform_location (`KismetMathLibrary.BreakTransform` (`self.GetGripperMoverTransform`)))
  (bind _current_target_transform_location (`KismetMathLibrary.BreakTransform` (`self.GetCurrentTargetTransform`)))
  (return (< (`KismetMathLibrary.Vector_Distance` _gripper_mover_transform_location _current_target_transform_location) Distance)))

(fn `NormalizeAxis`
  (params (Axis :type "/Game/Structs/AdaptiveAxis Structure"))
  (returns (`Normalized Axis` :type "/Game/Structs/AdaptiveAxis Structure"))
  (bind _returnvalue (`KismetMathLibrary.Sqrt` (+ (`KismetMathLibrary.MultiplyMultiply_FloatFloat` (.x (break `/Game/Structs/AdaptiveAxis` Axis)) 2.0) (`KismetMathLibrary.MultiplyMultiply_FloatFloat` (.y (break `/Game/Structs/AdaptiveAxis` Axis)) 2.0) (`KismetMathLibrary.MultiplyMultiply_FloatFloat` (.z (break `/Game/Structs/AdaptiveAxis` Axis)) 2.0) (`KismetMathLibrary.MultiplyMultiply_FloatFloat` (.roll (`.rotation_19_FFE889E94E9766A894E731A12272FCE9` (break `/Game/Structs/AdaptiveAxis` Axis))) 2.0) (`KismetMathLibrary.MultiplyMultiply_FloatFloat` (.pitch (`.rotation_19_FFE889E94E9766A894E731A12272FCE9` (break `/Game/Structs/AdaptiveAxis` Axis))) 2.0) (`KismetMathLibrary.MultiplyMultiply_FloatFloat` (.yaw (`.rotation_19_FFE889E94E9766A894E731A12272FCE9` (break `/Game/Structs/AdaptiveAxis` Axis))) 2.0) (`KismetMathLibrary.MultiplyMultiply_FloatFloat` Axis_gripper_20_4B3264B549C0E645475061BAF82933A2 2.0))))
  (return (make `/Game/Structs/AdaptiveAxis` (`KismetMathLibrary.MakeVector` (/ (.x (break `/Game/Structs/AdaptiveAxis` Axis)) _returnvalue) (/ (.y (break `/Game/Structs/AdaptiveAxis` Axis)) _returnvalue) (/ (.z (break `/Game/Structs/AdaptiveAxis` Axis)) _returnvalue)) (`KismetMathLibrary.MakeRotator` (/ (.roll (`.rotation_19_FFE889E94E9766A894E731A12272FCE9` (break `/Game/Structs/AdaptiveAxis` Axis))) _returnvalue) (/ (.pitch (`.rotation_19_FFE889E94E9766A894E731A12272FCE9` (break `/Game/Structs/AdaptiveAxis` Axis))) _returnvalue) (/ (.yaw (`.rotation_19_FFE889E94E9766A894E731A12272FCE9` (break `/Game/Structs/AdaptiveAxis` Axis))) _returnvalue)) (/ Axis_gripper_20_4B3264B549C0E645475061BAF82933A2 _returnvalue))))

(fn `NormalizeRotatorAsVector`
  (params (InRot :type "Rotator Structure"))
  (returns (ReturnValue :type "Rotator Structure"))
  (bind (_returnvalue_x _returnvalue_y _returnvalue_z) (`KismetMathLibrary.BreakVector` (`KismetMathLibrary.Normal` (`KismetMathLibrary.MakeVector` (.roll InRot) (.pitch InRot) (.yaw InRot)))))
  (return (`KismetMathLibrary.MakeRotator` _returnvalue_x _returnvalue_y _returnvalue_z)))

(fn `Print Adaptive Axis`
  (params (AdaptiveAxis :type "/Game/Structs/AdaptiveAxis Structure (by ref)"))
  (bind (_location _rotation _gripper) (break `/Game/Structs/AdaptiveAxis` AdaptiveAxis))
  (`KismetSystemLibrary.PrintString` (`KismetStringLibrary.Conv_VectorToString` _location) true true (struct :`G` 0.66 :`B` 1.0 :`A` 1.0) 15.0)
  (`KismetSystemLibrary.PrintString` (`KismetStringLibrary.Conv_RotatorToString` _rotation) true true (struct :`G` 0.66 :`B` 1.0 :`A` 1.0) 15.0)
  (`KismetSystemLibrary.PrintString` (`KismetStringLibrary.Conv_DoubleToString` _gripper) true true (struct :`G` 0.66 :`B` 1.0 :`A` 1.0) 15.0))

(fn `SetJaco`
  (bind _returnvalue (`GameplayStatics.GetActorOfClass` "/Game/Blueprints/BP_JacoArm/Jaco.Jaco_C"))
  (set `self.Jaco` _returnvalue))

(fn `SetPlayerPawn`
  (bind _asbp_whs_vr_pawn (cast `/Game/WHS_HCI_Study/Blueprints/BP_WHS_VR_Pawn` (`GameplayStatics.GetPlayerPawn` 0))
    (:`then`
      (set `self.Player Pawn` _asbp_whs_vr_pawn))
    (:`CastFailed`
      (`KismetSystemLibrary.PrintString` "Player not VR Pawn"))))

(fn `TargetIsDirectlyInfront`
  (returns (ReturnValue :type Boolean))
  (bind (_gripper_mover_transform_location _gripper_mover_transform_rotation) (`KismetMathLibrary.BreakTransform` (`self.GetGripperMoverTransform`)))
  (return (== (`KismetMathLibrary.GetForwardVector` _gripper_mover_transform_rotation) (`self.GetLookAtTargetNormal`) :`ErrorTolerance` 0.1)))

(fn `UserConstructionScript`)