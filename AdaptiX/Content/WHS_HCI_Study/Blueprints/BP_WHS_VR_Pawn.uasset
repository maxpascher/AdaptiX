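; Player pawn for an HCI study where a VR or desktop user teleoperates a Jaco robot arm through GripperMover.
; Two adaptive input axes move and grasp along AdaptiveSet directions, within height and reach limits.
; Mode switches cycle those directions by button or retriggerable delay, coordinating with BP_AxisWizard and logging to BP_GM_Study.
; It also handles direct axis control, timed gripper return, a wrist or screen camera HUD and a UI beam pointer; SendInputToCNN is empty.
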(event `self.ReceiveBeginPlay`
  (bind _returnvalue (`GameplayStatics.GetPlayerController` 0))
  (bind _non_vrviewpointcamera (`self.Non-VRViewpointCamera`))
  (bind _widgetinteraction (`self.WidgetInteraction`))
  (bind _jaco (`self.Jaco`))
  ;[1 1 1] Begin Play
  (if (`HeadMountedDisplayFunctionLibrary.IsHeadMountedDisplayConnected`)
    (`ActorComponent.Activate` (`self.LeftHandMotionController`) false)
    (`ActorComponent.Activate` (`self.RightHandMotionController`) false)
    (`ActorComponent.Activate` (`self.VRCamera`) false)
    (`ActorComponent.Deactivate` _non_vrviewpointcamera)
    (bind _returnvalue_2 (`AddComponent|NODE_AddWidgetComponent-0` :`bManualAttachment` true))
    (`WidgetComponent.SetTwoSided` _returnvalue_2 true) ; Bug here, back is black
    (`WidgetComponent.SetDrawSize` _returnvalue_2 (1491.0 923.0))
    (bind _returnvalue_3 (`|CreateWidget` "/Game/Blueprints/BP_JacoArm/HUD_on_Wrist.HUD_on_Wrist_C" (`GameplayStatics.GetPlayerController` 0)))
    (bind _output_get (set `self.HUD` _returnvalue_3))
    (`WidgetComponent.SetWidget` _returnvalue_2 _output_get)
    (`SceneComponent.K2_AttachToComponent` _returnvalue_2 (`self.RightControllerMesh`) "None" "KeepRelative" "SnapToTarget" "KeepWorld" true)
    (`SceneComponent.K2_SetRelativeTransform` _returnvalue_2 (`KismetMathLibrary.MakeTransform` (-15.5 0.0 20.0) (struct :`Yaw` 180.0) (0.03 0.03 0.03)) false true)
    (set `WidgetInteractionComponent.InteractionSource` "World" _widgetinteraction)
    (else
      (`ActorComponent.Deactivate` (`self.RightHandMotionController`))
      (`ActorComponent.Deactivate` (`self.LeftHandMotionController`))
      (`ActorComponent.Deactivate` (`self.VRCamera`))
      (`ActorComponent.Activate` _non_vrviewpointcamera false)
      (if (`KismetSystemLibrary.IsValid` _returnvalue)
        (bind _returnvalue_4 (`|CreateWidget` "/Game/Blueprints/BP_JacoArm/HUD_on_Wrist.HUD_on_Wrist_C" _returnvalue))
        (`UserWidget.AddToViewport` _returnvalue_4 0)
        (set `self.HUD` _returnvalue_4))
      (set `WidgetInteractionComponent.InteractionSource` "CenterScreen" _widgetinteraction)
      (set `WidgetInteractionComponent.bShowDebug` true _widgetinteraction)))
  (`SceneComponent.K2_SetWorldTransform` (`self.GripperMover`) (`KismetMathLibrary.MakeTransform` (180.0 -160.0 110.0) (struct :`Yaw` -90.0)) false false)
  (`self.Connect Jaco`)
  (bind _returnvalue_5 (`GameplayStatics.GetActorOfClass` "/Game/WHS_HCI_Study/Blueprints/UIWidgets/UIWidget.UIWidget_C"))
  (set `self.UIWidget` _returnvalue_5)
  (`FXSystemComponent.SetColorParameter` (`self.ParticleSystem`) "BeamColor" (make `LinearColor` 0.0 0.5 0.5))
  (`/Game/Blueprints/BP_JacoArm/Jaco.SetFinger` _jaco 1 0.0)
  (`/Game/Blueprints/BP_JacoArm/Jaco.Set Finger Tip` _jaco 1 0.0)
  (`/Game/Blueprints/BP_JacoArm/Jaco.SetFinger` _jaco 2 0.0)
  (`/Game/Blueprints/BP_JacoArm/Jaco.Set Finger Tip` _jaco 2 0.0)
  (`/Game/Blueprints/BP_JacoArm/Jaco.SetFinger` _jaco 3 0.0)
  (`/Game/Blueprints/BP_JacoArm/Jaco.Set Finger Tip` _jaco 3 0.0)
  (bind _returnvalue_6 (`GameplayStatics.GetActorOfClass` "/Game/WHS_HCI_Study/Blueprints/BP_AxisWizard.BP_AxisWizard_C"))
  (set `self.Wizard` _returnvalue_6)
  (bind _asbp_gm_study (cast `/Game/WHS_HCI_Study/Blueprints/BP_GM_Study` (`GameplayStatics.GetGameMode`)))
  (set `self.GM_Study` _asbp_gm_study))

(event `InputAction|ConnectToJaco`
  (params (Key :type "Key Structure"))
  ;[1 1 1] Connect to Jaco
  (:`Pressed`
    (`self.Connect Jaco`)))

(event `InputAction|Quit`
  (params (Key :type "Key Structure"))
  ;[1 1 1] Quit Game on User Input
  (:`Pressed`
    (`KismetSystemLibrary.QuitGame` null "Quit")))

(event `InputAxis|Adaptive_1`
  (params (AxisValue :type "Float (single-precision)"))
  (bind (_adaptiveset_direction_0 _adaptiveset_direction_1) (break `/Game/Structs/AdaptiveSet` (`self.AdaptiveSet`)))
  ;[1 1 1] Adaptive Input
  (if (or (not (`self.RealtimeVisu`)) (not (`/Game/WHS_HCI_Study/Blueprints/BP_AxisWizard.Enabled` (`self.Wizard`))))
    (`self.LogMovementEvents` (`KismetMathLibrary.FMax` (`KismetMathLibrary.Abs` (stale `InputAxis|Adaptive_0` AxisValue)) (`KismetMathLibrary.Abs` AxisValue)))
    (set `/Game/WHS_HCI_Study/Blueprints/BP_AxisWizard.AdaptiveInputAxis1` AxisValue (`self.Wizard`))
    (if (and (not (`self.StopInput`)) (> (`KismetMathLibrary.Abs` AxisValue) 0.2))
      (`self.Adaptive Movement` AxisValue _adaptiveset_direction_1))))

(event `InputAxis|Adaptive_0`
  (params (AxisValue :type "Float (single-precision)"))
  (bind (_adaptiveset_direction_0 _adaptiveset_direction_1) (break `/Game/Structs/AdaptiveSet` (`self.AdaptiveSet`)))
  ;[1 1 1] Adaptive Input
  (`self.LogMovementEvents` (`KismetMathLibrary.FMax` (`KismetMathLibrary.Abs` AxisValue) (`KismetMathLibrary.Abs` (stale `InputAxis|Adaptive_1` AxisValue))))
  (set `/Game/WHS_HCI_Study/Blueprints/BP_AxisWizard.AdaptiveInputAxis0` AxisValue (`self.Wizard`))
  (if (and (not (`self.StopInput`)) (> (`KismetMathLibrary.Abs` AxisValue) 0.2))
    (`self.Adaptive Movement` AxisValue _adaptiveset_direction_0)))

(event `InputAction|Adaptive_Update_Once`
  (params (Key :type "Key Structure"))
  ;[1 1 1] Adaptive Input
  (:`Pressed`
    (`self.SendInputToCNN`)))

(event `InputAction|Adaptive_Start_Regular_Update`
  (params (Key :type "Key Structure"))
  ;[1 1 1] Adaptive Input
  (:`Pressed`
    (`KismetSystemLibrary.K2_SetTimer` null "SendInputToCNN" 0.5 true)
    (`KismetSystemLibrary.PrintString` "Adaptive Data Is send regularly.")))

(event `InputAction|Adaptive_Stop_Regular_Update`
  (params (Key :type "Key Structure"))
  ;[1 1 1] Adaptive Input
  (:`Pressed`
    (`KismetSystemLibrary.K2_ClearTimer` null "SendInputToCNN")))

(event `InputAction|Toggle_Hud`
  (params (Key :type "Key Structure"))
  (bind _jaco (`self.Jaco`))
  ;[1 1 1] Toggle HUD
  (:`Pressed`
    (`/Game/Blueprints/BP_JacoArm/HUD_on_Wrist.ToggleVisibility` (`self.HUD`))
    (`SceneComponent.ToggleVisibility` (`self.RightControllerMesh`) false)
    (if (!= _jaco null)
      (bind _asbp_d435 (cast `/Game/Blueprints/BP_JacoArm/BP_D435` (`ChildActorComponent.ChildActor` (`/Game/Blueprints/BP_JacoArm/Jaco.CameraAbove` _jaco))))
      (`/Game/Blueprints/BP_JacoArm/HUD_on_Wrist.SetCameras` (`self.HUD`) (`/Game/Blueprints/BP_JacoArm/BP_D435.RGB_Cam` _asbp_d435) (`/Game/Blueprints/BP_JacoArm/BP_D435.Depth_Cam` _asbp_d435) (`/Game/Blueprints/BP_JacoArm/BP_D435.Segment_Cam` _asbp_d435))
      (`/Game/Blueprints/BP_JacoArm/BP_D435.ActivateCameras` _asbp_d435)
      (else
        (`KismetSystemLibrary.PrintString` "No robot with camera connected")))))

(event `InputAxis|Gripper_X`
  (params (AxisValue :type "Float (single-precision)"))
  ;[1 1 1] Move based on Input
  (`SceneComponent.K2_AddLocalTransform` (`self.GripperMover`) (`KismetMathLibrary.MakeTransform` (`KismetMathLibrary.MakeVector` (.z (* (.location (`KismetMathLibrary.MakeTransform` (`KismetMathLibrary.MakeVector` AxisValue (`self.GetInputAxisValue`) (`self.GetInputAxisValue`)) (`KismetMathLibrary.MakeRotator` (`self.GetInputAxisValue`) (`self.GetInputAxisValue`) (`self.GetInputAxisValue`)))) (`self.Vel_Trans`))) (.x (* (.location (`KismetMathLibrary.MakeTransform` (`KismetMathLibrary.MakeVector` AxisValue (`self.GetInputAxisValue`) (`self.GetInputAxisValue`)) (`KismetMathLibrary.MakeRotator` (`self.GetInputAxisValue`) (`self.GetInputAxisValue`) (`self.GetInputAxisValue`)))) (`self.Vel_Trans`))) (* -1.0 (.y (* (.location (`KismetMathLibrary.MakeTransform` (`KismetMathLibrary.MakeVector` AxisValue (`self.GetInputAxisValue`) (`self.GetInputAxisValue`)) (`KismetMathLibrary.MakeRotator` (`self.GetInputAxisValue`) (`self.GetInputAxisValue`) (`self.GetInputAxisValue`)))) (`self.Vel_Trans`))))) (`KismetMathLibrary.MakeRotator` (.yaw (* (.rotation (`KismetMathLibrary.MakeTransform` (`KismetMathLibrary.MakeVector` AxisValue (`self.GetInputAxisValue`) (`self.GetInputAxisValue`)) (`KismetMathLibrary.MakeRotator` (`self.GetInputAxisValue`) (`self.GetInputAxisValue`) (`self.GetInputAxisValue`)))) (`self.Vel_Rot`))) (.pitch (* (.rotation (`KismetMathLibrary.MakeTransform` (`KismetMathLibrary.MakeVector` AxisValue (`self.GetInputAxisValue`) (`self.GetInputAxisValue`)) (`KismetMathLibrary.MakeRotator` (`self.GetInputAxisValue`) (`self.GetInputAxisValue`) (`self.GetInputAxisValue`)))) (`self.Vel_Rot`))) (.roll (* (.rotation (`KismetMathLibrary.MakeTransform` (`KismetMathLibrary.MakeVector` AxisValue (`self.GetInputAxisValue`) (`self.GetInputAxisValue`)) (`KismetMathLibrary.MakeRotator` (`self.GetInputAxisValue`) (`self.GetInputAxisValue`) (`self.GetInputAxisValue`)))) (`self.Vel_Rot`)))) (.scale (`KismetMathLibrary.MakeTransform` (`KismetMathLibrary.MakeVector` AxisValue (`self.GetInputAxisValue`) (`self.GetInputAxisValue`)) (`KismetMathLibrary.MakeRotator` (`self.GetInputAxisValue`) (`self.GetInputAxisValue`) (`self.GetInputAxisValue`))))) false false))

(event `InputAxisKey|MouseY`
  (params (AxisValue :type "Float (single-precision)"))
  ;[1 1 1] Move based on Input
  (`SceneComponent.K2_AddRelativeRotation` (`self.Non-VRViewpointCamera`) (`KismetMathLibrary.MakeRotator` 0.0 AxisValue (`self.GetInputAxisKeyValue`)) false false))

(event `InputAxis|MoveForward`
  (params (AxisValue :type "Float (single-precision)"))
  ;[1 1 1] Move based on Input
  (`SceneComponent.K2_AddLocalOffset` (`self.Non-VRViewpointCamera`) (`KismetMathLibrary.MakeVector` AxisValue (`self.GetInputAxisValue`) (`self.GetInputAxisValue`)) false false))

(event `InputAxis|Gripper_Close`
  (params (AxisValue :type "Float (single-precision)"))
  ;[1 1 1] Move based on Input
  (if (!= (`self.Jaco`) null)
    (`/Game/Blueprints/BP_JacoArm/Jaco.Grasp` (`self.Jaco`) (+ AxisValue (`self.GetInputAxisValue`) (`self.GetInputAxisValue`)))))

(event `self.ReceiveTick`
  (params (DeltaSeconds :type "Float (single-precision)"))
  (bind _array (`|MakeArray` 0 1 2 6 7 0 4 5 6 2 3 4))
  (bind _timer (`self.Timer`))
  (bind (_lastgrippermovertransform_location _lastgrippermovertransform_rotation) (`KismetMathLibrary.BreakTransform` (`self.LastGripperMoverTransform`)))
  (bind (_adaptiveset_direction_0 _adaptiveset_direction_1 _adaptiveset_direction_2 _adaptiveset_direction_3 _adaptiveset_direction_4 _adaptiveset_direction_5 _adaptiveset_direction_6) (break `/Game/Structs/AdaptiveSet` (`self.AdaptiveSet`)))
  (bind (_adaptiveset_direction_0_2 _adaptiveset_direction_1_2 _adaptiveset_direction_2_2 _adaptiveset_direction_3_2 _adaptiveset_direction_4_2 _adaptiveset_direction_5_2 _adaptiveset_direction_6_2) (break `/Game/Structs/AdaptiveSet` (`self.AdaptiveSet`)))
  (bind (_adaptiveset_direction_0_3 _adaptiveset_direction_1_3 _adaptiveset_direction_2_3 _adaptiveset_direction_3_3 _adaptiveset_direction_4_3 _adaptiveset_direction_5_3 _adaptiveset_direction_6_3) (break `/Game/Structs/AdaptiveSet` (`self.AdaptiveSet`)))
  (bind (_adaptivesetdefault_direction_0 _adaptivesetdefault_direction_1 _adaptivesetdefault_direction_2 _adaptivesetdefault_direction_3 _adaptivesetdefault_direction_4 _adaptivesetdefault_direction_5 _adaptivesetdefault_direction_6) (break `/Game/Structs/AdaptiveSet` (`self.AdaptiveSetDefault`)))
  (bind _unrotatearray (`self.UnrotateArray`))
  (bind _particlesystem (`self.ParticleSystem`))
  (bind _widgetinteraction (`self.WidgetInteraction`))
  (bind (_returnvalue_bblockinghit _returnvalue_binitialoverlap _returnvalue_time _returnvalue_distance _returnvalue_location _returnvalue_impactpoint _returnvalue_normal _returnvalue_impactnormal _returnvalue_physmat _returnvalue_hitactor) (`GameplayStatics.BreakHitResult` (`WidgetInteractionComponent.GetLastHitResult` _widgetinteraction)))
  (bind _returnvalue (`SceneComponent.K2_GetComponentRotation` (`self.GripperMover`)))
  (bind _returnvalue_2 (`KismetSystemLibrary.K2_GetTimerElapsedTimeHandle` _timer))
  (bind _returnvalue_3 (not (`self.ButtonModeSwitch`)))
  (bind _returnvalue_4 (* (`self.AdaptiveSetModeSwitchCount`) 3))
  (bind _returnvalue_5 (+ (`self.AdaptiveSetModeSwitchCount`) 1))
  (bind _array_2 (`|MakeArray` _adaptivesetdefault_direction_0 _adaptivesetdefault_direction_1 _adaptivesetdefault_direction_2 _adaptivesetdefault_direction_3 _adaptivesetdefault_direction_4 _adaptivesetdefault_direction_5 _adaptivesetdefault_direction_6))
  (bind _returnvalue_6 (== _returnvalue_hitactor (`self.UIWidget`)))
  (bind _returnvalue_7 (mod _returnvalue_5 4))
  (bind _returnvalue_8 (and (`KismetMathLibrary.NearlyEqual_FloatFloat` (`self.GetInputAxisValue`) 0.0 0.1) (`KismetMathLibrary.NearlyEqual_FloatFloat` (`self.GetInputAxisValue`) 0.0 0.1)))
  (bind (_output_location _output_rotation _output_gripper) (break `/Game/Structs/AdaptiveAxis` (`|GetArrayItem` _array_2 2)))
  (bind (_output_location_2 _output_rotation_2 _output_gripper_2) (break `/Game/Structs/AdaptiveAxis` (`|GetArrayItem` _array_2)))
  (bind (_output_location_3 _output_rotation_3 _output_gripper_3) (break `/Game/Structs/AdaptiveAxis` (`|GetArrayItem` _array_2 1)))
  (bind _returnvalue_9 (/ _returnvalue_2 (+ _returnvalue_2 (`KismetSystemLibrary.K2_GetTimerRemainingTimeHandle` _timer))))
  (if (not (`self.JacoAttached`))
    (`/Game/Blueprints/BP_JacoArm/Jaco.Connect to Motion Controller` (`self.Jaco`) (`self.GripperMover`) true false false)
    (set `self.JacoAttached` true))
  (`ParticleSystemComponent.SetBeamSourcePoint` _particlesystem 0 (`KismetMathLibrary.SelectVector` (`SceneComponent.K2_GetComponentLocation` _widgetinteraction) (0.0 0.0 0.0) _returnvalue_6) 0)
  (`ParticleSystemComponent.SetBeamEndPoint` _particlesystem 0 (`KismetMathLibrary.SelectVector` _returnvalue_impactpoint (0.0 0.0 0.0) _returnvalue_6))
  (if (and (`self.RealtimeVisu`) (not (`/Game/WHS_HCI_Study/Blueprints/BP_AxisWizard.Enabled` (`self.Wizard`))))
    (set `self.UnrotateArray` (`|MakeArray` _adaptiveset_direction_0_3 _adaptiveset_direction_1_3 _adaptiveset_direction_2_3 _adaptiveset_direction_3_3 _adaptiveset_direction_4_3 _adaptiveset_direction_5_3 _adaptiveset_direction_6_3 (`self.LastBufferSetDirection`)))
    (`KismetArrayLibrary.Array_Set` _unrotatearray (`|GetArrayItem` _array (+ _returnvalue_4 0)) (make `/Game/Structs/AdaptiveAxis` (`KismetMathLibrary.LessLess_VectorRotator` _output_location_2 _returnvalue) _output_rotation_2 _output_gripper_2))
    (`KismetArrayLibrary.Array_Set` _unrotatearray (`|GetArrayItem` _array (+ _returnvalue_4 1)) (make `/Game/Structs/AdaptiveAxis` (`KismetMathLibrary.LessLess_VectorRotator` _output_location_3 _returnvalue) _output_rotation_3 _output_gripper_3))
    (`KismetArrayLibrary.Array_Set` _unrotatearray (`|GetArrayItem` _array (+ _returnvalue_4 2)) (make `/Game/Structs/AdaptiveAxis` (`KismetMathLibrary.LessLess_VectorRotator` _output_location _returnvalue) _output_rotation _output_gripper))
    (set `self.AdaptiveSet` (make `/Game/Structs/AdaptiveSet` (`|GetArrayItem` _unrotatearray) (`|GetArrayItem` _unrotatearray 1) (`|GetArrayItem` _unrotatearray 2) (`|GetArrayItem` _unrotatearray 3) (`|GetArrayItem` _unrotatearray 4) (`|GetArrayItem` _unrotatearray 5) (`|GetArrayItem` _unrotatearray 6)))
    (set `self.LastBufferSetDirection` (`|GetArrayItem` _unrotatearray 7)))
  (if (`KismetSystemLibrary.K2_IsTimerActiveHandle` _timer)
    (`SceneComponent.K2_SetWorldLocationAndRotation` (`self.GripperMover`) (`KismetMathLibrary.VLerp` _lastgrippermovertransform_location (180.0 -160.0 110.0) _returnvalue_9) (`KismetMathLibrary.RLerp` _lastgrippermovertransform_rotation (struct :`Yaw` -90.0) _returnvalue_9) false false)
    (`/Game/Blueprints/BP_JacoArm/Jaco.Grasp` (`self.Jaco`) -1.0)
    (else
      (set `self.LastGripperMoverTransform` (`SceneComponent.K2_GetComponentToWorld` (`self.GripperMover`)))))
  (if _returnvalue_3
    (if (not _returnvalue_8)
      (`KismetSystemLibrary.RetriggerableDelay` (`self.Mode Switch Delay`) :!label _label)
      (if (and (`self.RealtimeVisu`) (`/Game/WHS_HCI_Study/Blueprints/BP_AxisWizard.Enabled` (`self.Wizard`))) :!label _label_2
        (set `self.AdaptiveSet` (make `/Game/Structs/AdaptiveSet` _adaptiveset_direction_2 _adaptiveset_direction_1 _adaptiveset_direction_3 _adaptiveset_direction_4 _adaptiveset_direction_5 _adaptiveset_direction_6 _adaptiveset_direction_0))
        (else
          (set `self.BufferSetDirection` _adaptiveset_direction_1_2)
          (set `self.AdaptiveSet` (make `/Game/Structs/AdaptiveSet` _adaptiveset_direction_2_2 _adaptiveset_direction_3_2 _adaptiveset_direction_4_2 _adaptiveset_direction_5_2 _adaptiveset_direction_6_2 (`self.LastBufferSetDirection`) _adaptiveset_direction_0_2))
          (set `self.LastBufferSetDirection` (`self.BufferSetDirection`))))
      (bind _output_get (set `self.SecondFour` (xor (> _returnvalue_5 3) (`self.SecondFour`))))
      (if _output_get
        (if (and (`/Game/WHS_HCI_Study/Blueprints/BP_AxisWizard.Enabled` (`self.Wizard`)) (> _returnvalue_7 1))
          (set `self.AdaptiveSetModeSwitchCount` 0)
          (set `self.SecondFour` false)
          (else
            (set `self.AdaptiveSetModeSwitchCount` _returnvalue_7 :!label _label_3)))
        (else
          (goto _label_3)))
      (`/Game/WHS_HCI_Study/Blueprints/BP_GM_Study.Mode Switched` (`self.GM_Study`))
      (if (and _returnvalue_3 _returnvalue_8)
        (goto _label)))))

(event `InputAction|ModeSwitch`
  (params (Key :type "Key Structure"))
  (:`Pressed`
    (if (`self.ButtonModeSwitch`)
      (goto _label_2))))

(event `Start Mode Switch Timer`
  (if (not (`self.ButtonModeSwitch`))
    (goto _label)))

(event `InputAction|TriggerPointer`
  (params (Key :type "Key Structure"))
  (:`Pressed`
    (`WidgetInteractionComponent.PressPointerKey` (`self.WidgetInteraction`) "LeftMouseButton")
    (`WidgetInteractionComponent.PressPointerKey` (`self.WidgetInteraction`) "RightMouseButton"))
  (:`Released`
    (`WidgetInteractionComponent.ReleasePointerKey` (`self.WidgetInteraction`) "LeftMouseButton")
    (`WidgetInteractionComponent.ReleasePointerKey` (`self.WidgetInteraction`) "RightMouseButton")))

(event `InputAction|RestartLevel`
  (params (Key :type "Key Structure"))
  (:`Pressed`
    (`GameplayStatics.OpenLevel` "WHS_Study_Room")))

(fn `Adaptive Movement`
  (params (AxisValue :type "Float (double-precision)") (Axis :type "/Game/Structs/AdaptiveAxis Structure"))
  (locals (`Prev Transform` :type "Transform Structure"))
  (bind (_location _rotation _gripper) (break `/Game/Structs/AdaptiveAxis` Axis))
  (bind _returnvalue (`SceneComponent.K2_GetComponentLocation` (`self.GripperMover`)))
  (set `local.Prev Transform` (`SceneComponent.K2_GetComponentToWorld` (`self.GripperMover`)))
  (`SceneComponent.K2_AddLocalTransform` (`self.GripperMover`) (`KismetMathLibrary.MakeTransform` (* (* _location AxisValue) (`self.Vel_Trans`)) (* (* _rotation AxisValue) (`self.Vel_Rot`))) true false)
  (if (or (< (.z _returnvalue) 80.0) (> (`KismetMathLibrary.Vector_Distance` _returnvalue (`SceneComponent.K2_GetComponentLocation` (`SkeletalMeshActor.SkeletalMeshComponent` (`self.Jaco`)))) 97.0))
    (`SceneComponent.K2_SetWorldTransform` (`self.GripperMover`) (`local.Prev Transform`) false false)
    (elif (!= (`self.Jaco`) null)
      (`/Game/Blueprints/BP_JacoArm/Jaco.Grasp` (`self.Jaco`) (* _gripper AxisValue)))))

(fn `Connect Jaco`
  ;[1 1 1] If unconnected
  (if (== (`self.Jaco`) null)
    (bind _returnvalue (`GameplayStatics.GetActorOfClass` "/Game/Blueprints/BP_JacoArm/Jaco.Jaco_C"))
    (set `self.Jaco` _returnvalue)
    (`KismetSystemLibrary.PrintString` "Connected to Jaco")
    (else
      (`KismetSystemLibrary.PrintString` "Jaco already connected"))))

(fn `LogMovementEvents`
  (params (AxisValue :type "Float (double-precision)"))
  (if (and (<= (`KismetMathLibrary.Abs` AxisValue) 0.2) (> (`KismetMathLibrary.Abs` (`self.LastAxisValue`)) 0.2))
    (`/Game/WHS_HCI_Study/Blueprints/BP_GM_Study.LogMovementEvent` (`self.GM_Study`) "movement_stop")
    (elif (and (<= (`KismetMathLibrary.Abs` (`self.LastAxisValue`)) 0.2) (> (`KismetMathLibrary.Abs` AxisValue) 0.2))
      (`/Game/WHS_HCI_Study/Blueprints/BP_GM_Study.LogMovementEvent` (`self.GM_Study`) "movement_start")))
  (set `self.LastAxisValue` AxisValue))

(fn `SendInputToCNN`)

(fn `Set Calculated Adaptive Set`
  (params (`New Adaptive Set` :type "/Game/Structs/AdaptiveSet Structure"))
  (locals (`Adaptive Set Array` :type "Array of /Game/Structs/AdaptiveAxis Structure"))
  (bind (_adaptiveset_direction_0 _adaptiveset_direction_1) (break `/Game/Structs/AdaptiveSet` (`self.AdaptiveSet`)))
  (set `self.AdaptiveSet` (make `/Game/Structs/AdaptiveSet` _adaptiveset_direction_0 _adaptiveset_direction_1 `New Adaptive Set_Direction_0_16_91C360CC44DBF37029EB10843AC88580` `New Adaptive Set_Direction_1_17_87DC5C864BD2C92B61D515966BE9795E` `New Adaptive Set_Direction_2_19_CB7E6B1B4BB556FBD1DD948D841CE654` `New Adaptive Set_Direction_3_18_BE2CBEF34BFE3E60BC9D61A226930034` `New Adaptive Set_Direction_4_20_5885B32748CCE6ECA9EE34A008E09773`))
  (set `self.LastBufferSetDirection` `New Adaptive Set_Direction_5_21_10E34D6D4CA3F7631F6E1F93C94C571C`)
  (set `self.AdaptiveSetModeSwitchCount` 1)
  (set `self.SecondFour` true))

(fn `StartGripperReturn`
  (params (Timer :type "TimerHandle Structure"))
  (set `self.Timer` Timer)
  (set `self.StopInput` true))

(fn `UserConstructionScript`)