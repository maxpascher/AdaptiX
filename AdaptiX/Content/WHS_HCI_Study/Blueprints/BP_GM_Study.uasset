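; Game mode for a VR user study of Jaco robot arm control, comparing control-method and visualisation conditions over box trials.
; Conditions come from a server, or local fallbacks when offline, and configure the gizmos, waypoints and axis wizard.
; Dispatcher events drive trial flow, level resets, threshold feedback and metric logging.
; EndGame uploads results and Base64 audio per condition; Tick spawns audio capture, checking Android permissions first.
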(event `Request User Properties Event`
  (params (Request :type "VaRestRequestJSON Object Reference"))
  (`self.Decode User Properties` Request
    (:`Completed`
      (add `self.BeginTrialDispatcher` (delegate `BeginTrial`) :!label _label)
      (add `self.BeginConditionDispatcher` (delegate `BeginCondition`))
      (add `self.EndTrainingTrialDispatcher` (delegate `EndTrainingTrial`))
      (add `self.BeginTrainingTrialDispatcher` (delegate `BeginTrainingTrial`))
      (add `self.ResetTrialDispatcher` (delegate `ResetTrial`))
      (add `self.ThresholdBrokenDispatcher` (delegate `ThresholdBroken`)))))

(event `self.ReceiveBeginPlay`
  (set `self.StudyStartTime` (`self.GetCurrentTime`))
  (add `self.Mode Switched Dispatcher` (delegate `Mode Switched`))
  (add `self.Trial Finished Dispatcher` (delegate `Trial Finished`))
  (`self.Setup Variables`)
  (`KismetArrayLibrary.Array_Clear` (`self.Box Indeces`))
  (for _index (range (`KismetArrayLibrary.Array_Length` (`/Game/WHS_HCI_Study/Blueprints/BP_Spawn_Volumes.BoxSpawnVolumes` (`self.Spawn Volumes`))))
    (`KismetArrayLibrary.Array_Add` (`self.Box Indeces`) _index))
  (if (`self.Online`)
    (set `self.RequestUserJson` (`|MakeJson`))
    (`VaRestJsonObject.SetStringField` (`self.RequestUserJson`) "api_key" (`self.ApiKey`))
    (`self.Call URL` (`self.User Properties URL`) "POST" "json" (`self.RequestUserJson`) (delegate `Request User Properties Event`))
    (else
      (`KismetSystemLibrary.Delay` 0.2) ; Simulates Request Delay
      (`self.SetupFallbackConditions`)
      (goto _label))))

(event `BeginCondition`
  (`self.Begin Condition`))

(event `BeginTrial`
  (`self.ResetLevel+`)
  (`self.Setup Variables`)
  (`self.Begin Trial`))

(event `EndTrainingTrial`
  (`/Game/WHS_HCI_Study/Blueprints/UIWidgets/UIWidget.EndTrainingTrial` (`self.UIWidget`)))

(event `BeginTrainingTrial`
  (bind _spawn_volumes (`self.Spawn Volumes`))
  (set `/Game/WHS_HCI_Study/Blueprints/BP_WHS_VR_Pawn.StopInput` false (`self.PlayerPawn`))
  (`/Game/WHS_HCI_Study/Blueprints/BP_Spawn_Volumes.PickBox` _spawn_volumes 0)
  (set `/Game/WHS_HCI_Study/Blueprints/BP_Spawn_Volumes.TrialStarted` false _spawn_volumes)
  (set `/Game/WHS_HCI_Study/Blueprints/BP_Spawn_Volumes.TimerStarted` false _spawn_volumes)
  (set `self.Mode Switches` (select `/Game/WHS_HCI_Study/Structs/ControlMethod` (`/Game/WHS_HCI_Study/Blueprints/DataClasses/BP_Condition.GetControlMethod` (`self.Get Current Condition`)) :`NewEnumerator1` -1))
  (`/Game/WHS_HCI_Study/Blueprints/BP_WHS_VR_Pawn.Start Mode Switch Timer` (`self.PlayerPawn`)))

(event `ThresholdBroken`
  (if (and (not (`self.ThresholdBrokenReset`)) (!= (`/Game/WHS_HCI_Study/Blueprints/BP_Gizmo_Arrow.RealtimeThreshold` (`|GetArrayItem` (`self.Gizmos`))) 0.0))
    (`GameplayStatics.PlaySound2D` "/Game/WHS_HCI_Study/AudioFiles/beep-point3-sec-6162.beep-point3-sec-6162" 0.5 1.0 0.0 null null)
    (`PlayerController.PlayHapticEffect` (`GameplayStatics.GetPlayerController` 0) "/Game/WHS_HCI_Study/Blueprints/ThresholdBrokenEffect.ThresholdBrokenEffect" "Right" 1.0 false)
    (set `self.ThresholdBrokenReset` true)))

(event `ResetTrial`
  (set `self.Mode Switches` 0)
  (set `self.Trial Start Time` (`self.GetCurrentTime`))
  (`/Engine/EditorBlueprintResources/StandardMacros.IncrementInt` (`self.TrialResets`)
    (:`  `
      (set `/Game/WHS_HCI_Study/Blueprints/BP_WHS_VR_Pawn.StopInput` false (`self.PlayerPawn`)))))

(event `Trial Finished`
  (`self.End Trial`
    (:`Next Trial Available`
      (`self.ResetLevel+`)
      (`self.Setup Variables`)
      (`self.Begin Trial`))
    (:`No More Trials`
      (`self.End Condition`)
      (`/Game/WHS_HCI_Study/Blueprints/UIWidgets/UIWidget.ShowQuestionnaire` (`self.UIWidget`)))))

(event `Mode Switched`
  (`/Engine/EditorBlueprintResources/StandardMacros.IncrementInt` (`self.Mode Switches`)
    (:`  `
      (`self.LogMovementEvent` "mode_switch")
      (set `self.ThresholdBrokenReset` false))))

(event `self.ReceiveTick`
  (params (DeltaSeconds :type "Float (single-precision)"))
  (bind _array (`|MakeArray` "android.permission.RECORD_AUDIO" "android.permission.WRITE_EXTERNAL_STORAGE" "android.permission.READ_EXTERNAL_STORAGE"))
  (if (`KismetStringLibrary.EqualEqual_StrStr` (`GameplayStatics.GetPlatformName`) "Android")
    (if (not (`self.PermissionsGranted`))
      (for _array_element _array
        (bind _returnvalue (`AndroidPermissionFunctionLibrary.CheckPermission` _array_element))
        (if _returnvalue
          (set `self.PermissionsGranted` true)
          (else
            (set `self.PermissionsGranted` false)
            (break))))
      (if (not (`self.PermissionsGranted`))
        (bind _returnvalue_2 (`AndroidPermissionFunctionLibrary.AcquirePermissions` _array))
        (add `AndroidPermissionCallbackProxy.OnPermissionsGrantedDynamicDelegate` _returnvalue_2 (delegate `OnPermissionsGrantedDynamicDelegate_Event_0`)))
      (else
        (if (not (`self.AudioCaptureSpawned`)) :!label _label_2
          (`|SpawnActorFromClass` "/Game/WHS_HCI_Study/Blueprints/BP_AudioCapture.BP_AudioCapture_C" (`KismetMathLibrary.MakeTransform` (0.0 0.0 0.0)) "Undefined" "OverrideRootScale" null null)
          (set `self.AudioCaptureSpawned` true))))
    (else
      (goto _label_2))))

(event `OnPermissionsGrantedDynamicDelegate_Event_0`
  (params (Permissions :type "Array of String (by ref)") (GrantResults :type "Array of Boolean (by ref)"))
  (set `self.PermissionsGranted` true))

(fn `Call URL`
  (params (URL :type String) (Verb :type "EVaRestRequestVerb Enum" :default "GET") (`Content Type` :type "EVaRestRequestContentType Enum" :default "x_www_form_urlencoded_url") (`Json Body` :type "VaRestJsonObject Object Reference") (`Response Callback` :type "Delegate (by ref)"))
  (`VaRestSubsystem.CallURL` (subsystem `VaRestSubsystem`) URL Verb `Content Type` `Json Body` `Response Callback`))

(fn `EndGame`
  (params (`Response Callback` :type "Delegate (by ref)"))
  (locals (AudioJson :type "VaRestJsonObject Object Reference"))
  (bind _audiojson (`local.AudioJson`))
  (bind _finaljsonobject (`self.FinalJsonObject`))
  (set `self.FinalJsonObject` (`|MakeJson`))
  (`VaRestJsonObject.SetStringField` _finaljsonobject "api_key" (`self.ApiKey`))
  (`VaRestJsonObject.SetIntegerField` _finaljsonobject "id" (`self.UserID`))
  (`VaRestJsonObject.SetNumberField` _finaljsonobject "study_completion_time" (- (`self.GetCurrentTime`) (`self.StudyStartTime`)))
  (for _array_element (`self.Conditions`)
    (`KismetArrayLibrary.Array_Add` (`self.ConditionsJsonArray`) (`/Game/WHS_HCI_Study/Blueprints/DataClasses/BP_Condition.ToJson` _array_element)))
  (`VaRestJsonObject.SetObjectArrayField` _finaljsonobject "conditions" (`self.ConditionsJsonArray`))
  (`self.Call URL` (`self.Save Results URL`) "POST" "json" _finaljsonobject `Response Callback`)
  (for _array_element_2 (`self.Conditions`)
    (set `local.AudioJson` (`|MakeJson`))
    (`VaRestJsonObject.SetStringField` _audiojson "api_key" (`self.ApiKey`))
    (`VaRestJsonObject.SetIntegerField` _audiojson "id" (`self.UserID`))
    (bind _audiobase64 (`/Game/WHS_HCI_Study/Blueprints/DataClasses/BP_Condition.Get Audio Base 64` _array_element_2))
    (`VaRestJsonObject.SetStringField` _audiojson "audio_base_64" _audiobase64)
    (`VaRestJsonObject.SetIntegerField` _audiojson "visualisation_type" (`KismetMathLibrary.Conv_ByteToInt` (`/Game/WHS_HCI_Study/Blueprints/DataClasses/BP_Condition.VisualisationType` _array_element_2)))
    (`VaRestJsonObject.SetIntegerField` _audiojson "control_method" (`KismetMathLibrary.Conv_ByteToInt` (`/Game/WHS_HCI_Study/Blueprints/DataClasses/BP_Condition.ControlMethod` _array_element_2)))
    (`self.Call URL` (`self.Save Audio URL`) "POST" "json" _audiojson `Response Callback`))
  (`/Game/WHS_HCI_Study/Blueprints/UIWidgets/UIWidget.ShowEndingWidget` (`self.UIWidget`)))

(fn `Get Current Box Index`
  (returns (`Current Trial Index` :type Integer))
  (return (`|GetArrayItem` (`self.Box Indeces`) (mod (`/Game/WHS_HCI_Study/Blueprints/DataClasses/BP_Condition.GetNumberOfTrials` (`self.Get Current Condition`)) 8))))

(fn `Get Current Condition`
  (returns (`Current Condition` :type "/Game/WHS_HCI_Study/Blueprints/DataClasses/BP_Condition Object Reference"))
  (return (`|GetArrayItem` (`self.Conditions`) (`self.CurrentConditionIndex`))))

(fn `GetCurrentTime`
  (returns (ReturnValue :type "Float (double-precision)"))
  (bind (_seconds _partialseconds) (`GameplayStatics.GetAccurateRealTime`))
  (return (+ (`KismetMathLibrary.Conv_IntToDouble` _seconds) _partialseconds)))

(fn `LogMovementEvent`
  (params (type :type String))
  (bind _currenttrialresult (`self.CurrentTrialResult`))
  (`/Engine/EditorBlueprintResources/StandardMacros.IsValid` _currenttrialresult
    (:`Is Valid`
      (if (`/Game/WHS_HCI_Study/Blueprints/BP_Spawn_Volumes.TrialStarted` (`self.Spawn Volumes`))
        (if (`KismetStringLibrary.EqualEqual_StrStr` type "movement_stop")
          (set `self.WaitForModeSwitch` true)
          (elif (`KismetStringLibrary.EqualEqual_StrStr` type "mode_switch")
            (set `self.WaitForModeSwitch` false)
            (elif (not (and (`KismetStringLibrary.EqualEqual_StrStr` type "movement_start") (`self.WaitForModeSwitch`)))
              (`/Game/WHS_HCI_Study/Blueprints/DataClasses/BP_Trial_Results.LogInputEvent` _currenttrialresult (`KismetMathLibrary.SelectString` "new_mode_engaged" "tr_new_mode_engaged" (> (`/Game/WHS_HCI_Study/Blueprints/DataClasses/BP_Condition.GetNumberOfTrials` (`self.Get Current Condition`)) 7)) (- (`self.GetCurrentTime`) (`self.Trial Start Time`))))))
        (`/Game/WHS_HCI_Study/Blueprints/DataClasses/BP_Trial_Results.LogInputEvent` _currenttrialresult (`KismetStringLibrary.Concat_StrStr` (`KismetMathLibrary.SelectString` "" "tr_" (> (`/Game/WHS_HCI_Study/Blueprints/DataClasses/BP_Condition.GetNumberOfTrials` (`self.Get Current Condition`)) 7)) type) (- (`self.GetCurrentTime`) (`self.Trial Start Time`)))
        (set `self.LastInputEvent` type)
        (bind _foundwidgets (`WidgetBlueprintLibrary.GetAllWidgetsOfClass` "/Game/WHS_HCI_Study/Blueprints/UIWidgets/InputEvents.InputEvents_C"))
        (`/Game/WHS_HCI_Study/Blueprints/UIWidgets/InputEvents.Update` (`|GetArrayItem` _foundwidgets))))))

(fn `ResetLevel+`
  (`self.ResetLevel`)
  (bind _returnvalue (`|SpawnActorFromClass` "/Game/WHS_HCI_Study/Blueprints/BP_WHS_VR_Pawn.BP_WHS_VR_Pawn_C" (`self.GetTransform` (`self.K2_FindPlayerStart` (`GameplayStatics.GetPlayerController` 0))) "Undefined" "OverrideRootScale" null 0.4 1.0 null null))
  (`Controller.Possess` (`GameplayStatics.GetPlayerController` 0) _returnvalue)
  (`/Game/WHS_HCI_Study/Blueprints/BP_WHS_VR_Pawn.Connect Jaco` _returnvalue))

(fn `SaveNasaTLX`
  (params (NasaTLXValues :type "Array of Integer"))
  (`/Game/WHS_HCI_Study/Blueprints/DataClasses/BP_Condition.AddNasaTLXValues` (`self.Get Current Condition`) NasaTLXValues))

(fn `SetupFallbackConditions`
  (locals (NewJsonObject :type "VaRestJsonObject Object Reference"))
  (bind _conditions (`self.Conditions`))
  (set `self.UserCode` "AB12")
  (set `self.UserID` -1)
  (for _index (range 3)
    (bind _returnvalue (`|GenericCreateObject` "/Game/WHS_HCI_Study/Blueprints/DataClasses/BP_Condition.BP_Condition_C" self))
    (bind _output_get (set `local.NewJsonObject` (`|MakeJson`)))
    (switch `int` _index
      (:`0`
        (`VaRestJsonObject.SetIntegerField` _output_get "visualisation_type" 0)
        (`VaRestJsonObject.SetIntegerField` _output_get "control_method" 1)
        (`/Game/WHS_HCI_Study/Blueprints/DataClasses/BP_Condition.FromJson` _returnvalue _output_get)
        (`KismetArrayLibrary.Array_Add` _conditions _returnvalue))
      (:`1`
        (`VaRestJsonObject.SetIntegerField` _output_get "visualisation_type" 1)
        (`VaRestJsonObject.SetIntegerField` _output_get "control_method" 1)
        (`/Game/WHS_HCI_Study/Blueprints/DataClasses/BP_Condition.FromJson` _returnvalue _output_get)
        (`KismetArrayLibrary.Array_Add` _conditions _returnvalue))
      (:`2`
        (`VaRestJsonObject.SetIntegerField` _output_get "visualisation_type" 1)
        (`VaRestJsonObject.SetIntegerField` _output_get "control_method" 0)
        (`/Game/WHS_HCI_Study/Blueprints/DataClasses/BP_Condition.FromJson` _returnvalue _output_get)
        (`KismetArrayLibrary.Array_Add` _conditions _returnvalue))))
  (return))

(fn `SetupSandbox`
  (params (`Visualisation Type` :type Integer) (`Control Method` :type Integer))
  (locals (NewJsonObject :type "VaRestJsonObject Object Reference"))
  (`KismetArrayLibrary.Array_Clear` (`self.Conditions`))
  (bind _returnvalue (`|GenericCreateObject` "/Game/WHS_HCI_Study/Blueprints/DataClasses/BP_Condition.BP_Condition_C" self))
  (bind _output_get (set `local.NewJsonObject` (`|MakeJson`)))
  (`VaRestJsonObject.SetIntegerField` _output_get "visualisation_type" `Visualisation Type`)
  (`VaRestJsonObject.SetIntegerField` _output_get "control_method" `Control Method`)
  (`/Game/WHS_HCI_Study/Blueprints/DataClasses/BP_Condition.FromJson` _returnvalue _output_get)
  (`KismetArrayLibrary.Array_Add` (`self.Conditions`) _returnvalue))

(fn `Start Gripper Return`
  (params (Timer :type "TimerHandle Structure"))
  (`/Game/WHS_HCI_Study/Blueprints/BP_WHS_VR_Pawn.StartGripperReturn` (`self.PlayerPawn`) Timer))

(fn `UserConstructionScript`)