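; BP_Mode_Gizmo is a VR mode display that shows which of four adaptive control modes the player is in.
; Each tick it follows the pawn's GripperMover, turns toward the camera, hides on StopInput and moves ModeIndicator to the active mode marker.
; Changes in the Wizard's adaptive axis magnitude play or reverse the FadeOut timeline, meant to drive marker opacity.
; OnReset pauses updates briefly and re-caches the VR pawn.
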(event `self.K2_OnReset`
  (set `self.Resetting` true)
  (`KismetSystemLibrary.Delay` 0.1)
  (set `self.Resetting` false)
  ;[1 1 1] Basic setup
  (`self.SetPlayerPawn` :!label _label))

(event `self.ReceiveBeginPlay`
  (goto _label))

(event `self.ReceiveTick`
  (params (DeltaSeconds :type "Float (single-precision)"))
  (bind _player_pawn (`self.Player Pawn`))
  (bind _fadeout (`self.FadeOut`))
  (bind _wizard (`/Game/WHS_HCI_Study/Blueprints/BP_WHS_VR_Pawn.Wizard` (`self.Player Pawn`)))
  (bind _returnvalue (`KismetMathLibrary.FMax` (`KismetMathLibrary.Abs` (`/Game/WHS_HCI_Study/Blueprints/BP_AxisWizard.AdaptiveInputAxis0` _wizard)) (`KismetMathLibrary.Abs` (`/Game/WHS_HCI_Study/Blueprints/BP_AxisWizard.AdaptiveInputAxis1` _wizard))))
  (if (not (`self.Resetting`))
    (`self.FollowPlayer`)
    (`SceneComponent.SetVisibility` (`self.DefaultSceneRoot`) (not (`/Game/WHS_HCI_Study/Blueprints/BP_WHS_VR_Pawn.StopInput` _player_pawn)) true)
    (`SceneComponent.K2_SetWorldLocation` (`self.ModeIndicator`) (`SceneComponent.K2_GetComponentLocation` (select `int` (`/Game/WHS_HCI_Study/Blueprints/BP_WHS_VR_Pawn.AdaptiveSetModeSwitchCount` _player_pawn) :`0` (`self.Mode1`) :`1` (`self.Mode2`) :`2` (`self.Mode3`) :`3` (`self.Mode4`))) false false)
    (if (!= (`self.Last Movement`) _returnvalue)
      (if (== _returnvalue 0.0)
        (`TimelineComponent.ReverseFromEnd` _fadeout)
        (else
          (`TimelineComponent.PlayFromStart` _fadeout))))
    (set `self.Last Movement` _returnvalue)))

(fn `FollowPlayer`
  (bind _defaultsceneroot (`self.DefaultSceneRoot`))
  (bind (_returnvalue_location _returnvalue_rotation) (`KismetMathLibrary.BreakTransform` (`SceneComponent.K2_GetComponentToWorld` (`/Game/WHS_HCI_Study/Blueprints/BP_WHS_VR_Pawn.GripperMover` (`self.Player Pawn`)))))
  (bind (_returnvalue_roll _returnvalue_pitch _returnvalue_yaw) (`KismetMathLibrary.BreakRotator` (`KismetMathLibrary.FindLookAtRotation` (`SceneComponent.K2_GetComponentLocation` _defaultsceneroot) (`PlayerCameraManager.GetCameraLocation` (`GameplayStatics.GetPlayerCameraManager` 0)))))
  (`SceneComponent.K2_SetWorldTransform` _defaultsceneroot (`KismetMathLibrary.MakeTransform` _returnvalue_location _returnvalue_rotation (`SceneComponent.K2_GetComponentScale` _defaultsceneroot)) false false)
  (`SceneComponent.K2_SetWorldRotation` _defaultsceneroot (`KismetMathLibrary.MakeRotator` 0.0 _returnvalue_pitch _returnvalue_yaw) false false))

(fn `SetPlayerPawn`
  (bind _asbp_whs_vr_pawn (cast `/Game/WHS_HCI_Study/Blueprints/BP_WHS_VR_Pawn` (`GameplayStatics.GetPlayerPawn` 0))
    (:`then`
      (set `self.Player Pawn` _asbp_whs_vr_pawn))
    (:`CastFailed`
      (`KismetSystemLibrary.PrintString` "Player not VR Pawn"))))

(fn `UserConstructionScript`)