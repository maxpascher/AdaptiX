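; In-world UI actor for the HCI study that shows the widget panel for each study phase.
; It binds to BP_GM_Study dispatchers, hides all widget components under Plane, then enables those for the current phase; Sandbox mode shows its own starting widget.
; Condition panels follow control method and visualisation type, while begin events call back into the game mode.
; Phases assign narration sounds, but every Audio.Play call is disconnected.
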(event `self.ReceiveBeginPlay`
  (bind _asbp_gm_study (cast `/Game/WHS_HCI_Study/Blueprints/BP_GM_Study` (`GameplayStatics.GetGameMode`)))
  (set `self.GameMode` _asbp_gm_study)
  (add `self.ShowNextConditionDispatcher` (delegate `ShowNextCondition`))
  (add `self.BeginConditionDispatcher` (delegate `BeginTrial`))
  (add `self.ShowEndingWidgetDispatcher` (delegate `ShowEndingWidget`))
  (add `self.ShowQuestionaireDispatcher` (delegate `ShowQuestionnaire`))
  (add `self.ShowBeginTrainingTrialDispatcher` (delegate `ShowBeginTrainingTrial`))
  (add `self.BeginTrainingTrialDispatcher` (delegate `BeginTrainingTrialEvent`))
  (add `self.EndTrainingTrialDispatcher` (delegate `EndTrainingTrial`))
  (if (not (not (`/Game/WHS_HCI_Study/Blueprints/BP_GM_Study.Sandbox` (`self.GameMode`))))
    (`self.DisableWidgets`)
    (`self.EnableWidgetComponent` (`self.StartingWidgetSandbox`))))

(event `ShowNextCondition`
  (bind _audio (`self.Audio`))
  (bind _current_condition (`/Game/WHS_HCI_Study/Blueprints/BP_GM_Study.Get Current Condition` (`self.GameMode`)))
  (`self.DisableWidgets`)
  (if (`|EnumEquality` (`/Game/WHS_HCI_Study/Blueprints/DataClasses/BP_Condition.GetControlMethod` _current_condition) "NewEnumerator0")
    (`self.EnableWidgetComponent` (`self.ConditionK2Widget`))
    (`AudioComponent.SetSound` _audio "/Game/WHS_HCI_Study/AudioFiles/ClassicWav.ClassicWav")
    (elif (`|EnumEquality` (`/Game/WHS_HCI_Study/Blueprints/DataClasses/BP_Condition.GetVisualisationType` _current_condition) "NewEnumerator0")
      (`self.EnableWidgetComponent` (`self.ConditionA1Widget`))
      (`AudioComponent.SetSound` _audio "/Game/WHS_HCI_Study/AudioFiles/SingleArrow.SingleArrow")
      (else
        (`self.EnableWidgetComponent` (`self.ConditionA2Widget`))
        (`AudioComponent.SetSound` _audio "/Game/WHS_HCI_Study/AudioFiles/DoubleArrows.DoubleArrows"))))
  (bind _asbegin_actual_run (cast `/Game/WHS_HCI_Study/Blueprints/UIWidgets/BeginActualRun` (`WidgetComponent.GetWidget` (`self.BeginActualRuns`))))
  (`Widget.SetIsEnabled` (`/Game/WHS_HCI_Study/Blueprints/UIWidgets/BeginActualRun.Button_0` _asbegin_actual_run) true)
  (`TextBlock.SetText` (`/Game/WHS_HCI_Study/Blueprints/UIWidgets/BeginActualRun.TextBlock_70` _asbegin_actual_run) "Begin")
  (bind _asbegin_training_run (cast `/Game/WHS_HCI_Study/Blueprints/UIWidgets/BeginTrainingRun` (`WidgetComponent.GetWidget` (`self.BeginTrainingTrial`))))
  (`Widget.SetIsEnabled` (`/Game/WHS_HCI_Study/Blueprints/UIWidgets/BeginTrainingRun.Button_0` _asbegin_training_run) true)
  (`TextBlock.SetText` (`/Game/WHS_HCI_Study/Blueprints/UIWidgets/BeginTrainingRun.TextBlock_70` _asbegin_training_run) "Begin Training")
  (`self.EnableWidgetComponent` (`self.ImageWidget`)))

(event `BeginTrial`
  (`/Game/WHS_HCI_Study/Blueprints/BP_GM_Study.BeginTrial` (`self.GameMode`))
  (`self.DisableWidgets`)
  (`self.EnableWidgetComponent` (`self.TrialRunningWidget`)))

(event `ShowEndingWidget`
  (bind _imagewidget (`self.ImageWidget`))
  (`self.DisableWidgets`)
  (`self.EnableWidgetComponent` (`self.EndingWidget`))
  (`SceneComponent.SetVisibility` _imagewidget false false)
  (`Widget.SetIsEnabled` (`WidgetComponent.GetWidget` _imagewidget) false)
  (`AudioComponent.SetSound` (`self.Audio`) "/Game/WHS_HCI_Study/AudioFiles/ThankYou.ThankYou"))

(event `ShowQuestionnaire`
  (`self.DisableWidgets`)
  (`self.EnableWidgetComponent` (`self.QuestionnaireWidget`))
  (`AudioComponent.SetSound` (`self.Audio`) "/Game/WHS_HCI_Study/AudioFiles/Questionnaire.Questionnaire"))

(event `ShowBeginTrainingTrial`
  (`self.DisableWidgets`)
  (`self.EnableWidgetComponent` (`self.BeginTrainingTrial`))
  (`AudioComponent.SetSound` (`self.Audio`) "/Game/WHS_HCI_Study/AudioFiles/TrainingTask.TrainingTask"))

(event `EndTrainingTrial`
  (bind _asbegin_training_run (cast `/Game/WHS_HCI_Study/Blueprints/UIWidgets/BeginTrainingRun` (`WidgetComponent.GetWidget` (`self.BeginTrainingTrial`))))
  (`Widget.SetVisibility` (`/Game/WHS_HCI_Study/Blueprints/UIWidgets/BeginTrainingRun.Button_0` _asbegin_training_run) "Visible")
  (`self.DisableWidgets`)
  (`self.EnableWidgetComponent` (`self.BeginActualRuns`))
  (`AudioComponent.SetSound` (`self.Audio`) "/Game/WHS_HCI_Study/AudioFiles/ActualTrialWav.ActualTrialWav"))

(event `BeginTrainingTrialEvent`
  (bind _asbegin_training_run (cast `/Game/WHS_HCI_Study/Blueprints/UIWidgets/BeginTrainingRun` (`WidgetComponent.GetWidget` (`self.BeginTrainingTrial`))))
  (`Widget.SetVisibility` (`/Game/WHS_HCI_Study/Blueprints/UIWidgets/BeginTrainingRun.Button_0` _asbegin_training_run) "Hidden")
  (`/Game/WHS_HCI_Study/Blueprints/BP_GM_Study.BeginTrainingTrial` (`self.GameMode`))
  (`AudioComponent.Stop` (`self.Audio`)))

(fn `EnableWidgetComponent`
  (params (WidgetComponent :type "WidgetComponent Object Reference"))
  (`SceneComponent.SetVisibility` WidgetComponent true false)
  (`Widget.SetIsEnabled` (`WidgetComponent.GetWidget` WidgetComponent) true))

(fn `UserConstructionScript`)