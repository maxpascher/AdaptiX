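; Manages box placement trials in an HCI study with the Jaco robot arm, spawning boxes and judging their delivery to a target.
; Caches box transforms and parks boxes at the origin; PickBox restores one by index, enabling physics after a short delay.
; Tick treats a still, released box on target as success and one straying too far as failure.
; Either outcome plays a sound, starts gripper return and notifies BP_GM_Study through timers.
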(event `self.ReceiveBeginPlay`
  (bind _returnvalue (`GameplayStatics.GetActorOfClass` "/Game/Blueprints/BP_JacoArm/Jaco.Jaco_C"))
  (set `self.Jaco` _returnvalue))

(event `InTrialReset`
  (bind _asbp_gm_study (cast `/Game/WHS_HCI_Study/Blueprints/BP_GM_Study` (`GameplayStatics.GetGameMode`)))
  (`/Game/WHS_HCI_Study/Blueprints/BP_GM_Study.ResetTrial` _asbp_gm_study)
  (set `self.ResetHappening` false))

(event `Trial Finished Timer`
  (set `self.TimerStarted` false)
  (bind _asbp_gm_study (cast `/Game/WHS_HCI_Study/Blueprints/BP_GM_Study` (`GameplayStatics.GetGameMode`)))
  (if (`self.TrialStarted`)
    (`/Game/WHS_HCI_Study/Blueprints/BP_GM_Study.Trial Finished` _asbp_gm_study)
    (else
      (`/Game/WHS_HCI_Study/Blueprints/BP_GM_Study.EndTrainingTrial` _asbp_gm_study)
      (set `self.TimerStarted` true))))

(event `self.ReceiveTick`
  (params (DeltaSeconds :type "Float (single-precision)"))
  (bind (_currentboxinitialtransform_location _currentboxinitialtransform_rotation _currentboxinitialtransform_scale) (`KismetMathLibrary.BreakTransform` (`self.CurrentBoxInitialTransform`)))
  (bind _p_static_mesh_actor_ref (`/Game/Blueprints/BP_SpawnAreas/BP_Dep_Mesh_SpawnArea.P_Static Mesh Actor Ref` (`self.CurrentBoxVolume`)))
  (bind _staticmeshcomponent (`StaticMeshActor.StaticMeshComponent` (`/Game/Blueprints/BP_SpawnAreas/BP_Dep_Mesh_SpawnArea.P_Static Mesh Actor Ref` (`self.CurrentBoxVolume`))))
  (if (not (> (`KismetArrayLibrary.Array_Length` (`self.BoxTransforms`)) 0))
    (`self.Setup Box Transform Array`))
  (if (`KismetSystemLibrary.IsValid` (`self.CurrentBoxVolume`))
    (if (< (`KismetMathLibrary.Vector_Distance` (`SceneComponent.K2_GetComponentLocation` (`StaticMeshActor.StaticMeshComponent` (`/Game/Blueprints/BP_SpawnAreas/BP_Dep_Mesh_SpawnArea.P_Static Mesh Actor Ref` (`self.TargetBoxSpawnVolume`)))) (`SceneComponent.K2_GetComponentLocation` _staticmeshcomponent)) 70.0)
      (if (and (`KismetMathLibrary.NearlyEqual_TransformTransform` (`self.GetTransform` _p_static_mesh_actor_ref) (`self.CurrentBoxLastTransform`)) (< (`KismetMathLibrary.Vector_Distance` (`SceneComponent.K2_GetComponentLocation` (`StaticMeshActor.StaticMeshComponent` _p_static_mesh_actor_ref)) (`SceneComponent.K2_GetComponentLocation` (`Actor.RootComponent` (`/Game/Blueprints/BP_SpawnAreas/BP_Dep_Mesh_SpawnArea.P_Static Mesh Actor Ref` (`self.TargetBoxSpawnVolume`))))) 10.0) (not (`KismetSystemLibrary.IsValid` (`/Game/Blueprints/BP_JacoArm/Jaco.GraspedObject` (`self.Jaco`)))) (not (`self.TimerStarted`)))
        (bind _returnvalue (`KismetSystemLibrary.K2_SetTimerDelegate` (delegate `Trial Finished Timer`) 1.0))
        (bind _asbp_gm_study (cast `/Game/WHS_HCI_Study/Blueprints/BP_GM_Study` (`GameplayStatics.GetGameMode`)))
        (`/Game/WHS_HCI_Study/Blueprints/BP_GM_Study.Start Gripper Return` _asbp_gm_study _returnvalue)
        (`GameplayStatics.PlaySound2D` "/Engine/VREditor/Sounds/VR_click3.VR_click3" 0.5 1.0 0.0 null null)
        (set `self.TimerStarted` true))
      (set `self.CurrentBoxLastTransform` (`self.GetTransform` (`/Game/Blueprints/BP_SpawnAreas/BP_Dep_Mesh_SpawnArea.P_Static Mesh Actor Ref` (`self.CurrentBoxVolume`))))
      (else
        (`SceneComponent.K2_SetWorldTransform` _staticmeshcomponent (`KismetMathLibrary.MakeTransform` (+ _currentboxinitialtransform_location (0.0 0.0 20.0)) _currentboxinitialtransform_rotation _currentboxinitialtransform_scale) false false)
        (if (not (`self.ResetHappening`))
          (bind _returnvalue_2 (`KismetSystemLibrary.K2_SetTimerDelegate` (delegate `InTrialReset`) 1.0))
          (bind _asbp_gm_study_2 (cast `/Game/WHS_HCI_Study/Blueprints/BP_GM_Study` (`GameplayStatics.GetGameMode`)))
          (`/Game/WHS_HCI_Study/Blueprints/BP_GM_Study.Start Gripper Return` _asbp_gm_study_2 _returnvalue_2)
          (set `/Game/WHS_HCI_Study/Blueprints/BP_WHS_VR_Pawn.StopInput` true (`/Game/WHS_HCI_Study/Blueprints/BP_GM_Study.PlayerPawn` _asbp_gm_study_2))
          (`GameplayStatics.PlaySound2D` "/Engine/VREditor/Sounds/VR_negative.VR_negative" 0.5 1.0 0.0 null null)
          (set `self.ResetHappening` true))))))

(fn `PickBox`
  (params (SpawnBoxIndex :type Integer))
  (bind _currentboxvolume (`self.CurrentBoxVolume`))
  (bind _boxtransforms (`self.BoxTransforms`))
  (bind _returnvalue (mod SpawnBoxIndex (`KismetArrayLibrary.Array_Length` (`self.BoxSpawnVolumes`))))
  (bind _staticmeshcomponent (`StaticMeshActor.StaticMeshComponent` (`/Game/Blueprints/BP_SpawnAreas/BP_Dep_Mesh_SpawnArea.P_Static Mesh Actor Ref` _currentboxvolume)))
  (bind _output (`|GetArrayItem` (`self.BoxSpawnVolumes`) _returnvalue))
  (bind _output_2 (`|GetArrayItem` _boxtransforms _returnvalue))
  (`/Engine/EditorBlueprintResources/StandardMacros.IsValid` _currentboxvolume
    (:`Is Valid`
      (`SceneComponent.K2_SetWorldLocation` _staticmeshcomponent (0.0 0.0 0.0) false false)
      (`PrimitiveComponent.SetSimulatePhysics` _staticmeshcomponent false))
    (:`Is Not Valid`
      _))
  (`SceneComponent.K2_SetWorldTransform` (`StaticMeshActor.StaticMeshComponent` (`/Game/Blueprints/BP_SpawnAreas/BP_Dep_Mesh_SpawnArea.P_Static Mesh Actor Ref` _output)) (`KismetMathLibrary.MakeTransform` (`KismetMathLibrary.MakeVector` (.x (.location _output_2)) (.y (.location _output_2)) (+ (.z (.location _output_2)) 10.0)) (.rotation _output_2) (.scale _output_2)) false false)
  (set `self.CurrentBoxInitialTransform` (`|GetArrayItem` _boxtransforms _returnvalue))
  (set `self.CurrentBoxVolume` _output)
  (`KismetSystemLibrary.K2_SetTimer` self "SetCurrentBoxPhysics" 0.1)
  (`PrimitiveComponent.SetCollisionEnabled` (`StaticMeshActor.StaticMeshComponent` (`/Game/Blueprints/BP_SpawnAreas/BP_Dep_Mesh_SpawnArea.P_Static Mesh Actor Ref` (`self.TargetBoxSpawnVolume`))) "NoCollision"))

(fn `ResetTrial`
  (bind _jaco (`self.Jaco`))
  (if (not (== (`/Game/Blueprints/BP_JacoArm/Jaco.GraspedObject` _jaco) null))
    (`/Game/Blueprints/BP_JacoArm/Jaco.Release Grasped Object` _jaco))
  (`SceneComponent.K2_SetWorldLocation` (`StaticMeshActor.StaticMeshComponent` (`/Game/Blueprints/BP_SpawnAreas/BP_Dep_Mesh_SpawnArea.P_Static Mesh Actor Ref` (`self.CurrentBoxVolume`))) (0.0 0.0 0.0) false false))

(fn `SetCurrentBoxPhysics`
  (`PrimitiveComponent.SetSimulatePhysics` (`StaticMeshActor.StaticMeshComponent` (`/Game/Blueprints/BP_SpawnAreas/BP_Dep_Mesh_SpawnArea.P_Static Mesh Actor Ref` (`self.CurrentBoxVolume`))) true))

(fn `Setup Box Transform Array`
  (for _array_element (`self.BoxSpawnVolumes`)
    (bind _staticmeshcomponent (`StaticMeshActor.StaticMeshComponent` (`/Game/Blueprints/BP_SpawnAreas/BP_Dep_Mesh_SpawnArea.P_Static Mesh Actor Ref` _array_element)))
    (`KismetArrayLibrary.Array_Add` (`self.BoxTransforms`) (`SceneComponent.K2_GetComponentToWorld` _staticmeshcomponent))
    (`SceneComponent.K2_SetWorldLocation` _staticmeshcomponent (0.0 0.0 0.0) false false)
    (`PrimitiveComponent.SetSimulatePhysics` _staticmeshcomponent false)))

(fn `UserConstructionScript`)