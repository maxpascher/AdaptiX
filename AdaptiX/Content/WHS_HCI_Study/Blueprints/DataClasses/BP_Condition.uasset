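; BP_Condition is a data class for one HCI study condition, pairing a visualisation type and control method with its recorded results.
; It collects trial results, maps ordered NASA-TLX scores to named workload keys, and holds a Base64 audio string.
; ToJson writes the condition, nested trial results and flattened TLX fields, omitting audio.
; FromJson restores only the visualisation type and control method.
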(fn `Add Audio Base 64`
  (params (AudioBase64 :type String))
  (set `self.AudioBase64` AudioBase64))

(fn `AddNasaTLXValues`
  (params (NasaTLXValues :type "Array of Integer"))
  (for (_array_element _array_index) NasaTLXValues
    (`BlueprintMapLibrary.Map_Add` (`self.NasaTLXValues`) (select `int` _array_index :`0` "nasatlx_mental_demand" :`1` "nasatlx_physical_demand" :`2` "nasatlx_temporal_demand" :`3` "nasatlx_performance" :`4` "nasatlx_effort" :`5` "nasatlx_frustration") _array_element)))

(fn `AddTrialResult`
  (params (`Trial Result` :type "/Game/WHS_HCI_Study/Blueprints/DataClasses/BP_Trial_Results Object Reference"))
  (`KismetArrayLibrary.Array_Add` (`self.Trial Results`) `Trial Result`))

(fn `FromJson`
  (params (JsonObject :type "VaRestJsonObject Object Reference"))
  (set `self.VisualisationType` (cast `/Game/WHS_HCI_Study/Structs/VisualisationType` (`KismetMathLibrary.Conv_IntToByte` (`VaRestJsonObject.GetIntegerField` JsonObject "visualisation_type"))))
  (set `self.ControlMethod` (cast `/Game/WHS_HCI_Study/Structs/ControlMethod` (`KismetMathLibrary.Conv_IntToByte` (`VaRestJsonObject.GetIntegerField` JsonObject "control_method")))))

(fn `Get Audio Base 64`
  (returns (AudioBase64 :type String))
  (return (`self.AudioBase64`)))

(fn `GetControlMethod`
  (returns (ControlMethod :type "/Game/WHS_HCI_Study/Structs/ControlMethod Enum"))
  (return (`self.ControlMethod`)))

(fn `GetNumberOfTrials`
  (returns (ReturnValue :type Integer))
  (return (`KismetArrayLibrary.Array_Length` (`self.Trial Results`))))

(fn `GetVisualisationType`
  (returns (VisualisationType :type "/Game/WHS_HCI_Study/Structs/VisualisationType Enum"))
  (return (`self.VisualisationType`)))

(fn `ToJson`
  (returns (JsonObject :type "VaRestJsonObject Object Reference"))
  (locals (NewJsonObject :type "VaRestJsonObject Object Reference") (`Trial Result Array` :type "Array of VaRestJsonObject Object Reference") (NasaTLXJsonObject :type "VaRestJsonObject Object Reference"))
  (bind _nasatlxvalues (`self.NasaTLXValues`))
  (bind _output_get (set `local.NewJsonObject` (`|MakeJson`)))
  (`VaRestJsonObject.SetIntegerField` _output_get "visualisation_type" (`KismetMathLibrary.Conv_ByteToInt` (`self.VisualisationType`)))
  (`VaRestJsonObject.SetIntegerField` _output_get "control_method" (`KismetMathLibrary.Conv_ByteToInt` (`self.ControlMethod`)))
  (for _array_element (`self.Trial Results`)
    (`KismetArrayLibrary.Array_Add` (`local.Trial Result Array`) (`/Game/WHS_HCI_Study/Blueprints/DataClasses/BP_Trial_Results.ToJson` _array_element)))
  (`VaRestJsonObject.SetObjectArrayField` _output_get "trial_results" (`local.Trial Result Array`))
  (bind _keys (`BlueprintMapLibrary.Map_Keys` _nasatlxvalues))
  (for _array_element_2 _keys
    (bind (_value _returnvalue) (`BlueprintMapLibrary.Map_Find` _nasatlxvalues _array_element_2))
    (if _returnvalue
      (`VaRestJsonObject.SetIntegerField` _output_get _array_element_2 _value)))
  (return _output_get))