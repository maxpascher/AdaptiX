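; BP_Trial_Results is a data class that records the results of a single trial in the WHS HCI study.
; Setters store the box's spawn volume name and rotation, completion time, mode switches and trial resets.
; LogInputEvent appends type and time to parallel arrays and prints the type.
; ToJson packs these values into a JSON object, saving only the rotation's yaw and zipping the arrays into an input event list.
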(fn `LogInputEvent`
  (params (type :type String) (time :type "Float (double-precision)"))
  (`KismetArrayLibrary.Array_Add` (`self.InputEventTypes`) type)
  (`KismetArrayLibrary.Array_Add` (`self.InputEventTimes`) time)
  (`KismetSystemLibrary.PrintString` null type))

(fn `SetBoxParameters`
  (params (`Spawn Volume` :type "/Game/Blueprints/BP_SpawnAreas/BP_Dep_Mesh_SpawnArea Object Reference"))
  (set `self.Initial Box Location` (`KismetSystemLibrary.GetDisplayName` `Spawn Volume`))
  (set `self.Initial Box Rotation` (`SceneComponent.K2_GetComponentRotation` (`StaticMeshActor.StaticMeshComponent` (`/Game/Blueprints/BP_SpawnAreas/BP_Dep_Mesh_SpawnArea.P_Static Mesh Actor Ref` `Spawn Volume`)))))

(fn `SetModeSwitches`
  (params (ModeSwitches :type Integer))
  (set `self.ModeSwitches` ModeSwitches))

(fn `SetTaskCompletionTime`
  (params (TaskCompletionTime :type "Float (double-precision)"))
  (set `self.TaskCompletionTime` TaskCompletionTime))

(fn `SetTrialResets`
  (params (TrialResets :type Integer))
  (set `self.TrialResets` TrialResets))

(fn `ToJson`
  (returns (JsonObject :type "VaRestJsonObject Object Reference"))
  (locals (NewJsonObject :type "VaRestJsonObject Object Reference") (InputEvents :type "Array of VaRestJsonObject Object Reference") (InputEvent :type "VaRestJsonObject Object Reference"))
  (bind (_initial_box_rotation_roll _initial_box_rotation_pitch _initial_box_rotation_yaw) (`KismetMathLibrary.BreakRotator` (`self.Initial Box Rotation`)))
  (bind _inputevent (`local.InputEvent`))
  (bind _output_get (set `local.NewJsonObject` (`|MakeJson`)))
  (`VaRestJsonObject.SetStringField` _output_get "initial_box_location" (`self.Initial Box Location`))
  (`VaRestJsonObject.SetNumberField` _output_get "initial_box_yaw" _initial_box_rotation_yaw)
  (`VaRestJsonObject.SetNumberField` _output_get "initial_box_yaw" _initial_box_rotation_yaw)
  (`VaRestJsonObject.SetNumberField` _output_get "task_completion_time" (`self.TaskCompletionTime`))
  (`VaRestJsonObject.SetIntegerField` _output_get "mode_switches" (`self.ModeSwitches`))
  (`VaRestJsonObject.SetIntegerField` _output_get "trial_resets" (`self.TrialResets`))
  (for (_array_element _array_index) (`self.InputEventTypes`)
    (set `local.InputEvent` (`|MakeJson`))
    (`VaRestJsonObject.SetStringField` _inputevent "type" _array_element)
    (`VaRestJsonObject.SetNumberField` _inputevent "time" (`|GetArrayItem` (`self.InputEventTimes`) _array_index))
    (`KismetArrayLibrary.Array_Add` (`local.InputEvents`) _inputevent))
  (`VaRestJsonObject.SetObjectArrayField` _output_get "input_events" (`local.InputEvents`))
  (return _output_get))