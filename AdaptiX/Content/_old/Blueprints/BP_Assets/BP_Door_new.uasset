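; Physics-driven door with child-actor door and handle, given random meshes and materials on BeginPlay; in replay mode it destroys its child actors instead.
; Constraints join handle, door, frame and two trigger boxes; Tick enables door physics when the handle twists far enough, otherwise disabling it past the lock swing.
; When pulling ("Ziehen") is enabled, box overlaps constrain the handle to the overlapping component, breaking at open/closed limits or excessive distance.
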(event `self.ReceiveBeginPlay`
  (bind _returnvalue (`self.GetComponentByClass` (`ChildActorComponent.ChildActor` (`self.Door`)) "/Script/Engine.PrimitiveComponent"))
  ;[1 1 1] Randomise
  ;;[1 1 1] Randomise Door Mesh
  (bind _output_get (set `self.Door Mesh Component` (`self.GetComponentByClass` (`ChildActorComponent.ChildActor` (`self.Door`)) "/Script/Engine.StaticMeshComponent")))
  (`StaticMeshComponent.SetStaticMesh` _output_get (`KismetArrayLibrary.Array_Random` (`self.Door Meshes`)))
  ;;[1 1 1] Randomise Handle Mesh
  (bind _output_get_2 (set `self.Handle Mesh Component` (`self.GetComponentByClass` (`ChildActorComponent.ChildActor` (`self.Handle`)) "/Script/Engine.StaticMeshComponent")))
  (`StaticMeshComponent.SetStaticMesh` _output_get_2 (`KismetArrayLibrary.Array_Random` (`self.Handle Meshes`)))
  ;;[1 1 1] Randomise Door Material
  (`PrimitiveComponent.SetMaterial` (`self.Door Mesh Component`) 0 (`KismetArrayLibrary.Array_Random` (`self.Door Materials`)))
  ;;[1 1 1] Randomise Handle Material
  (`PrimitiveComponent.SetMaterial` (`self.Handle Mesh Component`) 0 (`KismetArrayLibrary.Array_Random` (`self.Handle Materials`)))
  ;[1 1 1] Destroy Child Actors when Replay
  (`Storage.loadInitFile`)
  (if (`Storage.GetPlayReplay`)
    (`self.K2_DestroyActor` (`self.GetAllChildActors` true)) ; In replay: Destroy child actors as they are created by replay logic
    (else
      ;[1 1 1] Simulate Physic for Child Actors
      (for _array_element (`self.GetAllChildActors` true)
        (`PrimitiveComponent.SetSimulatePhysics` (`self.GetComponentByClass` _array_element "/Script/Engine.PrimitiveComponent") true)
        ;[1 1 1] Link Constraints
        ;;[1 1 1] Link Components
        (`PhysicsConstraintComponent.SetConstrainedComponents` (`self.Handle_Constraint`) (`self.Handle Mesh Component`) "None" (`self.Door Mesh Component`) "None")
        (`PhysicsConstraintComponent.SetConstrainedComponents` (`self.Door_Constraint`) (`self.Door Mesh Component`) "None" (`self.StaticMeshComponent`) "None")
        ;;[1 1 1] Link Collision Boxes to Handle
        (`PhysicsConstraintComponent.SetConstrainedComponents` (`self.Box1_constraint`) (`self.Box1`) "None" (`self.Handle Mesh Component`) "None")
        (`PhysicsConstraintComponent.SetConstrainedComponents` (`self.Box2_constraint`) (`self.Box2`) "None" (`self.Handle Mesh Component`) "None")
        ;[1 1 1] Physic Settings Door and Handle
        ;;[1 1 1] Set Door Physics and Gravity Off
        (bind _output_get_3 (set `self.Door Primitive Component` _returnvalue))
        (`PrimitiveComponent.SetSimulatePhysics` _returnvalue false)
        (`PrimitiveComponent.SetSimulatePhysics` _output_get_3 false)
        (`PrimitiveComponent.SetEnableGravity` _output_get_3 false)
        (`PrimitiveComponent.SetLinearDamping` _output_get_3 5.0)
        ;;[1 1 1] Set Gravity Off and Mass for Handle
        (bind _output_get_4 (set `self.Handle Primitive Component` (`self.GetComponentByClass` (`ChildActorComponent.ChildActor` (`self.Handle`)) "/Script/Engine.PrimitiveComponent")))
        (`PrimitiveComponent.SetEnableGravity` _output_get_4 false)
        (`PrimitiveComponent.SetMassOverrideInKg` (`self.Handle Primitive Component`) "None" 5.0 true)
        ;;[1 1 1] Set Mass Door
        (`PrimitiveComponent.SetMassOverrideInKg` (`self.Door Primitive Component`) "None" 5.0 true)))))

(event `self.ReceiveTick`
  (params (DeltaSeconds :type "Float (single-precision)"))
  (`|ExecutionSequence`
    (:`then_0`
      ;[1 1 1] Handle and Lock Mechanic
      ;;[1 1 1] Set Door simulate Physic if Handle Rotation > Min Rotation for Open
      (if (> (`PhysicsConstraintComponent.GetCurrentTwist` (`self.Handle_Constraint`)) (`self.Min Rot for Open`))
        (`PrimitiveComponent.SetSimulatePhysics` (`self.Door Primitive Component`) true)
        (else
          ;;[1 1 1] Set Door simulate no Physics if Door Rotation > Lock Position
          (if (> (`PhysicsConstraintComponent.GetCurrentSwing1` (`self.Door_Constraint`)) (`self.Lock Position Door`))
            (`PrimitiveComponent.SetSimulatePhysics` (`self.Door Primitive Component`) false)))))
    (:`then_1`
      ;[1 1 1] Pull Mechanic
      (`|ExecutionSequence`
        (:`then_0`
          ;;[1 1 1] Kann die Tür gezogen werden?
          (if (`self.Ziehen`)
            (`|ExecutionSequence`
              (:`then_0`
                ;;[1 1 1] Break Link when Open
                (if (`self.Link Open`)
                  (if (< (`PhysicsConstraintComponent.GetCurrentSwing1` (`self.Door_Constraint`)) (`self.Open Position for Door`))
                    (`/Engine/EditorBlueprintResources/StandardMacros.DoOnce` false
                      (:`Completed`
                        (`PhysicsConstraintComponent.BreakConstraint` (`self.Pull Constraint`))
                        (`KismetSystemLibrary.PrintString` "Broken")
                        (set `self.Link Open` false))))))
              (:`then_1`
                ;;[1 1 1] Break Link when Closed
                (if (`self.Link Close`)
                  (if (>= (`PhysicsConstraintComponent.GetCurrentSwing1` (`self.Door_Constraint`)) (`self.Lock Position Door`))
                    (`/Engine/EditorBlueprintResources/StandardMacros.DoOnce` false
                      (:`Completed`
                        (`PhysicsConstraintComponent.BreakConstraint` (`self.Pull Constraint`))
                        (`KismetSystemLibrary.PrintString` "Broken")
                        (set `self.Link Close` false)))))))))
        (:`then_1`
          ;;[1 1 1] Is linked?
          (if (or (`self.Link Open`) (`self.Link Close`))
            ;;[1 1 1] Break if true
            (if (> (`KismetMathLibrary.VSize` (- (`SceneComponent.K2_GetComponentLocation` (`self.Handle Mesh Component`)) (`SceneComponent.K2_GetComponentLocation` (`self.Overlapped Component`)))) (`self.Break Distance`))
              (`PhysicsConstraintComponent.BreakConstraint` (`self.Pull Constraint`))
              (`KismetSystemLibrary.PrintString` "Too far away")
              (set `self.Link Open` false)
              (set `self.Link Close` false)
              ;;[1 1 1] Reset Link Option
              (`|ExecutionSequence`
                (:`then_0`
                  (goto _label :!via `Reset`))
                (:`then_1`
                  (goto _label_2 :!via `Reset`))))))))))

(event `self.Box1.OnComponentBeginOverlap`
  (params (OverlappedComponent :type "PrimitiveComponent Object Reference") (OtherActor :type "Actor Object Reference") (OtherComp :type "PrimitiveComponent Object Reference") (OtherBodyIndex :type Integer) (bFromSweep :type Boolean) (SweepResult :type "HitResult Structure (by ref)"))
  ;[1 1 1] Pull Mechanic
  ;;[1 1 1] Open Door by Pulling
  (bind _output_get (set `self.Overlapped Component` OtherComp))
  (if (`self.Ziehen`)
    (`/Engine/EditorBlueprintResources/StandardMacros.DoOnce` false :!label _label
      (:`Completed`
        (`PhysicsConstraintComponent.SetConstrainedComponents` (`self.Pull Constraint`) (`self.Handle Mesh Component`) "None" _output_get "None")
        (`KismetSystemLibrary.PrintString` "Connected Open")
        (set `self.Link Open` true)))))

(event `self.Box2.OnComponentBeginOverlap`
  (params (OverlappedComponent :type "PrimitiveComponent Object Reference") (OtherActor :type "Actor Object Reference") (OtherComp :type "PrimitiveComponent Object Reference") (OtherBodyIndex :type Integer) (bFromSweep :type Boolean) (SweepResult :type "HitResult Structure (by ref)"))
  ;[1 1 1] Pull Mechanic
  ;;[1 1 1] Close Door by Pulling
  (bind _output_get (set `self.Overlapped Component` OtherComp))
  (if (`self.Ziehen`)
    (`/Engine/EditorBlueprintResources/StandardMacros.DoOnce` false :!label _label_2
      (:`Completed`
        (`PhysicsConstraintComponent.SetConstrainedComponents` (`self.Pull Constraint`) (`self.Handle Mesh Component`) "None" _output_get "None")
        (`KismetSystemLibrary.PrintString` "Connected Close")
        (set `self.Link Close` true)
        (`PrimitiveComponent.SetMassOverrideInKg` (`self.Handle Primitive Component`) "None" 0.1 true)
        (`PrimitiveComponent.SetMassOverrideInKg` (`self.Door Primitive Component`) "None" 0.1 true)))))

(fn `UserConstructionScript`)