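; Physics-driven door with a turnable handle and randomised meshes and materials, built from child actors linked by physics constraints at BeginPlay.
; Each tick, handle twist unlatches the door by enabling its physics, which switches off again when the swing returns to the lock position.
; When pulling is enabled, two handle-mounted boxes constrain the overlapping component to the handle to open or close the door, releasing at swing limits or excessive distance.
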(event `self.ReceiveBeginPlay`
  (bind _returnvalue (`self.GetComponentByClass` (`ChildActorComponent.ChildActor` (`self.Door`)) "/Script/Engine.PrimitiveComponent"))
  (bind _output_get (set `self.Door Mesh Component` (`self.GetComponentByClass` (`ChildActorComponent.ChildActor` (`self.Door`)) "/Script/Engine.StaticMeshComponent")))
  (`StaticMeshComponent.SetStaticMesh` _output_get (`KismetArrayLibrary.Array_Random` (`self.Door Meshes`)))
  (bind _output_get_2 (set `self.Handle Mesh Component` (`self.GetComponentByClass` (`ChildActorComponent.ChildActor` (`self.Handle`)) "/Script/Engine.StaticMeshComponent")))
  (`StaticMeshComponent.SetStaticMesh` _output_get_2 (`KismetArrayLibrary.Array_Random` (`self.Handle Meshes`)))
  (`PrimitiveComponent.SetMaterial` (`self.Door Mesh Component`) 0 (`KismetArrayLibrary.Array_Random` (`self.Door Materials`)))
  (`PrimitiveComponent.SetMaterial` (`self.Handle Mesh Component`) 0 (`KismetArrayLibrary.Array_Random` (`self.Handle Materials`)))
  (`PrimitiveComponent.SetMaterial` (`self.StaticMeshComponent`) 0 (`KismetArrayLibrary.Array_Random` (`self.Frame Materials`)))
  (for _array_element (`self.GetAllChildActors` true)
    (`PrimitiveComponent.SetSimulatePhysics` (`self.GetComponentByClass` _array_element "/Script/Engine.PrimitiveComponent") true))
  (`PhysicsConstraintComponent.SetConstrainedComponents` (`self.Handle_Constraint`) (`self.Handle Mesh Component`) "None" (`self.Door Mesh Component`) "None")
  (`PhysicsConstraintComponent.SetConstrainedComponents` (`self.Door_Constraint`) (`self.Door Mesh Component`) "None" (`self.StaticMeshComponent`) "None")
  (`PhysicsConstraintComponent.SetConstraintReferenceFrame` (`self.Door_Constraint`) "Frame1" (`KismetMathLibrary.MakeTransform` (0.0 0.0 0.0) (`KismetMathLibrary.MakeRotator` 0.0 0.0 (* -1 (`self.InitalDoorAngle`))))) ; compensate for initial door angle
  (`PhysicsConstraintComponent.SetConstrainedComponents` (`self.Box1_constraint`) (`self.Box1`) "None" (`self.Handle Mesh Component`) "None")
  (`PhysicsConstraintComponent.SetConstrainedComponents` (`self.Box2_constraint`) (`self.Box2`) "None" (`self.Handle Mesh Component`) "None")
  (bind _output_get_3 (set `self.Door Primitive Component` _returnvalue))
  (`PrimitiveComponent.SetSimulatePhysics` _returnvalue (!= (`self.InitalDoorAngle`) 0.0))
  (`PrimitiveComponent.SetSimulatePhysics` _output_get_3 (!= (`self.InitalDoorAngle`) 0.0))
  (`PrimitiveComponent.SetEnableGravity` _output_get_3 false)
  (`PrimitiveComponent.SetLinearDamping` _output_get_3 5.0)
  (bind _output_get_4 (set `self.Handle Primitive Component` (`self.GetComponentByClass` (`ChildActorComponent.ChildActor` (`self.Handle`)) "/Script/Engine.PrimitiveComponent")))
  (`PrimitiveComponent.SetEnableGravity` _output_get_4 false)
  (`PrimitiveComponent.SetMassOverrideInKg` (`self.Handle Primitive Component`) "None" 5.0 true)
  (`PrimitiveComponent.SetMassOverrideInKg` (`self.Door Primitive Component`) "None" 5.0 true))

(event `self.ReceiveTick`
  (params (DeltaSeconds :type "Float (single-precision)"))
  (`|ExecutionSequence`
    (:`then_0`
      (if (or (> (`PhysicsConstraintComponent.GetCurrentTwist` (`self.Handle_Constraint`)) (`self.Min Rot for Open`)) false)
        (`PrimitiveComponent.SetSimulatePhysics` (`self.Door Primitive Component`) true)
        (else
          (`PrimitiveComponent.SetSimulatePhysics` (`self.Door Primitive Component`) (< (`PhysicsConstraintComponent.GetCurrentSwing1` (`self.Door_Constraint`)) (`self.Lock Position Door`))))))
    (:`then_1`
      (`|ExecutionSequence`
        (:`then_0`
          (if (`self.Ziehen`)
            (`|ExecutionSequence`
              (:`then_0`
                (if (`self.Link Open`)
                  (if (< (`PhysicsConstraintComponent.GetCurrentSwing1` (`self.Door_Constraint`)) (`self.Open Position for Door`))
                    (`/Engine/EditorBlueprintResources/StandardMacros.DoOnce` false
                      (:`Completed`
                        (`PhysicsConstraintComponent.BreakConstraint` (`self.Pull Constraint`))
                        (`KismetSystemLibrary.PrintString` "Broken")
                        (set `self.Link Open` false))))))
              (:`then_1`
                (if (`self.Link Close`)
                  (if (>= (`PhysicsConstraintComponent.GetCurrentSwing1` (`self.Door_Constraint`)) (`self.Lock Position Door`))
                    (`/Engine/EditorBlueprintResources/StandardMacros.DoOnce` false
                      (:`Completed`
                        (`PhysicsConstraintComponent.BreakConstraint` (`self.Pull Constraint`))
                        (`KismetSystemLibrary.PrintString` "Broken")
                        (set `self.Link Close` false)))))))))
        (:`then_1`
          (if (or (`self.Link Open`) (`self.Link Close`))
            (if (> (`KismetMathLibrary.VSize` (- (`SceneComponent.K2_GetComponentLocation` (`self.Handle Mesh Component`)) (`SceneComponent.K2_GetComponentLocation` (`self.Overlapped Component`)))) (`self.Break Distance`))
              (`PhysicsConstraintComponent.BreakConstraint` (`self.Pull Constraint`))
              (`KismetSystemLibrary.PrintString` "Too far away")
              (set `self.Link Open` false)
              (set `self.Link Close` false)
              (`|ExecutionSequence`
                (:`then_0`
                  (goto _label_2 :!via `Reset`))
                (:`then_1`
                  (goto _label :!via `Reset`))))))))))

(event `self.Box2.OnComponentBeginOverlap`
  (params (OverlappedComponent :type "PrimitiveComponent Object Reference") (OtherActor :type "Actor Object Reference") (OtherComp :type "PrimitiveComponent Object Reference") (OtherBodyIndex :type Integer) (bFromSweep :type Boolean) (SweepResult :type "HitResult Structure (by ref)"))
  (bind _output_get (set `self.Overlapped Component` OtherComp))
  (if (`self.Ziehen`)
    (`/Engine/EditorBlueprintResources/StandardMacros.DoOnce` false :!label _label
      (:`Completed`
        (`PhysicsConstraintComponent.SetConstrainedComponents` (`self.Pull Constraint`) (`self.Handle Mesh Component`) "None" _output_get "None")
        (`KismetSystemLibrary.PrintString` "Connected Close")
        (set `self.Link Close` true)
        (`PrimitiveComponent.SetMassOverrideInKg` (`self.Handle Primitive Component`) "None" 0.1 true)
        (`PrimitiveComponent.SetMassOverrideInKg` (`self.Door Primitive Component`) "None" 0.1 true)))))

(event `self.Box1.OnComponentBeginOverlap`
  (params (OverlappedComponent :type "PrimitiveComponent Object Reference") (OtherActor :type "Actor Object Reference") (OtherComp :type "PrimitiveComponent Object Reference") (OtherBodyIndex :type Integer) (bFromSweep :type Boolean) (SweepResult :type "HitResult Structure (by ref)"))
  (bind _output_get (set `self.Overlapped Component` OtherComp))
  (if (`self.Ziehen`)
    (`/Engine/EditorBlueprintResources/StandardMacros.DoOnce` false :!label _label_2
      (:`Completed`
        (`PhysicsConstraintComponent.SetConstrainedComponents` (`self.Pull Constraint`) (`self.Handle Mesh Component`) "None" _output_get "None")
        (`KismetSystemLibrary.PrintString` "Connected Open")
        (set `self.Link Open` true)))))

(fn `UserConstructionScript`
  (`SceneComponent.K2_SetRelativeRotation` (`self.Door`) (`KismetMathLibrary.MakeRotator` 0.0 0.0 (* -1 (`self.InitalDoorAngle`))) false true))