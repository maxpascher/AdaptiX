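; Spawn area that, on BeginPlay, places one random parent mesh on its box floor and optionally scatters child meshes just above it.
; Parent and children get configurable transforms, segmentation and graspability tags, static or physics-simulated collision, optional random materials and mass overrides.
; Child count is fixed or random, with positions offset from the parent's spawn point within set extents.
; The construction script previews a random parent and child through visualiser meshes.
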(event `self.ReceiveBeginPlay`
  (bind _p_static_mesh_actor_ref (`self.P_Static Mesh Actor Ref`))
  (bind _number_children (`self.Number Children`))
  (bind _c_static_mesh_actor_ref (`self.C_Static Mesh Actor Ref`))
  (bind _c_static_mesh_actor_ref_2 (`self.C_Static Mesh Actor Ref`))
  (bind _p_static_mesh_actor_ref_2 (`self.P_Static Mesh Actor Ref`))
  ;[0 0 0] Spawn a parent mesh with a randomly selected number of child meshes from a random selection of meshes on top
  (if (!= (`KismetArrayLibrary.Array_Length` (`self.P_Meshes`)) 0)
    (`|ExecutionSequence`
      (:`then_0`
        ;;[0.09896 0.09896 0.09896] Parent mesh
        ;;;[1 1 1] Get Position in Box
        (bind _output_get (set `self.P_Position` (`self.Get Random Point in Box`)))
        (bind _returnvalue (`|SpawnActorFromClass` "/Script/Engine.StaticMeshActor" (`KismetMathLibrary.MakeTransform` _output_get (`KismetMathLibrary.MakeRotator` (`KismetMathLibrary.RandomFloatInRange` (`self.P_Min Degree Roll Rot`) (`self.P_Max Degree Roll Rot`)) (`KismetMathLibrary.RandomFloatInRange` (`self.P_Min Degree Pitch Rot`) (`self.P_Max Degree Pitch Rot`)) (`KismetMathLibrary.RandomFloatInRange` (`self.P_Min Degree Yaw Rot`) (`self.P_Max Degree Yaw Rot`))) (`self.P_Scale`)) "AdjustIfPossibleButDontSpawnIfColliding" "OverrideRootScale" null null))
        (bind _output_get_2 (set `self.P_Static Mesh Actor Ref` _returnvalue))
        (`StaticMeshComponent.SetStaticMesh` (`StaticMeshActor.StaticMeshComponent` _output_get_2) (`KismetArrayLibrary.Array_Random` (`self.P_Meshes`))) ; Set the Mesh of this Actor
        ;;;[0.3802 0.3802 0.3802] Determine, if graspable
        (if (`self.P_Graspable`)
          (set `self.P_Grasp Tag` "Graspable")
          (else
            (set `self.P_Grasp Tag` "UnGraspable")))
        (set `Actor.Tags` (`|MakeArray` (`self.P_Segmentation Tag`) (`self.P_Grasp Tag`)) (`self.P_Static Mesh Actor Ref`))
        ;;;[1 1 1] Set Collision and Physics
        (if (`self.P_Static`)
          (`self.Collision and Physic Settings Static` _p_static_mesh_actor_ref _p_static_mesh_actor_ref _p_static_mesh_actor_ref)
          (else
            (`self.Collision and Physic Settings Moveable` _p_static_mesh_actor_ref_2 _p_static_mesh_actor_ref_2 _p_static_mesh_actor_ref_2)))
        (if (`self.P_Material from Texture`)
          ;;;[1 1 1] Set Random Material from Texture
          (`/Game/Makros/MacroLibrary.Random Material Texture` (`StaticMeshActor.StaticMeshComponent` (`self.P_Static Mesh Actor Ref`))
            (:`Exec Out`
              _))
          (elif (`self.P_Material from Array`)
            ;;;[0.3802 0.3802 0.3802] Set Random Material from Array
            (`/Game/Makros/MacroLibrary.Random Material Array` (`StaticMeshActor.StaticMeshComponent` (`self.P_Static Mesh Actor Ref`)) (`self.P_Material Array`)
              (:`Exec Out`
                _))))
        ;[1 1 1] Set Parent Mass if aplicable
        (if (and (!= (`self.P_OverwriteWeight`) 0.0) (not (`self.P_Static`)))
          (`PrimitiveComponent.SetMassOverrideInKg` (`StaticMeshActor.StaticMeshComponent` (`self.P_Static Mesh Actor Ref`)) "None" (`self.P_OverwriteWeight`) true)))
      (:`then_1`
        (if (`self.Spawn Children`)
          ;;[0.09896 0.09896 0.09896] Spawn random number of children from a variety of meshes
          ;;;[1 1 1] Loop for Child Counter
          (for _ (range 1 (+ (`KismetMathLibrary.SelectInt` (`KismetMathLibrary.RandomIntegerInRange` (`KismetMathLibrary.SelectInt` 0 1 (`self.AllowZeroChildren`)) _number_children) _number_children (`self.RandomiseChildNumber`)) 1))
            (bind _returnvalue_2 (`|SpawnActorFromClass` "/Script/Engine.StaticMeshActor" (`KismetMathLibrary.MakeTransform` (+ (`self.P_Position`) (`KismetMathLibrary.RandomPointInBoundingBox` (0.0 0.0 7.0) (`KismetMathLibrary.MakeVector` (`self.C_Extent X`) (`self.C_Extent Y`)))) (`KismetMathLibrary.MakeRotator` 0.0 0.0 (`KismetMathLibrary.RandomFloatInRange` (`self.C_Min Degree Yaw Rot`) (`self.C_Max Degree Yaw Rot`))) (`self.C_Scale`)) "AdjustIfPossibleButAlwaysSpawn" "OverrideRootScale" null null))
            (bind _output_get_3 (set `self.C_Static Mesh Actor Ref` _returnvalue_2))
            (`StaticMeshComponent.SetStaticMesh` (`StaticMeshActor.StaticMeshComponent` _output_get_3) (`KismetArrayLibrary.Array_Random` (`self.C_Meshes`))) ; Set the Mesh of this Actor
            ;;;[0.3802 0.3802 0.3802] Determine, if actor is graspable
            (set `self.C_Grasp Tag` (select `bool` (`self.C_Graspable`) :`false` "UnGraspable" :`true` "Graspable" :!type "Name"))
            (set `Actor.Tags` (`|MakeArray` (`self.C_Segmentation Tag`) (`self.C_Grasp Tag`)) (`self.C_Static Mesh Actor Ref`))
            ;;;[1 1 1] Set Collision and Physics
            (if (`self.C_Static`)
              (`self.Collision and Physic Settings Static` _c_static_mesh_actor_ref_2 _c_static_mesh_actor_ref_2 _c_static_mesh_actor_ref_2)
              (else
                (`self.Collision and Physic Settings Moveable` _c_static_mesh_actor_ref _c_static_mesh_actor_ref _c_static_mesh_actor_ref)))
            (if (`self.C_Material from Texture`)
              ;;;[1 1 1] Set Random Material from Texture
              (`/Game/Makros/MacroLibrary.Random Material Texture` (`StaticMeshActor.StaticMeshComponent` (`self.C_Static Mesh Actor Ref`))
                (:`Exec Out`
                  _))
              (elif (`self.C_Material from Array`)
                ;;;[0.3802 0.3802 0.3802] Set Random Material from Array
                (`/Game/Makros/MacroLibrary.Random Material Array` (`StaticMeshActor.StaticMeshComponent` (`self.C_Static Mesh Actor Ref`)) (`self.C_Material Array`)
                  (:`Exec Out`
                    _))))
            ;[1 1 1] Set Child Mass if aplicable
            (if (and (!= (`self.C_OverwriteWeight`) 0.0) (not (`self.C_Static`)))
              (`PrimitiveComponent.SetMassOverrideInKg` (`StaticMeshActor.StaticMeshComponent` (`self.C_Static Mesh Actor Ref`)) "None" (`self.C_OverwriteWeight`) true))))))))

(fn `Collision and Physic Settings Moveable`
  (params (self2 :type "StaticMeshActor Object Reference") (self3 :type "Actor Object Reference") (self4 :type "StaticMeshActor Object Reference"))
  (bind _staticmeshcomponent (`StaticMeshActor.StaticMeshComponent` self4))
  (`StaticMeshActor.SetMobility` self2 "Movable")
  (`self.SetActorEnableCollision` self3 true)
  (`PrimitiveComponent.SetSimulatePhysics` _staticmeshcomponent true)
  (`PrimitiveComponent.SetNotifyRigidBodyCollision` _staticmeshcomponent true)
  (set `PrimitiveComponent.bGenerateOverlapEvents` true _staticmeshcomponent)
  (`PrimitiveComponent.SetCollisionResponseToAllChannels` _staticmeshcomponent "ECR_Block")
  (`PrimitiveComponent.SetCollisionObjectType` _staticmeshcomponent "ECC_PhysicsBody"))

(fn `Collision and Physic Settings Static`
  (params (self2 :type "StaticMeshActor Object Reference") (self3 :type "Actor Object Reference") (self4 :type "StaticMeshActor Object Reference"))
  (bind _staticmeshcomponent (`StaticMeshActor.StaticMeshComponent` self4))
  (`StaticMeshActor.SetMobility` self2 "Static")
  (`self.SetActorEnableCollision` self3 true)
  (`PrimitiveComponent.SetSimulatePhysics` _staticmeshcomponent false)
  (`PrimitiveComponent.SetNotifyRigidBodyCollision` _staticmeshcomponent true)
  (set `PrimitiveComponent.bGenerateOverlapEvents` true _staticmeshcomponent)
  (`PrimitiveComponent.SetCollisionResponseToAllChannels` _staticmeshcomponent "ECR_Block")
  (`PrimitiveComponent.SetCollisionObjectType` _staticmeshcomponent "ECC_WorldStatic"))

(fn `Get Random Point in Box`
  (returns (ReturnValue :type "Vector Structure"))
  (bind (_returnvalue_x _returnvalue_y _returnvalue_z) (`KismetMathLibrary.BreakVector` (`BoxComponent.GetScaledBoxExtent` (`self.Spawn Volume`))))
  (return (+ (`KismetMathLibrary.MakeVector` (`KismetMathLibrary.RandomFloatInRange` (* _returnvalue_x -1.0) _returnvalue_x) (`KismetMathLibrary.RandomFloatInRange` (* _returnvalue_y -1.0) _returnvalue_y) (* _returnvalue_z -1.0)) (`self.K2_GetActorLocation`))))

(fn `UserConstructionScript`
  (bind _c_meshes (`self.C_Meshes`))
  (bind _ui_visualiser_child (`self.UI Visualiser Child`))
  (bind _ui_visualiser (`self.UI Visualiser`))
  ;[1 1 1] Visualise Parent
  (if (> (`KismetArrayLibrary.Array_Length` (`self.P_Meshes`)) 0)
    (`StaticMeshComponent.SetStaticMesh` _ui_visualiser (`KismetArrayLibrary.Array_Random` (`self.P_Meshes`)))
    (`SceneComponent.K2_SetWorldTransform` (`self.UI Visualiser`) (`KismetMathLibrary.MakeTransform` (`self.Get Random Point in Box`) (`KismetMathLibrary.MakeRotator` (`KismetMathLibrary.RandomFloatInRange` (`self.P_Min Degree Roll Rot`) (`self.P_Max Degree Roll Rot`)) (`KismetMathLibrary.RandomFloatInRange` (`self.P_Min Degree Pitch Rot`) (`self.P_Max Degree Pitch Rot`)) (`KismetMathLibrary.RandomFloatInRange` (`self.P_Min Degree Yaw Rot`) (`self.P_Max Degree Yaw Rot`))) (`self.P_Scale`)) false true)
    (if (> (`KismetArrayLibrary.Array_Length` _c_meshes) 0)
      (`StaticMeshComponent.SetStaticMesh` _ui_visualiser_child (`KismetArrayLibrary.Array_Random` _c_meshes))
      (`SceneComponent.K2_SetWorldTransform` (`self.UI Visualiser Child`) (`KismetMathLibrary.MakeTransform` (+ (`SceneComponent.K2_GetComponentLocation` (`self.UI Visualiser`)) (`KismetMathLibrary.RandomPointInBoundingBox` (0.0 0.0 7.0) (`KismetMathLibrary.MakeVector` (`self.C_Extent X`) (`self.C_Extent Y`)))) (`KismetMathLibrary.MakeRotator` 0.0 0.0 (`KismetMathLibrary.RandomFloatInRange` (`self.C_Min Degree Yaw Rot`) (`self.C_Max Degree Yaw Rot`))) (`self.C_Scale`)) false false)
      (else
        (`StaticMeshComponent.SetStaticMesh` _ui_visualiser_child null)))
    (else
      (`StaticMeshComponent.SetStaticMesh` _ui_visualiser null))))