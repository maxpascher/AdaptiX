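; Spawn area actor that places one actor of a randomly picked class on its box volume's floor at BeginPlay.
; The spawn gets a random rotation within set ranges, a set scale, segmentation and graspability tags, and an optional mass override for movable static mesh actors.
; The construction script previews a separately randomized result through a child actor, cleared at play.
; Random points ignore the area's rotation, using only scaled extents and actor location.
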(event `self.ReceiveBeginPlay`
  ;[0 0 0] Spawn a number of Actors from a determinable number of Classes
  (`ChildActorComponent.SetChildActorClass` (`self.UI Visualiser Child Actor`) null) ; Stop Child actor spawning only used for visualisation
  (bind _output_get (set `self.TargetBlueprint` (`KismetArrayLibrary.Array_Random` (`self.Classes to Spawn from`))))
  (if (!= _output_get null)
    (bind _returnvalue (`|SpawnActorFromClass` _output_get (`KismetMathLibrary.MakeTransform` (`self.Get Random Point in Box`) (`KismetMathLibrary.MakeRotator` (`KismetMathLibrary.RandomFloatInRange` (`self.Min Degree Roll Rotation`) (`self.Max Degree Roll Rotation`)) (`KismetMathLibrary.RandomFloatInRange` (`self.Min Degree Pitch Rotation`) (`self.Max Degree Pitch Rotation`)) (`KismetMathLibrary.RandomFloatInRange` (`self.Min Degree Yaw Rotation`) (`self.Max Degree Yaw Rotation`))) (`self.Scale`)) "AdjustIfPossibleButAlwaysSpawn" "OverrideRootScale" null null))
    ;;[0 0 0] Determine, if actor is graspable
    (if (`self.Graspable`)
      (set `self.Grasp Tag` "Graspable")
      (else
        (set `self.Grasp Tag` "UnGraspable")))
    (`KismetArrayLibrary.Array_Append` (`Actor.Tags` _returnvalue) (`|MakeArray` (`self.Segmentation Tag`) (`self.Grasp Tag`)))
    ;[1 1 1] Set Weight if so defined
    (bind _asstatic_mesh_actor (cast `StaticMeshActor` _returnvalue))
    (bind _staticmeshcomponent (`StaticMeshActor.StaticMeshComponent` _asstatic_mesh_actor))
    (if (and (`|EnumEquality` (`SceneComponent.Mobility` _staticmeshcomponent) "Movable") (!= (`self.OverwriteWeight`) 0.0))
      (`PrimitiveComponent.SetMassOverrideInKg` _staticmeshcomponent "None" (`self.OverwriteWeight`) true))))

(fn `Get Random Point in Box`
  (returns (ReturnValue :type "Vector Structure"))
  (bind (_returnvalue_x _returnvalue_y _returnvalue_z) (`KismetMathLibrary.BreakVector` (`BoxComponent.GetScaledBoxExtent` (`self.Spawn Volume`))))
  (return (+ (`KismetMathLibrary.MakeVector` (`KismetMathLibrary.RandomFloatInRange` (* _returnvalue_x -1.0) _returnvalue_x) (`KismetMathLibrary.RandomFloatInRange` (* _returnvalue_y -1.0) _returnvalue_y) (* _returnvalue_z -1.0)) (`self.K2_GetActorLocation`))))

(fn `UserConstructionScript`
  (bind _classes_to_spawn_from (`self.Classes to Spawn from`))
  (bind _ui_visualiser_child_actor (`self.UI Visualiser Child Actor`))
  (if (> (`KismetArrayLibrary.Array_Length` _classes_to_spawn_from) 0)
    (`ChildActorComponent.SetChildActorClass` _ui_visualiser_child_actor (`KismetArrayLibrary.Array_Random` _classes_to_spawn_from))
    (`SceneComponent.K2_SetWorldTransform` (`self.UI Visualiser Child Actor`) (`KismetMathLibrary.MakeTransform` (`self.Get Random Point in Box`) (`KismetMathLibrary.MakeRotator` (`KismetMathLibrary.RandomFloatInRange` (`self.Min Degree Roll Rotation`) (`self.Max Degree Roll Rotation`)) (`KismetMathLibrary.RandomFloatInRange` (`self.Min Degree Pitch Rotation`) (`self.Max Degree Pitch Rotation`)) (`KismetMathLibrary.RandomFloatInRange` (`self.Min Degree Yaw Rotation`) (`self.Max Degree Yaw Rotation`))) (`self.Scale`)) false true)
    (else
      (`ChildActorComponent.SetChildActorClass` _ui_visualiser_child_actor null))))