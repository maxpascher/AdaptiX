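; Spawn area that, on BeginPlay, attempts to spawn one StaticMeshActor with a random mesh from its list.
; It uses a random rotation and point on the box's bottom plane, skipping the spawn if collision can't be resolved.
; The actor gets segmentation and graspability tags, static or physics-simulated collision settings, optional random material and mass override.
; The construction script previews an independently randomized mesh and transform through UIVisualiser.
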(event `self.ReceiveBeginPlay`
  (bind _static_mesh_actor_ref (`self.Static Mesh Actor Ref`))
  (bind _static_mesh_actor_ref_2 (`self.Static Mesh Actor Ref`))
  ;[0 0 0] Spawn a number of Actors from a determinable number of Meshes
  (if (!= (`KismetArrayLibrary.Array_Length` (`self.Meshes to Spawn from`)) 0)
    (bind _returnvalue (`|SpawnActorFromClass` "/Script/Engine.StaticMeshActor" (`KismetMathLibrary.MakeTransform` (`self.Get Random Point in Box`) (`KismetMathLibrary.MakeRotator` (`KismetMathLibrary.RandomFloatInRange` (`self.Min Degree Roll Rotation`) (`self.Max Degree Roll Rotation`)) (`KismetMathLibrary.RandomFloatInRange` (`self.Min Degree Pitch Rotation`) (`self.Max Degree Pitch Rotation`)) (`KismetMathLibrary.RandomFloatInRange` (`self.Min Degree Yaw Rotation`) (`self.Max Degree Yaw Rotation`))) (`self.Scale`)) "AdjustIfPossibleButDontSpawnIfColliding" "OverrideRootScale" null null))
    ;;[0.09896 0.09896 0.09896] Mesh Randomization
    (bind _output_get (set `self.Static Mesh Actor Ref` _returnvalue))
    (`StaticMeshComponent.SetStaticMesh` (`StaticMeshActor.StaticMeshComponent` _output_get) (`KismetArrayLibrary.Array_Random` (`self.Meshes to Spawn from`))) ; Set the Mesh of this Actor
    ;;[0.09896 0.09896 0.09896] Determine, if graspable
    (if (`self.Graspable`)
      (set `self.Grasp Tag` "Graspable")
      (else
        (set `self.Grasp Tag` "UnGraspable")))
    (set `Actor.Tags` (`|MakeArray` (`self.Segmentation Tag`) (`self.Grasp Tag`)) (`self.Static Mesh Actor Ref`))
    ;;[1 1 1] Set Collision and Physics
    (if (`self.Static`)
      (`self.Collision and Physic Settings Static` _static_mesh_actor_ref_2 _static_mesh_actor_ref_2 _static_mesh_actor_ref_2)
      (else
        (`self.Collision and Physic Settings Moveable` _static_mesh_actor_ref _static_mesh_actor_ref _static_mesh_actor_ref)))
    (if (`self.Material from Texture`)
      ;;[1 1 1] Set Random Material from Texture
      (`/Game/Makros/MacroLibrary.Random Material Texture` (`StaticMeshActor.StaticMeshComponent` (`self.Static Mesh Actor Ref`))
        (:`Exec Out`
          _))
      (elif (`self.Material from Array`)
        ;;[0.09896 0.09896 0.09896] Set Random Material
        (`/Game/Makros/MacroLibrary.Random Material Array` (`StaticMeshActor.StaticMeshComponent` (`self.Static Mesh Actor Ref`)) (`self.Material Array`)
          (:`Exec Out`
            _))))
    ;[1 1 1] Set Weight if applicable
    (if (and (!= (`self.OverwriteWeight`) 0.0) (not (`self.Static`)))
      (`PrimitiveComponent.SetMassOverrideInKg` (`StaticMeshActor.StaticMeshComponent` (`self.Static Mesh Actor Ref`)) "None" (`self.OverwriteWeight`) true))))

(fn `Collision and Physic Settings Moveable`
  (params (self2 :type "StaticMeshActor Object Reference") (self3 :type "Actor Object Reference") (self4 :type "StaticMeshActor Object Reference"))
  (bind _staticmeshcomponent (`StaticMeshActor.StaticMeshComponent` self4))
  (`StaticMeshActor.SetMobility` self2 "Movable")
  (`self.SetActorEnableCollision` self3 true)
  (`PrimitiveComponent.SetSimulatePhysics` _staticmeshcomponent true)
  (`PrimitiveComponent.SetNotifyRigidBodyCollision` _staticmeshcomponent true)
  (set `PrimitiveComponent.bGenerateOverlapEvents` true _staticmeshcomponent)
  (`PrimitiveComponent.SetCollisionResponseToAllChannels` _staticmeshcomponent "ECR_Block")
  (`PrimitiveComponent.SetCollisionObjectType` _staticmeshcomponent "ECC_PhysicsBody"))

(fn `Collision and Physic Settings Static`
  (params (self2 :type "StaticMeshActor Object Reference") (self3 :type "Actor Object Reference") (self4 :type "StaticMeshActor Object Reference"))
  (bind _staticmeshcomponent (`StaticMeshActor.StaticMeshComponent` self4))
  (`StaticMeshActor.SetMobility` self2 "Static")
  (`self.SetActorEnableCollision` self3 true)
  (`PrimitiveComponent.SetSimulatePhysics` _staticmeshcomponent false)
  (`PrimitiveComponent.SetNotifyRigidBodyCollision` _staticmeshcomponent true)
  (set `PrimitiveComponent.bGenerateOverlapEvents` true _staticmeshcomponent)
  (`PrimitiveComponent.SetCollisionResponseToAllChannels` _staticmeshcomponent "ECR_Block")
  (`PrimitiveComponent.SetCollisionObjectType` _staticmeshcomponent "ECC_WorldStatic"))

(fn `Get Random Point in Box`
  (returns (ReturnValue :type "Vector Structure"))
  (bind (_returnvalue_x _returnvalue_y _returnvalue_z) (`KismetMathLibrary.BreakVector` (`BoxComponent.GetScaledBoxExtent` (`self.Spawn Volume`))))
  (return (+ (`KismetMathLibrary.MakeVector` (`KismetMathLibrary.RandomFloatInRange` (* _returnvalue_x -1.0) _returnvalue_x) (`KismetMathLibrary.RandomFloatInRange` (* _returnvalue_y -1.0) _returnvalue_y) (* _returnvalue_z -1.0)) (`self.K2_GetActorLocation`))))

(fn `UserConstructionScript`
  (bind _meshes_to_spawn_from (`self.Meshes to Spawn from`))
  (if (> (`KismetArrayLibrary.Array_Length` _meshes_to_spawn_from) 0)
    (`StaticMeshComponent.SetStaticMesh` (`self.UI Visualiser`) (`KismetArrayLibrary.Array_Random` _meshes_to_spawn_from))
    (`SceneComponent.K2_SetWorldTransform` (`self.UI Visualiser`) (`KismetMathLibrary.MakeTransform` (`self.Get Random Point in Box`) (`KismetMathLibrary.MakeRotator` (`KismetMathLibrary.RandomFloatInRange` (`self.Min Degree Roll Rotation`) (`self.Max Degree Roll Rotation`)) (`KismetMathLibrary.RandomFloatInRange` (`self.Min Degree Pitch Rotation`) (`self.Max Degree Pitch Rotation`)) (`KismetMathLibrary.RandomFloatInRange` (`self.Min Degree Yaw Rotation`) (`self.Max Degree Yaw Rotation`))) (`self.Scale`)) false true)
    (else
      (`StaticMeshComponent.SetStaticMesh` (`self.UI Visualiser`) null))))