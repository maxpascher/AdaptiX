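; Spawn-variation helper that moves a referenced level actor to one of several alternative transforms at game start.
; Construction script previews alternatives as ghost-material child actors copying the original's class and static mesh, and toggles an error billboard.
; On BeginPlay, a "ChosenAlternative" tag on the original or a ghost forces that spot.
; Otherwise it picks randomly, including the original position, then destroys the ghosts.
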(event `self.ReceiveBeginPlay`
  (`|ExecutionSequence`
    (:`then_0`
      (if (not (`self.ActorHasTag` (`self.OriginalActor`) "ChosenAlternative"))
        (for _array_element (`self.GetAllChildActors` true)
          (if (`self.ActorHasTag` _array_element "ChosenAlternative")
            (set `self.ChosenSpawn` (`self.GetTransform` _array_element))
            (set `self.SpawnHasChosen` true)
            (break)))
        (if (`self.SpawnHasChosen`)
          (`self.K2_SetActorTransform` (`self.OriginalActor`) (`self.ChosenSpawn`) false true)
          (else
            (`self.SpawnActorOnAlternative`)))))
    (:`then_1`
      (`self.K2_DestroyActor` (`self.GetAllChildActors` true)))))

(fn `SpawnActorOnAlternative`
  (locals (SpawnIndex :type Integer :default 0))
  (bind _output_get (set `local.SpawnIndex` (`KismetMathLibrary.RandomIntegerInRange` 0 (`KismetArrayLibrary.Array_Length` (`self.AlternativeSpawnPoses`)))))
  (if (< _output_get (`KismetArrayLibrary.Array_Length` (`self.AlternativeSpawnPoses`)))
    (`self.K2_SetActorTransform` (`self.OriginalActor`) (`KismetMathLibrary.ComposeTransforms` (`|GetArrayItem` (`self.AlternativeSpawnPoses`) (`local.SpawnIndex`)) (`self.GetTransform`)) false true)))

(fn `UserConstructionScript`
  (`SceneComponent.SetVisibility` (`self.ErrorBillboard`) (or (== (`self.OriginalActor`) null) (== (`KismetArrayLibrary.Array_Length` (`self.AlternativeSpawnPoses`)) 0) (not (`self.ActivateAlternatives`))) false)
  (if (`self.ActivateAlternatives`)
    ;[1 1 1] Ghosts
    (for _array_element (`self.AlternativeSpawnPoses`)
      (bind _returnvalue (`AddComponent|NODE_AddChildActorComponent-1` :`RelativeTransform` _array_element))
      (`ChildActorComponent.SetChildActorClass` _returnvalue (`GameplayStatics.GetObjectClass` (`self.OriginalActor`)))
      (`|ExecutionSequence`
        (:`then_0`
          (bind _childactor (`ChildActorComponent.ChildActor` _returnvalue))
          (bind _asstatic_mesh_actor (cast `StaticMeshActor` _childactor))
          (bind _asstatic_mesh_actor_2 (cast `StaticMeshActor` (`self.OriginalActor`)))
          (`StaticMeshComponent.SetStaticMesh` (`StaticMeshActor.StaticMeshComponent` _asstatic_mesh_actor) (`StaticMeshComponent.StaticMesh` (`StaticMeshActor.StaticMeshComponent` _asstatic_mesh_actor_2))))
        (:`then_1`
          (for _array_element_2 (`self.K2_GetComponentsByClass` _childactor "/Script/Engine.MeshComponent")
            (for _index (range (`PrimitiveComponent.GetNumMaterials` _array_element_2))
              (`PrimitiveComponent.SetMaterial` _array_element_2 _index "/Game/Blueprints/BP_SpawnAreas/resources/M_AlternativeSpawnGhosts.M_AlternativeSpawnGhosts"))))))))