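; A test light switch Blueprint that swaps level lighting from midday to night when something overlaps its cube trigger.
; On overlap it plays a button sound, starts unloading the EssenMidday streaming level and does a blocking load of EssenNight, made visible after loading.
; A Switchable flag with a two-second delay debounces repeated hits; the switch only goes one way, toward night.
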(event `self.Cube1.OnComponentBeginOverlap`
  (params (OverlappedComponent :type "PrimitiveComponent Object Reference") (OtherActor :type "Actor Object Reference") (OtherComp :type "PrimitiveComponent Object Reference") (OtherBodyIndex :type Integer) (bFromSweep :type Boolean) (SweepResult :type "HitResult Structure (by ref)"))
  (if (`self.Switchable?`)
    (set `self.Switchable?` false)
    (`GameplayStatics.PlaySoundAtLocation` "/Game/Sounds/SoundCue_Minecraft_Button.SoundCue_Minecraft_Button" (`SceneComponent.K2_GetComponentLocation` (`self.Cube1`)) (struct) 1.0 1.0 0.0 null null null)
    (`GameplayStatics.UnloadStreamLevel` "EssenMidday")
    (`GameplayStatics.LoadStreamLevel` "EssenNight" true true)
    (`KismetSystemLibrary.PrintString` "Lightswitch hit")
    (`KismetSystemLibrary.Delay` 2.0)
    (set `self.Switchable?` true)))

(fn `UserConstructionScript`)