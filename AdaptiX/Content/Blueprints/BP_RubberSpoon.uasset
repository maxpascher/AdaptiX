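; BP_RubberSpoon is a spoon actor that scoops cereal-style contents and can force a cereal bowl into the level.
; When its ScoopSphere overlaps a component attached to a "Reservoir" socket, it teleports that actor's child actors to the sphere.
; With ForceCereals on, BeginPlay finds the nearest "Plate"-tagged static mesh, destroys "Food"-tagged meshes within range of it, then swaps it for a BP_Cerealbowl.
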(event `self.ReceiveBeginPlay`
  (if (`self.ForceCereals`)
    (`self.ReplaceClosestPlate`)))

(event `self.ScoopSphere.OnComponentBeginOverlap`
  (params (OverlappedComponent :type "PrimitiveComponent Object Reference") (OtherActor :type "Actor Object Reference") (OtherComp :type "PrimitiveComponent Object Reference") (OtherBodyIndex :type Integer) (bFromSweep :type Boolean) (SweepResult :type "HitResult Structure (by ref)"))
  (if (== (`SceneComponent.GetAttachSocketName` OtherComp) "Reservoir")
    (for _array_element (`self.GetAllChildActors` OtherActor false)
      (`self.K2_SetActorLocation` _array_element (`SceneComponent.K2_GetComponentLocation` (`self.ScoopSphere`)) false true))))

(fn `ReplaceClosestPlate`
  (locals (closestPlate :type "StaticMeshActor Object Reference") (closestPlateDistance :type "Float (double-precision)"))
  (bind _closestplate (`local.closestPlate`))
  (bind _outactors (`GameplayStatics.GetAllActorsOfClassWithTag` "/Script/Engine.StaticMeshActor" "Plate"))
  (if (> (`KismetArrayLibrary.Array_Length` _outactors) 0)
    (`|ExecutionSequence`
      (:`then_0`
        (bind _output (`|GetArrayItem` _outactors))
        (set `local.closestPlate` _output)
        (set `local.closestPlateDistance` (`self.GetDistanceTo` _output))
        (for _array_element _outactors
          (bind _returnvalue (`self.GetDistanceTo` _array_element))
          (if (< _returnvalue (`local.closestPlateDistance`))
            (set `local.closestPlateDistance` _returnvalue)
            (set `local.closestPlate` _array_element))))
      (:`then_1`
        (bind _outactors_2 (`GameplayStatics.GetAllActorsOfClassWithTag` "/Script/Engine.StaticMeshActor" "Food"))
        (for _array_element_2 _outactors_2
          (if (<= (`self.GetDistanceTo` (`local.closestPlate`) _array_element_2) (`self.ForceCereals_MaxFoodDistance`))
            (`self.K2_DestroyActor` _array_element_2))))
      (:`then_2`
        (bind _returnvalue_2 (`|SpawnActorFromClass` "/Game/RealObjects/FUA/BP_Cerealbowl.BP_Cerealbowl_C" (`self.GetTransform` _closestplate) "AlwaysSpawn" "OverrideRootScale" null 10 null))
        (`self.K2_DestroyActor` _closestplate)
        (set `local.closestPlate` _returnvalue_2)))))

(fn `UserConstructionScript`)