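; Microwave actor with a hinged door that a Jaco robot arm opens through a detachable handle proxy.
; Tick checks the handle's attach parent: when grasped, the door follows the handle's clamped angle and constraints link the arm to the body and door.
; On release it breaks those constraints and reattaches the handle after a tick-counted delay.
; With the handle on the door, physics runs only while open; either swing direction is supported.
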(event `self.ReceiveBeginPlay`
  (bind _returnvalue (`GameplayStatics.GetActorOfClass` "/Game/Blueprints/BP_JacoArm/Jaco.Jaco_C"))
  (set `self.Jaco` _returnvalue)
  (bind _asstatic_mesh_actor (cast `StaticMeshActor` (`ChildActorComponent.ChildActor` (`self.Door`))))
  (set `self.DoorActor` _asstatic_mesh_actor)
  (set `self.DoorMeshComponent` (`StaticMeshActor.StaticMeshComponent` _asstatic_mesh_actor))
  (bind _asstatic_mesh_actor_2 (cast `StaticMeshActor` (`ChildActorComponent.ChildActor` (`self.HandleProxy`))))
  (set `self.HandleProxyActor` _asstatic_mesh_actor_2)
  (set `self.HandleProxyMeshComponent` (`StaticMeshActor.StaticMeshComponent` _asstatic_mesh_actor_2))
  (`self.K2_AttachToActor` (`self.HandleProxyActor`) (`self.DoorActor`) "Handle" "SnapToTarget" "SnapToTarget" "SnapToTarget" true)
  (set `self.HandleRotationOffset` (- (`self.GetHandleRotation`) (`self.InitialDoorOpening`))) ; Initially store offset to be used in handleRotation Function
  (`PhysicsConstraintComponent.SetAngularSwing1Limit` (`self.DoorHinge`) "ACM_Limited" (`self.MaxDoorRotation_Swing`))
  (`PhysicsConstraintComponent.SetConstraintReferenceFrame` (`self.DoorHinge`) "Frame1" (`KismetMathLibrary.MakeTransform` (0.0 0.0 0.0))) ; Revert Initial opening angle value
)

(event `self.ReceiveTick`
  (params (DeltaSeconds :type "Float (single-precision)"))
  (bind _lethandlegodelaycounter (`self.LetHandleGoDelayCounter`))
  (bind _returnvalue (`self.GetAttachParentActor` (`self.HandleProxyActor`)))
  (bind _skeletalmeshcomponent (`SkeletalMeshActor.SkeletalMeshComponent` (`self.Jaco`)))
  (if (== _returnvalue (`self.DoorActor`))
    (`PrimitiveComponent.SetSimulatePhysics` (`self.DoorMeshComponent`) (> (`self.GetHandleRotation`) 0.0))
    (if (not (`SceneComponent.IsSimulatingPhysics` (`self.DoorMeshComponent`) "None"))
      (`self.K2_AttachToActor` (`self.DoorActor`) self "Door" "SnapToTarget" "SnapToTarget" "SnapToTarget" true))
    (elif (!= _returnvalue null)
      (`PrimitiveComponent.SetSimulatePhysics` (`self.DoorMeshComponent`) false)
      (`self.K2_AttachToActor` (`self.DoorActor`) self "Door" "SnapToTarget" "KeepWorld" "KeepWorld" true)
      (`self.K2_SetActorRelativeRotation` (`self.DoorActor`) (`KismetMathLibrary.MakeRotator` 0.0 0.0 (* (`KismetMathLibrary.SelectInt` 1 -1 (`self.PositiveOpeningAngle`)) (`KismetMathLibrary.FClamp` (`self.GetHandleRotation`) 0.0 (`self.MaxDoorRotation_ProxyPull`)))) true false)
      (`/Engine/EditorBlueprintResources/StandardMacros.DoOnce` false :!label _label
        (:`Completed`
          (`PhysicsConstraintComponent.SetConstrainedComponents` (`self.Jaco-on-arc-Constraint`) _skeletalmeshcomponent "joint7" (`self.StaticMeshComponent`) "None")
          (`PhysicsConstraintComponent.SetConstrainedComponents` (`self.DoorJacoCollisionDeactivator`) _skeletalmeshcomponent "joint7" (`self.DoorMeshComponent`) "None")))
      (else
        (`PhysicsConstraintComponent.BreakConstraint` (`self.Jaco-on-arc-Constraint`))
        (`PhysicsConstraintComponent.BreakConstraint` (`self.DoorJacoCollisionDeactivator`))
        (if (> _lethandlegodelaycounter 20)
          (set `self.LetHandleGoDelayCounter` 0)
          (`self.K2_AttachToActor` (`self.HandleProxyActor`) (`self.DoorActor`) "Handle" "SnapToTarget" "SnapToTarget" "SnapToTarget" true)
          (goto _label :!via `Reset`)
          (else
            (`/Engine/EditorBlueprintResources/StandardMacros.IncrementInt` _lethandlegodelaycounter)))))))

(fn `GetHandleRotation`
  (returns (ReturnValue_Yaw :type "Float (double-precision)"))
  (bind (_returnvalue_roll _returnvalue_pitch _returnvalue_yaw) (`KismetMathLibrary.BreakRotator` (`KismetMathLibrary.Conv_VectorToRotator` (`KismetMathLibrary.InverseTransformLocation` (`SceneComponent.GetSocketTransform` (`self.StaticMeshComponent`) "Door" "RTS_World") (`SceneComponent.K2_GetComponentLocation` (`self.HandleProxyMeshComponent`))))))
  (bind _returnvalue (- (* (`KismetMathLibrary.SelectInt` 1 -1 (`self.PositiveOpeningAngle`)) _returnvalue_yaw) (`self.HandleRotationOffset`)))
  (return (`KismetMathLibrary.SelectFloat` (+ _returnvalue 360.0) _returnvalue (< _returnvalue -45.0))))

(fn `UserConstructionScript`
  (`SceneComponent.K2_SetRelativeRotation` (`self.Door`) (`KismetMathLibrary.MakeRotator` 0.0 0.0 (* (`KismetMathLibrary.SelectInt` 1 -1 (`self.PositiveOpeningAngle`)) (`self.InitialDoorOpening`))) false true))