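; Double wall light switch with two independent toggle buttons that the player pawn flips by overlapping them.
; Each button has a top collision box for off and a bottom one for on, which rotate it, play a click and call UpdateLinkedLight.
; That function matches the button's light class against a hard-coded list and calls UpdateLight on every actor of that class, reporting an error otherwise.
; BeginPlay sets initial button rotations; random placement logic is unused.
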(event `self.ReceiveBeginPlay`
  ;[0 0 0] Initial left and right button states
  (`self.SetInitialButtonRotationLeftAndRight` (`self.ButtonPressed_Left?`) (`self.ButtonPressed_Right?`)))

(event `self.Button_Collision_Left_Top.OnComponentBeginOverlap`
  (params (OverlappedComponent :type "PrimitiveComponent Object Reference") (OtherActor :type "Actor Object Reference") (OtherComp :type "PrimitiveComponent Object Reference") (OtherBodyIndex :type Integer) (bFromSweep :type Boolean) (SweepResult :type "HitResult Structure (by ref)"))
  (bind _buttonpressed_left_ (`self.ButtonPressed_Left?`))
  (bind _switch_button_left (`self.Switch_Button_Left`))
  ;[0 0 0] Left Button Interaction
  ;;[0.0336 0.04114 0.05729] Button from ON to OFF
  ;;;[0.0336 0.04114 0.05729] Check, if upper collision box is overlapping player pawn
  (if (== OtherActor (`GameplayStatics.GetPlayerPawn` 0))
    ;;;[0.0336 0.04114 0.05729] Rotate Button
    (if _buttonpressed_left_
      (`KismetSystemLibrary.MoveComponentTo` _switch_button_left (`self.ButtonLocationLeft`) (`KismetMathLibrary.MakeRotator` (`self.ButtonRotationNotPressed`)) true false 0.15 true)
      (set `self.ButtonPressed_Left?` (not _buttonpressed_left_))
      (`GameplayStatics.PlaySoundAtLocation` (`self.ToggleSound`) (`SceneComponent.K2_GetComponentLocation` _switch_button_left) (struct) 1.0 (`KismetMathLibrary.RandomFloatInRange` 0.995 1.005) 0.0 null null null)
      (`KismetSystemLibrary.PrintString` "ON TO OFF" true true (struct :`R` 0.048407 :`G` 0.075412 :`B` 0.760417 :`A` 1.0))
      ;;;[0.5833 0 0.01004] Set all light sources linked to THIS BUTTON to HIDDEN
      (`self.UpdateLinkedLight` (`self.ClassOfLinkedLightLeft`)))))

(event `self.Button_Collision_Left_Bottom.OnComponentBeginOverlap`
  (params (OverlappedComponent :type "PrimitiveComponent Object Reference") (OtherActor :type "Actor Object Reference") (OtherComp :type "PrimitiveComponent Object Reference") (OtherBodyIndex :type Integer) (bFromSweep :type Boolean) (SweepResult :type "HitResult Structure (by ref)"))
  (bind _buttonpressed_left_ (`self.ButtonPressed_Left?`))
  (bind _switch_button_left (`self.Switch_Button_Left`))
  ;[0 0 0] Left Button Interaction
  ;;[0.0336 0.04114 0.05729] Button from OFF to ON
  ;;;[0.0336 0.04114 0.05729] Check, if lower collision box is overlapping pawn
  (if (== OtherActor (`GameplayStatics.GetPlayerPawn` 0))
    ;;;[0.0336 0.04114 0.05729] Rotate Button
    (if (not _buttonpressed_left_)
      (`KismetSystemLibrary.MoveComponentTo` _switch_button_left (`self.ButtonLocationLeft`) (`KismetMathLibrary.MakeRotator` (`self.ButtonRotationPressed`)) true false 0.15 true)
      (set `self.ButtonPressed_Left?` (not _buttonpressed_left_))
      (`GameplayStatics.PlaySoundAtLocation` (`self.ToggleSound`) (`SceneComponent.K2_GetComponentLocation` _switch_button_left) (struct) 1.0 (`KismetMathLibrary.RandomFloatInRange` 0.995 1.005) 0.0 null null null)
      (`KismetSystemLibrary.PrintString` "OFF TO ON" true true (struct :`R` 0.577581 :`G` 0.114435 :`B` 0.020289 :`A` 1.0))
      ;;;[0.5833 0 0.01004] Set all light sources linked to this switch actor to VISIBLE
      (`self.UpdateLinkedLight` (`self.ClassOfLinkedLightLeft`)))))

(event `self.Button_Collision_Right_Top.OnComponentBeginOverlap`
  (params (OverlappedComponent :type "PrimitiveComponent Object Reference") (OtherActor :type "Actor Object Reference") (OtherComp :type "PrimitiveComponent Object Reference") (OtherBodyIndex :type Integer) (bFromSweep :type Boolean) (SweepResult :type "HitResult Structure (by ref)"))
  (bind _buttonpressed_right_ (`self.ButtonPressed_Right?`))
  (bind _switch_button_right (`self.Switch_Button_Right`))
  ;[0 0 0] Right Button Interaction
  ;;[0.0336 0.04114 0.05729] Button from OFF to ON
  ;;;[0.0336 0.04114 0.05729] Check, if upper collision box is overlapping pawn
  (if (== OtherActor (`GameplayStatics.GetPlayerPawn` 0))
    ;;;[0.0336 0.04114 0.05729] Rotate Button
    (if _buttonpressed_right_
      (`KismetSystemLibrary.MoveComponentTo` _switch_button_right (`self.ButtonLocationRight`) (`KismetMathLibrary.MakeRotator` (`self.ButtonRotationNotPressed`)) true false 0.15 true)
      (set `self.ButtonPressed_Right?` (not _buttonpressed_right_))
      (`GameplayStatics.PlaySoundAtLocation` (`self.ToggleSound`) (`SceneComponent.K2_GetComponentLocation` _switch_button_right) (struct) 1.0 (`KismetMathLibrary.RandomFloatInRange` 0.995 1.005) 0.0 null null null)
      (`KismetSystemLibrary.PrintString` "ON TO OFF" true true (struct :`R` 0.048407 :`G` 0.075412 :`B` 0.760417 :`A` 1.0))
      ;;;[0.5833 0 0.01004] Set all light sources linked to this switch actor to HIDDEN
      (`self.UpdateLinkedLight` (`self.ClassOfLinkedLightRight`)))))

(event `self.Button_Collision_Right_Bottom.OnComponentBeginOverlap`
  (params (OverlappedComponent :type "PrimitiveComponent Object Reference") (OtherActor :type "Actor Object Reference") (OtherComp :type "PrimitiveComponent Object Reference") (OtherBodyIndex :type Integer) (bFromSweep :type Boolean) (SweepResult :type "HitResult Structure (by ref)"))
  (bind _buttonpressed_right_ (`self.ButtonPressed_Right?`))
  (bind _switch_button_right (`self.Switch_Button_Right`))
  ;[0 0 0] Right Button Interaction
  ;;[0.0336 0.04114 0.05729] Button from OFF to ON
  ;;;[0.0336 0.04114 0.05729] Check, if lower collision box is overlapping pawn
  (if (== OtherActor (`GameplayStatics.GetPlayerPawn` 0))
    ;;;[0.0336 0.04114 0.05729] Rotate Button
    (if (not _buttonpressed_right_)
      (`KismetSystemLibrary.MoveComponentTo` _switch_button_right (`self.ButtonLocationRight`) (`KismetMathLibrary.MakeRotator` (`self.ButtonRotationPressed`)) true false 0.15 true)
      (set `self.ButtonPressed_Right?` (not _buttonpressed_right_))
      (`GameplayStatics.PlaySoundAtLocation` (`self.ToggleSound`) (`SceneComponent.K2_GetComponentLocation` _switch_button_right) (struct) 1.0 (`KismetMathLibrary.RandomFloatInRange` 0.995 1.005) 0.0 null null null)
      (`KismetSystemLibrary.PrintString` "OFF TO ON" true true (struct :`R` 0.577581 :`G` 0.114435 :`B` 0.020289 :`A` 1.0))
      ;;;[0.5833 0 0.01004] Set all light sources linked to this switch actor to VISIBLE
      (`self.UpdateLinkedLight` (`self.ClassOfLinkedLightRight`)))))

(fn `SetInitialButtonRotationLeftAndRight`
  (params (Left :type Boolean) (Right :type Boolean))
  (if Left
    (`SceneComponent.K2_SetRelativeLocationAndRotation` (`self.Switch_Button_Left`) (`self.ButtonLocationLeft`) (`KismetMathLibrary.MakeRotator` (`self.ButtonRotationPressed`)) false true)
    (else
      (`SceneComponent.K2_SetRelativeLocationAndRotation` (`self.Switch_Button_Left`) (`self.ButtonLocationLeft`) (`KismetMathLibrary.MakeRotator` (`self.ButtonRotationNotPressed`)) false true)))
  (if Right
    (`SceneComponent.K2_SetRelativeLocationAndRotation` (`self.Switch_Button_Right`) (`self.ButtonLocationRight`) (`KismetMathLibrary.MakeRotator` (`self.ButtonRotationPressed`)) false true)
    (else
      (`SceneComponent.K2_SetRelativeLocationAndRotation` (`self.Switch_Button_Right`) (`self.ButtonLocationRight`) (`KismetMathLibrary.MakeRotator` (`self.ButtonRotationNotPressed`)) false true)))
  (return))

(fn `UserConstructionScript`)