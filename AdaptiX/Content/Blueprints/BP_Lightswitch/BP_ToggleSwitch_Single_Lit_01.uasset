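; Single toggle wall switch with an indicator lamp that the player pawn flips by overlapping its top (off) or bottom (on) collision box.
; Each flip eases the button to its new pose, plays a pitch-varied click, prints debug text and swaps the lamp material.
; UpdateLinkedLights then calls UpdateLight on every actor of the chosen BP_ToggleLight class, so linking is per class, with an error for unsupported classes.
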(event `self.ReceiveBeginPlay`
  ;[0 0 0] Initial Button State
  (`self.SetInitialButtonRotation` (`self.ButtonPressed?`)))

(event `self.Button_Collision_Top.OnComponentBeginOverlap`
  (params (OverlappedComponent :type "PrimitiveComponent Object Reference") (OtherActor :type "Actor Object Reference") (OtherComp :type "PrimitiveComponent Object Reference") (OtherBodyIndex :type Integer) (bFromSweep :type Boolean) (SweepResult :type "HitResult Structure (by ref)"))
  (bind _switch_button (`self.Switch_Button`))
  (bind _buttonpressed_ (`self.ButtonPressed?`))
  ;[0 0 0] Button from ON to OFF
  ;;[0.0336 0.04114 0.05729] Check, if upper collision box is overlapping pawn
  (if (== OtherActor (`GameplayStatics.GetPlayerPawn` 0))
    ;;[0.0336 0.04114 0.05729] Rotate Button
    (if _buttonpressed_
      (`KismetSystemLibrary.MoveComponentTo` _switch_button (`self.ButtonLocationNotPressed`) (`KismetMathLibrary.MakeRotator` (`self.ButtonRotationNotPressed`)) true false 0.15 true)
      (set `self.ButtonPressed?` (not _buttonpressed_))
      (`GameplayStatics.PlaySoundAtLocation` (`self.ToggleSound`) (`SceneComponent.K2_GetComponentLocation` _switch_button) (struct) 1.0 (`KismetMathLibrary.RandomFloatInRange` 0.95 1.05) 0.0 null null null)
      (`KismetSystemLibrary.PrintString` "ON TO OFF" true true (struct :`R` 0.023153 :`G` 0.035601 :`B` 0.351533 :`A` 1.0))
      ;;[0.5833 0 0.01004] Set all light sources linked to this switch actor to HIDDEN
      (`self.UpdateLinkedLights` (`self.ClassOfLinkedLight`))
      (`PrimitiveComponent.SetMaterial` (`self.Switch_Lamp`) 0 "/Game/Materials_Randomise/Materials/Mat_Light.Mat_Light"))))

(event `self.Button_Collision_Bottom.OnComponentBeginOverlap`
  (params (OverlappedComponent :type "PrimitiveComponent Object Reference") (OtherActor :type "Actor Object Reference") (OtherComp :type "PrimitiveComponent Object Reference") (OtherBodyIndex :type Integer) (bFromSweep :type Boolean) (SweepResult :type "HitResult Structure (by ref)"))
  (bind _buttonpressed_ (`self.ButtonPressed?`))
  (bind _switch_button (`self.Switch_Button`))
  ;[0 0 0] Button from OFF to ON
  ;;[0.0336 0.04114 0.05729] Check, if lower collision box is overlapping pawn
  (if (== OtherActor (`GameplayStatics.GetPlayerPawn` 0))
    ;;[0.0336 0.04114 0.05729] Rotate Button
    (if (not _buttonpressed_)
      (`KismetSystemLibrary.MoveComponentTo` _switch_button (`self.ButtonLocationPressed`) (`KismetMathLibrary.MakeRotator` (`self.ButtonRotationPressed`)) true false 0.15 true)
      (set `self.ButtonPressed?` (not _buttonpressed_))
      (`GameplayStatics.PlaySoundAtLocation` (`self.ToggleSound`) (`SceneComponent.K2_GetComponentLocation` _switch_button) (struct) 1.0 (`KismetMathLibrary.RandomFloatInRange` 0.995 1.005) 0.0 null null null)
      (`KismetSystemLibrary.PrintString` "OFF TO ON" true true (struct :`R` 0.577581 :`G` 0.114435 :`B` 0.020289 :`A` 1.0))
      ;;[0.5833 0 0.01004] Set all light sources linked to this switch actor to VISIBLE
      (`self.UpdateLinkedLights` (`self.ClassOfLinkedLight`))
      (`PrimitiveComponent.SetMaterial` (`self.Switch_Lamp`) 0 "/Game/Materials_Randomise/Meshes/kitchen/Glass.Glass"))))

(fn `SetInitialButtonRotation`
  (params (Condition :type Boolean))
  (bind _switch_button (`self.Switch_Button`))
  (if Condition
    (`SceneComponent.K2_SetRelativeLocationAndRotation` _switch_button (`self.ButtonLocationPressed`) (`KismetMathLibrary.MakeRotator` (`self.ButtonRotationPressed`)) false true)
    (`PrimitiveComponent.SetMaterial` (`self.Switch_Lamp`) 0 "/Game/Materials_Randomise/Meshes/kitchen/Glass.Glass")
    (else
      (`SceneComponent.K2_SetRelativeLocationAndRotation` _switch_button (`self.ButtonLocationNotPressed`) (`KismetMathLibrary.MakeRotator` (`self.ButtonRotationNotPressed`)) false true)
      (`PrimitiveComponent.SetMaterial` (`self.Switch_Lamp`) 0 "/Game/Materials_Randomise/Materials/Mat_Light.Mat_Light"))))

(fn `UserConstructionScript`)