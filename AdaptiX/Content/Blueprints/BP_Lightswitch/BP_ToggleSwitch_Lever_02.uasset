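; Physical lever light switch that the player pushes between ON and OFF.
; Player overlap on touch volumes enables physics on the button; end-position collisions freeze it, flip ButtonPressed, play a sound and call UpdateLight on every BP_ToggleLight_Hanging_01 in the level.
; When the player leaves, physics stops, and after a random delay a half-moved lever is meant to ease back to its previous state.
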(event `self.ReceiveBeginPlay`
  (bind _switch_button (`self.Switch_Button`))
  ;[0 0 0] 1) Initial Button State and relative world position / rotation
  (`PrimitiveComponent.SetSimulatePhysics` _switch_button false)
  (`SceneComponent.K2_SetRelativeLocationAndRotation` _switch_button (`SceneComponent.RelativeLocation` _switch_button) (`KismetMathLibrary.Conv_VectorToRotator` (`SceneComponent.GetForwardVector` _switch_button)) false false)
  (if (`self.ButtonPressed?`)
    (`SceneComponent.K2_AddRelativeRotation` (`self.Switch_Button`) (`KismetMathLibrary.MakeRotator` (`self.ButtonRotationPressed`)) false true)
    (else
      (`SceneComponent.K2_AddRelativeLocation` (`self.Switch_Button`) (`KismetMathLibrary.MakeVector` (`self.ButtonRotationNotPressed`)) false true))))

(event `self.Button_TouchCollision_Top.OnComponentBeginOverlap`
  (params (OverlappedComponent :type "PrimitiveComponent Object Reference") (OtherActor :type "Actor Object Reference") (OtherComp :type "PrimitiveComponent Object Reference") (OtherBodyIndex :type Integer) (bFromSweep :type Boolean) (SweepResult :type "HitResult Structure (by ref)"))
  ;[0 0 0] 2) Set switch button movable
  (if (`self.ButtonPressed?`)
    _
    (elif (== OtherActor (`GameplayStatics.GetPlayerPawn` 0))
      (`PrimitiveComponent.SetSimulatePhysics` (`self.Switch_Button`) true))))

(event `self.Button_TouchCollision_Bottom.OnComponentBeginOverlap`
  (params (OverlappedComponent :type "PrimitiveComponent Object Reference") (OtherActor :type "Actor Object Reference") (OtherComp :type "PrimitiveComponent Object Reference") (OtherBodyIndex :type Integer) (bFromSweep :type Boolean) (SweepResult :type "HitResult Structure (by ref)"))
  ;[0 0 0] 2) Set switch button movable
  (if (`self.ButtonPressed?`)
    (if (== OtherActor (`GameplayStatics.GetPlayerPawn` 0))
      (`PrimitiveComponent.SetSimulatePhysics` (`self.Switch_Button`) true))))

(event `self.Switch_Collision.OnComponentEndOverlap`
  (params (OverlappedComponent :type "PrimitiveComponent Object Reference") (OtherActor :type "Actor Object Reference") (OtherComp :type "PrimitiveComponent Object Reference") (OtherBodyIndex :type Integer))
  (bind _switch_button (`self.Switch_Button`))
  (bind _switch_button_2 (`self.Switch_Button`))
  (bind _returnvalue (`SceneComponent.K2_GetComponentLocation` _switch_button_2))
  (bind _returnvalue_2 (`SceneComponent.K2_GetComponentLocation` _switch_button))
  ;[0 0 0] 3) Reset button rotation to its former state when not fully ON or OFF after a short delay
  (`PrimitiveComponent.SetSimulatePhysics` (`self.Switch_Button`) false)
  (if (== OtherActor (`GameplayStatics.GetPlayerPawn` 0))
    (if (not (`self.ButtonPressed?`))
      (`KismetSystemLibrary.Delay` (`KismetMathLibrary.RandomFloatInRange` 2.0 6.0))
      (if (not (`PrimitiveComponent.IsOverlappingActor` (`self.Button_TouchCollision_Top`) (`GameplayStatics.GetPlayerPawn` 0)))
        ;;[0.3362 0.849 0.5728] Check, if buttons rotation has terminated
        (if (not (`self.CheckIfButtonStateFinal`))
          (`KismetSystemLibrary.MoveComponentTo` _switch_button_2 _returnvalue (`KismetMathLibrary.MakeRotator` (`self.ButtonRotationNotPressed`)) false true 0.2 true)
          (`GameplayStatics.PlaySoundAtLocation` (`self.ToggleSound`) _returnvalue (struct) 1.0 1.0 0.0 null null null)))
      (else
        (`KismetSystemLibrary.Delay` (`KismetMathLibrary.RandomFloatInRange` 2.0 6.0))
        (if (not (`PrimitiveComponent.IsOverlappingActor` (`self.Button_TouchCollision_Bottom`) (`GameplayStatics.GetPlayerPawn` 0)))
          ;;[0.3362 0.849 0.5728] Check, if buttons rotation has terminated
          (if (not (`self.CheckIfButtonStateFinal`))
            (`KismetSystemLibrary.MoveComponentTo` _switch_button _returnvalue_2 (`KismetMathLibrary.MakeRotator` (`self.ButtonRotationPressed`)) false true 0.2 true)
            (`GameplayStatics.PlaySoundAtLocation` (`self.ToggleSound`) _returnvalue_2 (struct) 1.0 1.0 0.0 null null null)))))))

(event `self.Button_Collision_Top.OnComponentBeginOverlap`
  (params (OverlappedComponent :type "PrimitiveComponent Object Reference") (OtherActor :type "Actor Object Reference") (OtherComp :type "PrimitiveComponent Object Reference") (OtherBodyIndex :type Integer) (bFromSweep :type Boolean) (SweepResult :type "HitResult Structure (by ref)"))
  (bind _buttonpressed_ (`self.ButtonPressed?`))
  (bind _switch_button (`self.Switch_Button`))
  ;[0.02363 0.03562 0.349] 2a) Switch button state from ON to OFF
  (if (`self.InputEnabled?`)
    (if (== OtherComp (`self.Body_Collision_Top`))
      (if _buttonpressed_
        (`PrimitiveComponent.SetSimulatePhysics` _switch_button false)
        (bind _result (`/Engine/EditorBlueprintResources/StandardMacros.NegateFloat` (`self.ButtonRotationPressed`))
          (:`  `
            (`SceneComponent.K2_AddRelativeLocation` (`self.Switch_Button`) (`KismetMathLibrary.MakeVector` _result) false false)
            (set `self.ButtonPressed?` (not _buttonpressed_))
            (`GameplayStatics.PlaySoundAtLocation` (`self.ToggleSound`) (`SceneComponent.K2_GetComponentLocation` _switch_button) (struct) 1.0 1.0 0.0 null null null)
            (`KismetSystemLibrary.PrintString` "LIGHT OFF")
            ;;[0.3362 0.849 0.5728] Set all light sources linked to this switch actor to HIDDEN
            (bind _outactors (`GameplayStatics.GetAllActorsOfClass` "/Game/Blueprints/BP_Lightswitch/BP_ToggleLight_Hanging_01.BP_ToggleLight_Hanging_01_C"))
            (for _array_element _outactors
              (`/Game/Blueprints/BP_Lightswitch/BP_ToggleLight_Hanging_01.UpdateLight` _array_element)
              (`KismetSystemLibrary.Delay` 2.0)
              (set `self.InputEnabled?` true))))))))

(event `self.Button_Collision_Bottom.OnComponentBeginOverlap`
  (params (OverlappedComponent :type "PrimitiveComponent Object Reference") (OtherActor :type "Actor Object Reference") (OtherComp :type "PrimitiveComponent Object Reference") (OtherBodyIndex :type Integer) (bFromSweep :type Boolean) (SweepResult :type "HitResult Structure (by ref)"))
  (bind _buttonpressed_ (`self.ButtonPressed?`))
  (bind _switch_button (`self.Switch_Button`))
  ;[0.5729 0.1148 0.02089] 2b) Switch button state from ON to OFF
  (if (`self.InputEnabled?`)
    (if (== OtherComp (`self.Body_Collision_Bottom`))
      (if (not _buttonpressed_)
        (set `self.InputEnabled?` false)
        (`PrimitiveComponent.SetSimulatePhysics` _switch_button false)
        (`SceneComponent.K2_AddRelativeLocation` (`self.Switch_Button`) (`KismetMathLibrary.MakeVector` (`self.ButtonRotationPressed`)) false false)
        (set `self.ButtonPressed?` (not _buttonpressed_))
        (`GameplayStatics.PlaySoundAtLocation` (`self.ToggleSound`) (`SceneComponent.K2_GetComponentLocation` _switch_button) (struct) 1.0 1.0 0.0 null null null)
        (`KismetSystemLibrary.PrintString` "LIGHT ON")
        ;;[0.3362 0.849 0.5728] Set all light sources linked to this switch actor to VISIBLE
        (bind _outactors (`GameplayStatics.GetAllActorsOfClass` "/Game/Blueprints/BP_Lightswitch/BP_ToggleLight_Hanging_01.BP_ToggleLight_Hanging_01_C"))
        (for _array_element _outactors
          (`/Game/Blueprints/BP_Lightswitch/BP_ToggleLight_Hanging_01.UpdateLight` _array_element)
          (`KismetSystemLibrary.Delay` 2.0)
          (set `self.InputEnabled?` true))))))

(fn `UserConstructionScript`)