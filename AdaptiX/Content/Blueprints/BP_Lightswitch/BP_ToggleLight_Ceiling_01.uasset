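; Ceiling light actor that turns on or off to match the button state of a linked toggle switch actor.
; BeginPlay and UpdateLight repeat the same class-check chain over five switch Blueprints, using left/right flags to pick a button on the double switch.
; The result sets RectLight visibility and swaps the Light material between lit and glass.
; Invalid links print an on-screen error, with an error sound at BeginPlay only.
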(event `self.ReceiveBeginPlay`
  (bind _linkedlightswitchactor (`self.LinkedLightSwitchActor`))
  (bind _linkedlightswitchactor_2 (`self.LinkedLightSwitchActor`))
  (bind _lighton_ (`self.LightOn?`))
  (bind _linkedlightswitchactor_3 (`self.LinkedLightSwitchActor`))
  (bind _linkedlightswitchactor_4 (`self.LinkedLightSwitchActor`))
  (bind _linkedlightswitchactor_5 (`self.LinkedLightSwitchActor`))
  ;[0 0 0] Check any linked light switch and use its button state to set whether this light is ON or OFF
  (if (== (`GameplayStatics.GetObjectClass` _linkedlightswitchactor_3) "/Game/Blueprints/BP_Lightswitch/BP_ToggleSwitch_Single_02.BP_ToggleSwitch_Single_02_C")
    (bind _asbp_toggle_switch_single_02 (cast `/Game/Blueprints/BP_Lightswitch/BP_ToggleSwitch_Single_02` _linkedlightswitchactor_3))
    (set `self.LightOn?` (`/Game/Blueprints/BP_Lightswitch/BP_ToggleSwitch_Single_02.ButtonPressed?` _asbp_toggle_switch_single_02))
    ;[0 0 0] Set visibility of components
    (`SceneComponent.SetVisibility` (`self.RectLight`) _lighton_ false :!label _label)
    (if _lighton_
      (`PrimitiveComponent.SetMaterial` (`self.Light`) 0 "/Game/Materials_Randomise/Materials/Mat_Light.Mat_Light")
      (else
        (`PrimitiveComponent.SetMaterial` (`self.Light`) 0 "/Game/Materials_Randomise/Materials/kitchen/Mat_Glass.Mat_Glass")))
    (elif (== (`GameplayStatics.GetObjectClass` _linkedlightswitchactor) "/Game/Blueprints/BP_Lightswitch/BP_ToggleSwitch_Single_Lit_01.BP_ToggleSwitch_Single_Lit_01_C")
      (bind _asbp_toggle_switch_single_lit_01 (cast `/Game/Blueprints/BP_Lightswitch/BP_ToggleSwitch_Single_Lit_01` _linkedlightswitchactor))
      (set `self.LightOn?` (`/Game/Blueprints/BP_Lightswitch/BP_ToggleSwitch_Single_Lit_01.ButtonPressed?` _asbp_toggle_switch_single_lit_01))
      (goto _label)
      (elif (== (`GameplayStatics.GetObjectClass` _linkedlightswitchactor_5) "/Game/Blueprints/BP_Lightswitch/BP_ToggleSwitch_Lever_01.BP_ToggleSwitch_Lever_01_C")
        (bind _asbp_toggle_switch_lever_01 (cast `/Game/Blueprints/BP_Lightswitch/BP_ToggleSwitch_Lever_01` _linkedlightswitchactor_5))
        (set `self.LightOn?` (`/Game/Blueprints/BP_Lightswitch/BP_ToggleSwitch_Lever_01.ButtonPressed?` _asbp_toggle_switch_lever_01))
        (goto _label)
        (elif (== (`GameplayStatics.GetObjectClass` _linkedlightswitchactor_2) "/Game/Blueprints/BP_Lightswitch/BP_ToggleSwitch_Single_01.BP_ToggleSwitch_Single_01_C")
          (bind _asbp_toggle_switch_single_01 (cast `/Game/Blueprints/BP_Lightswitch/BP_ToggleSwitch_Single_01` _linkedlightswitchactor_2))
          (set `self.LightOn?` (`/Game/Blueprints/BP_Lightswitch/BP_ToggleSwitch_Single_01.ButtonPressed?` _asbp_toggle_switch_single_01))
          (goto _label)
          (else
            ;[0 0 0] Check, if the light switch is a double switch actor
            (if (== (`GameplayStatics.GetObjectClass` _linkedlightswitchactor_4) "/Game/Blueprints/BP_Lightswitch/BP_ToggleSwitch_Double_01.BP_ToggleSwitch_Double_01_C")
              (bind _asbp_toggle_switch_double_01 (cast `/Game/Blueprints/BP_Lightswitch/BP_ToggleSwitch_Double_01` _linkedlightswitchactor_4))
              ;;[0.6094 0.02826 0.089] Check left button state
              (if (`self.AffectedByLeftSwitchButton?`)
                (set `self.LightOn?` (`/Game/Blueprints/BP_Lightswitch/BP_ToggleSwitch_Double_01.ButtonPressed_Left?` _asbp_toggle_switch_double_01))
                (goto _label)
                (else
                  ;;[0.1525 0.08683 1] Check right button state
                  (if (`self.AffectedByRightSwitchButton?`)
                    (set `self.LightOn?` (`/Game/Blueprints/BP_Lightswitch/BP_ToggleSwitch_Double_01.ButtonPressed_Right?` _asbp_toggle_switch_double_01))
                    (goto _label)
                    (else
                      ;[1 0.2175 0.006859] Throw error message when double switch asigned but no button
                      (`KismetSystemLibrary.PrintString` "ERROR: Light linked to double switch actor but no specific button asigned" true true (struct :`R` 0.822917 :`B` 0.014551 :`A` 1.0) 10.0)
                      (`GameplayStatics.PlaySound2D` "/Engine/EditorSounds/Notifications/CompileFailed_Cue.CompileFailed_Cue" 1.0 1.0 0.0 null null)))))
              (else
                ;[1 0.2175 0.006859] Throw error message when switch actor not valid
                (`KismetSystemLibrary.PrintString` "ERROR: A linked switch actor is not valid or none has been asigned!" true true (struct :`R` 0.822917 :`B` 0.014551 :`A` 1.0) 10.0)
                (`GameplayStatics.PlaySound2D` "/Engine/EditorSounds/Notifications/CompileFailed_Cue.CompileFailed_Cue" 1.0 1.0 0.0 null null)))))))))

(fn `UpdateLight`
  (bind _linkedlightswitchactor (`self.LinkedLightSwitchActor`))
  (bind _linkedlightswitchactor_2 (`self.LinkedLightSwitchActor`))
  (bind _lighton_ (`self.LightOn?`))
  (bind _linkedlightswitchactor_3 (`self.LinkedLightSwitchActor`))
  (bind _linkedlightswitchactor_4 (`self.LinkedLightSwitchActor`))
  (bind _linkedlightswitchactor_5 (`self.LinkedLightSwitchActor`))
  ;[0 0 0] If linked switch is of class BP_Master_ToggleSwitch
  (if (== (`GameplayStatics.GetObjectClass` _linkedlightswitchactor_3) "/Game/Blueprints/BP_Lightswitch/BP_ToggleSwitch_Single_02.BP_ToggleSwitch_Single_02_C")
    (bind _asbp_toggle_switch_single_02 (cast `/Game/Blueprints/BP_Lightswitch/BP_ToggleSwitch_Single_02` _linkedlightswitchactor_3))
    (set `self.LightOn?` (`/Game/Blueprints/BP_Lightswitch/BP_ToggleSwitch_Single_02.ButtonPressed?` _asbp_toggle_switch_single_02))
    ;[0 0 0] Set visibility of components
    (`SceneComponent.SetVisibility` (`self.RectLight`) _lighton_ false :!label _label)
    (if _lighton_
      (`PrimitiveComponent.SetMaterial` (`self.Light`) 0 "/Game/Materials_Randomise/Materials/Mat_Light.Mat_Light")
      (else
        (`PrimitiveComponent.SetMaterial` (`self.Light`) 0 "/Game/Materials_Randomise/Materials/kitchen/Mat_Glass.Mat_Glass")))
    (else
      ;[0 0 0] If linked switch is of class class BP_ToggleSwitch_Night
      (if (== (`GameplayStatics.GetObjectClass` _linkedlightswitchactor) "/Game/Blueprints/BP_Lightswitch/BP_ToggleSwitch_Single_Lit_01.BP_ToggleSwitch_Single_Lit_01_C")
        (bind _asbp_toggle_switch_single_lit_01 (cast `/Game/Blueprints/BP_Lightswitch/BP_ToggleSwitch_Single_Lit_01` _linkedlightswitchactor))
        (set `self.LightOn?` (`/Game/Blueprints/BP_Lightswitch/BP_ToggleSwitch_Single_Lit_01.ButtonPressed?` _asbp_toggle_switch_single_lit_01))
        (goto _label)
        (else
          ;[0 0 0] If linked switch is of class BP_ToggleSwitch_Lever_01
          (if (== (`GameplayStatics.GetObjectClass` _linkedlightswitchactor_5) "/Game/Blueprints/BP_Lightswitch/BP_ToggleSwitch_Lever_01.BP_ToggleSwitch_Lever_01_C")
            (bind _asbp_toggle_switch_lever_01 (cast `/Game/Blueprints/BP_Lightswitch/BP_ToggleSwitch_Lever_01` _linkedlightswitchactor_5))
            (set `self.LightOn?` (`/Game/Blueprints/BP_Lightswitch/BP_ToggleSwitch_Lever_01.ButtonPressed?` _asbp_toggle_switch_lever_01))
            (goto _label)
            (else
              ;[0 0 0] If linked switch is of class BP_ToggleSwitch_Day
              (if (== (`GameplayStatics.GetObjectClass` _linkedlightswitchactor_2) "/Game/Blueprints/BP_Lightswitch/BP_ToggleSwitch_Single_01.BP_ToggleSwitch_Single_01_C")
                (bind _asbp_toggle_switch_single_01 (cast `/Game/Blueprints/BP_Lightswitch/BP_ToggleSwitch_Single_01` _linkedlightswitchactor_2))
                (set `self.LightOn?` (`/Game/Blueprints/BP_Lightswitch/BP_ToggleSwitch_Single_01.ButtonPressed?` _asbp_toggle_switch_single_01))
                (goto _label)
                (else
                  ;[0 0 0] Check, if the light switch is a double switch actor
                  (if (== (`GameplayStatics.GetObjectClass` _linkedlightswitchactor_4) "/Game/Blueprints/BP_Lightswitch/BP_ToggleSwitch_Double_01.BP_ToggleSwitch_Double_01_C")
                    (bind _asbp_toggle_switch_double_01 (cast `/Game/Blueprints/BP_Lightswitch/BP_ToggleSwitch_Double_01` _linkedlightswitchactor_4))
                    ;;[0.6094 0.02826 0.089] Check left button state
                    (if (`self.AffectedByLeftSwitchButton?`)
                      (set `self.LightOn?` (`/Game/Blueprints/BP_Lightswitch/BP_ToggleSwitch_Double_01.ButtonPressed_Left?` _asbp_toggle_switch_double_01))
                      (goto _label)
                      (else
                        ;;[0.1525 0.08683 1] Check right button state
                        (if (`self.AffectedByRightSwitchButton?`)
                          (set `self.LightOn?` (`/Game/Blueprints/BP_Lightswitch/BP_ToggleSwitch_Double_01.ButtonPressed_Right?` _asbp_toggle_switch_double_01))
                          (goto _label)
                          (else
                            ;[1 0.2175 0.006859] Throw error message when double switch asigned but no button
                            (`KismetSystemLibrary.PrintString` "ERROR: Light linked to double switch actor but no specific button asigned" true true (struct :`R` 0.822917 :`B` 0.014551 :`A` 1.0) 10.0)))))
                    (else
                      ;[1 0.2175 0.006859] Throw error message when switch actor not valid
                      (`KismetSystemLibrary.PrintString` "ERROR: A linked switch actor is not valid or none has been asigned!" true true (struct :`R` 0.822917 :`B` 0.014551 :`A` 1.0) 10.0))))))))))))

(fn `UserConstructionScript`)