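; Wardrobe prop Blueprint that randomises how far its door is open each time play begins.
; BeginPlay picks one of three states at random: closed, partially open or completely open.
; It then teleports the WardrobeDoor component along its local X axis to match, using a random offset for the partial state, and prints the chosen state as debug text.
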(event `self.ReceiveBeginPlay`
  ;[0 0 0] Wardrobe02 state randomisation
  ;;[0.0336 0.04114 0.05729] Randomise Wardrobe02 state
  (set `self.CurrentWardrobeState` (`KismetArrayLibrary.Array_Random` (`|MakeArray` (`self.WardrobeClosed`) (`self.WardrobeOpen`) (`self.WardrobeOpenComplete`))))
  ;;[0.0336 0.04114 0.05729] Wardrobe02 set to closed
  (if (== (`self.CurrentWardrobeState`) (`self.WardrobeClosed`))
    (`SceneComponent.K2_SetRelativeLocation` (`self.Wardrobe_Door`) (0.0 37.0 -40.0) false true)
    (`KismetSystemLibrary.PrintString` "Wardrobe02 set to closed")
    (else
      ;;[0.0336 0.04114 0.05729] Wardrobe02 set to partially open
      (if (== (`self.CurrentWardrobeState`) (`self.WardrobeOpen`))
        (`SceneComponent.K2_SetRelativeLocation` (`self.Wardrobe_Door`) (`KismetMathLibrary.MakeVector` (`KismetMathLibrary.RandomFloatInRange` 50.0 100.0) 37.0 -40.0) false true)
        (`KismetSystemLibrary.PrintString` "Wardrobe02 set to partially open")
        (else
          ;;[0.0336 0.04114 0.05729] Wardrobe02 set to completely open
          (if (== (`self.CurrentWardrobeState`) (`self.WardrobeOpenComplete`))
            (`SceneComponent.K2_SetRelativeLocation` (`self.Wardrobe_Door`) (130.0 37.0 -40.0) false true)
            (`KismetSystemLibrary.PrintString` "Wardrobe02 set to completely open")))))))

(fn `UserConstructionScript`)