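; Wardrobe prop Blueprint that randomises the pose of its two doors when play begins.
; BeginPlay picks one of four states: closed, left open, right open or both open.
; Closed doors snap to stored closed yaws, while open doors teleport to a random yaw within their swing range.
; Each branch prints a debug string, though the left and right messages are swapped relative to the door that opens.
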(event `self.ReceiveBeginPlay`
  ;[0 0 0] Wadrobe01 state randomisation
  ;;[0.0336 0.04114 0.05729] Wardrobe01 state randomisation
  (set `self.WardrobeState` (`KismetArrayLibrary.Array_Random` (`|MakeArray` (`self.WardrobeClosed`) (`self.WardrobeOpenLeft`) (`self.WardrobeOpenRight`) (`self.WardrobeOpenAll`))))
  ;;[0.0336 0.04114 0.05729] Wardrobe 01 set to closed
  (if (== (`self.WardrobeState`) (`self.WardrobeClosed`))
    (`SceneComponent.K2_SetRelativeRotation` (`self.Wardrobe_Door_Left`) (`KismetMathLibrary.MakeRotator` 0.0 0.0 (`self.DoorClosedLeft`)) false true)
    (`SceneComponent.K2_SetRelativeRotation` (`self.Wardrobe_Door_Right`) (`KismetMathLibrary.MakeRotator` 0.0 0.0 (`self.DoorClosedRight`)) false true)
    (`KismetSystemLibrary.PrintString` "Wardrobe01 set to closed")
    (else
      ;;[0.0336 0.04114 0.05729] Wardrobe01 set to open right
      (if (== (`self.WardrobeState`) (`self.WardrobeOpenLeft`))
        (`SceneComponent.K2_SetRelativeRotation` (`self.Wardrobe_Door_Left`) (`KismetMathLibrary.MakeRotator` 0.0 0.0 (`KismetMathLibrary.RandomFloatInRange` -150.0)) false true)
        (`SceneComponent.K2_SetRelativeRotation` (`self.Wardrobe_Door_Right`) (`KismetMathLibrary.MakeRotator` 0.0 0.0 (`self.DoorClosedRight`)) false true)
        (`KismetSystemLibrary.PrintString` "Wardrobe01 set to right partially open")
        (else
          ;;[0.0336 0.04114 0.05729] Wardrobe01 set to open left
          (if (== (`self.WardrobeState`) (`self.WardrobeOpenRight`))
            (`SceneComponent.K2_SetRelativeRotation` (`self.Wardrobe_Door_Left`) (`KismetMathLibrary.MakeRotator` 0.0 0.0 (`self.DoorClosedLeft`)) false true)
            (`SceneComponent.K2_SetRelativeRotation` (`self.Wardrobe_Door_Right`) (`KismetMathLibrary.MakeRotator` 0.0 0.0 (`KismetMathLibrary.RandomFloatInRange` 150.0)) false true)
            (`KismetSystemLibrary.PrintString` "Wardrobe01 set to left partially open")
            (else
              ;;[0.0336 0.04114 0.05729] Wardrobe01 set to completely open
              (if (== (`self.WardrobeState`) (`self.WardrobeOpenAll`))
                (`SceneComponent.K2_SetRelativeRotation` (`self.Wardrobe_Door_Left`) (`KismetMathLibrary.MakeRotator` 0.0 0.0 (`KismetMathLibrary.RandomFloatInRange` -150.0)) false true)
                (`SceneComponent.K2_SetRelativeRotation` (`self.Wardrobe_Door_Right`) (`KismetMathLibrary.MakeRotator` 0.0 0.0 (`KismetMathLibrary.RandomFloatInRange` 150.0)) false true)
                (`KismetSystemLibrary.PrintString` "Wardrobe01 set to completely open")))))))))

(fn `UserConstructionScript`)