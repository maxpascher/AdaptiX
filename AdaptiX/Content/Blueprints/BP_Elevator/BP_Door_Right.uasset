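; BP_Door_Right is the right-hand elevator door, sliding its static mesh between open and closed positions.
; Custom events openDoor and closeDoor each check the DoorOpen flag, then play their own timeline to lerp the mesh's relative location along Y between hardcoded endpoints.
; DoorOpen flips on timeline updates rather than on completion, and the existing "Open"/"Close" comments contradict the event names.
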(event `closeDoor`
  ;[1 1 1] Open the door
  (if (`self.Door_Open`)
    (bind (_direction _dooropens) (`Timeline|Timeline_0`)
      (:`Update`
        (`SceneComponent.K2_SetRelativeLocation` (`self.StaticMeshComponent`) (`KismetMathLibrary.VLerp` (-326.0 550.0 0.1) (-326.0 606.0 0.1) _dooropens) false false)
        (set `self.Door_Open` false)))))

(event `openDoor`
  ;[1 1 1] Close the door
  (if (not (`self.Door_Open`))
    (bind (_direction _dooropens) (`Timeline|Timeline_1`)
      (:`Update`
        (`SceneComponent.K2_SetRelativeLocation` (`self.StaticMeshComponent`) (`KismetMathLibrary.VLerp` (-326.0 606.0 0.1) (-326.0 550.0 0.1) _dooropens) false false)
        (set `self.Door_Open` true)))))

(fn `UserConstructionScript`)