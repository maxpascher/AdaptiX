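; BP_Taste is an elevator button that closes or opens the doors when its mesh is overlapped.
; The Innen flag marks it as inside or outside: overlap rotates the mesh, then after a delay closes (inside) or opens (outside) BP_Door_Left and BP_Door_Right.
; On BeginPlay it picks one of four meshes for its side, indexed by BP_LevelDatabase's RandomInt inside or a fresh random number outside.
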(event `self.StaticMeshComponent.OnComponentBeginOverlap`
  (params (OverlappedComponent :type "PrimitiveComponent Object Reference") (OtherActor :type "Actor Object Reference") (OtherComp :type "PrimitiveComponent Object Reference") (OtherBodyIndex :type Integer) (bFromSweep :type Boolean) (SweepResult :type "HitResult Structure (by ref)"))
  ;[1 1 1] Open or close the doors depending on the position
  (if (`self.innen`)
    (`SceneComponent.K2_SetRelativeRotation` (`self.StaticMeshComponent`) (struct :`Roll` 180.0) false false)
    (`KismetSystemLibrary.Delay` 2.0)
    (bind _returnvalue (`GameplayStatics.GetActorOfClass` "/Game/Blueprints/BP_Elevator/BP_Door_Left.BP_Door_Left_C"))
    (`/Game/Blueprints/BP_Elevator/BP_Door_Left.closeDoor` _returnvalue)
    (bind _returnvalue_2 (`GameplayStatics.GetActorOfClass` "/Game/Blueprints/BP_Elevator/BP_Door_Right.BP_Door_Right_C"))
    (`/Game/Blueprints/BP_Elevator/BP_Door_Right.closeDoor` _returnvalue_2)
    (else
      (`SceneComponent.K2_SetRelativeRotation` (`self.StaticMeshComponent`) (struct :`Pitch` 180.0) false false)
      (`KismetSystemLibrary.Delay` 4.0)
      (bind _returnvalue_3 (`GameplayStatics.GetActorOfClass` "/Game/Blueprints/BP_Elevator/BP_Door_Left.BP_Door_Left_C"))
      (`/Game/Blueprints/BP_Elevator/BP_Door_Left.openDoor` _returnvalue_3)
      (bind _returnvalue_4 (`GameplayStatics.GetActorOfClass` "/Game/Blueprints/BP_Elevator/BP_Door_Right.BP_Door_Right_C"))
      (`/Game/Blueprints/BP_Elevator/BP_Door_Right.openDoor` _returnvalue_4))))

(event `self.ReceiveBeginPlay`
  ;[1 1 1] Choose a random type of button and set the static mesh of the button accordingly
  (if (`self.innen`)
    (bind _returnvalue (`GameplayStatics.GetActorOfClass` "/Game/Blueprints/BP_Elevator/BP_LevelDatabase.BP_LevelDatabase_C"))
    (`StaticMeshComponent.SetStaticMesh` (`self.StaticMeshComponent`) (`|GetArrayItem` (`|MakeArray` "/Game/Materials_Randomise/Meshes/elevator/Leuchtrand/Taste_Leuchtrand_innen_halbrund.Taste_Leuchtrand_innen_halbrund" "/Game/Materials_Randomise/Meshes/elevator/Leuchtrand/Taste_Leuchtrand_innen_rechteckig.Taste_Leuchtrand_innen_rechteckig" "/Game/Materials_Randomise/Meshes/elevator/Leuchtrand/Taste_Leuchtrand_innen_rechteckig_IL.Taste_Leuchtrand_innen_rechteckig_IL" "/Game/Materials_Randomise/Meshes/elevator/Leuchtrand/Taste_Leuchtrand_innen_rund.Taste_Leuchtrand_innen_rund" :!type "StaticMesh Object Reference") (`/Game/Blueprints/BP_Elevator/BP_LevelDatabase.randomInt` _returnvalue)))
    (else
      (`StaticMeshComponent.SetStaticMesh` (`self.StaticMeshComponent`) (`|GetArrayItem` (`|MakeArray` "/Game/Materials_Randomise/Meshes/elevator/Leuchtrand/Taste_Leuchtrand__außen_halbrund.Taste_Leuchtrand__außen_halbrund" "/Game/Materials_Randomise/Meshes/elevator/Leuchtrand/Taste_Leuchtrand_außen_rechteckig.Taste_Leuchtrand_außen_rechteckig" "/Game/Materials_Randomise/Meshes/elevator/Leuchtrand/Taste_Leuchtrand_außen_rechteckig_IL.Taste_Leuchtrand_außen_rechteckig_IL" "/Game/Materials_Randomise/Meshes/elevator/Leuchtrand/Taste_Leuchtrand_außen_rund.Taste_Leuchtrand_außen_rund" :!type "StaticMesh Object Reference") (`KismetMathLibrary.RandomInteger` 4))))))

(fn `UserConstructionScript`)