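; Wheelchair user character whose neck pose follows a VR head actor and which can eat food.
; BeginPlay enables neck posing in its animation Blueprint; Tick feeds it the head's transform with a fixed neck-to-eyes offset.
; The head is looked up by class on first Tick because the other reference is destroyed in replay.
; Food touching the mouth snaps to a Stomach socket; construction configures the optional head proxy and table.
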(event `self.ReceiveBeginPlay`
  (bind _aswheelchair_user_anim_blueprint (cast `/Game/Blueprints/BP_WheelchairUser/Character/Mesh/WheelchairUser_AnimBlueprint` (`SkeletalMeshComponent.GetAnimInstance` (`self.SkeletalMesh`)))
    (:`then`
      (bind _output_get (set `self.Animation_BP` _aswheelchair_user_anim_blueprint))
      (set `/Game/Blueprints/BP_WheelchairUser/Character/Mesh/WheelchairUser_AnimBlueprint.TransformNeckPose` true _output_get)
      (set `/Game/Blueprints/BP_WheelchairUser/Character/Mesh/WheelchairUser_AnimBlueprint.RootWorldHeight` (.z (.location (`SceneComponent.K2_GetComponentToWorld` (`self.SkeletalMesh`)))) _output_get))
    (:`CastFailed`
      (`self.SetActorTickEnabled` false) ; Deactive Tick if not necessary
      (`KismetSystemLibrary.PrintString` "Unexpected WheelchairUser Animation Blueprint"))))

(event `self.ReceiveTick`
  (params (DeltaSeconds :type "Float (single-precision)"))
  ;[1 1 1] First Tick: Store reference to Head (needs to be done here as the other reference is being destroyed in replay). Then align Head Transforms
  (`|ExecutionSequence`
    (:`then_0`
      (`/Engine/EditorBlueprintResources/StandardMacros.DoOnce` false
        (:`Completed`
          (bind _returnvalue (`GameplayStatics.GetActorOfClass` "/Game/Blueprints/BP_WheelchairUser/ressources/BP_WheelchairUser_Head.BP_WheelchairUser_Head_C"))
          (set `self.VR_Head_Component` _returnvalue))))
    (:`then_1`
      (set `/Game/Blueprints/BP_WheelchairUser/Character/Mesh/WheelchairUser_AnimBlueprint.HeadTransform` (`KismetMathLibrary.ComposeTransforms` (`KismetMathLibrary.MakeTransform` (-9.283613 0.0 -15.0) (struct :`Pitch` 74.651344 :`Roll` 90.0)) (`SceneComponent.K2_GetComponentToWorld` (`Actor.RootComponent` (`self.VR_Head_Component`)))) (`self.Animation_BP`)))))

(event `self.MouthOverlap.OnComponentBeginOverlap`
  (params (OverlappedComponent :type "PrimitiveComponent Object Reference") (OtherActor :type "Actor Object Reference") (OtherComp :type "PrimitiveComponent Object Reference") (OtherBodyIndex :type Integer) (bFromSweep :type Boolean) (SweepResult :type "HitResult Structure (by ref)"))
  ;[1 1 1] Enable Eating Food
  (if (`self.ActorHasTag` OtherActor "Food")
    (`self.K2_AttachToComponent` OtherActor (`self.SkeletalMesh`) "Stomach" "SnapToTarget" "SnapToTarget" "SnapToTarget" true)))

(fn `UserConstructionScript`
  (`ChildActorComponent.SetChildActorClass` (`self.HeadProxy`) (select `bool` (`self.CreatesHeadProxy`) :`true` "/Game/Blueprints/BP_WheelchairUser/ressources/BP_WheelchairUser_Head.BP_WheelchairUser_Head_C" :!type "Actor Class Reference"))
  ;[1 1 1] Handle Wheelchair Table
  (if (not (`self.HasTable`))
    (`ChildActorComponent.SetChildActorClass` (`self.Table`) null)))