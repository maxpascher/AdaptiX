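; Head actor of the wheelchair user, carrying a Google Glass mesh and an RGB camera whose images can be saved as JPGs.
; A low-resolution render target is created for the camera at BeginPlay, and the camera activates only during replay with headset image storage enabled.
; Outside replay, active VR hides the glasses and enables the otherwise disabled Tick, which snaps the mesh to the VR pawn's camera.
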(event `self.ReceiveBeginPlay`
  (bind _returnvalue (`KismetRenderingLibrary.CreateRenderTarget2D` 424 240 "RTF_RGBA8"))
  (set `Texture.LODGroup` "TEXTUREGROUP_Pixels2D" _returnvalue)
  (set `SceneCaptureComponent2D.TextureTarget` _returnvalue (`self.RGB_cam`))
  (if (`Storage.GetPlayReplay`)
    ;[1 1 1] In Replay: Activat e the Camera, if defined by setup file
    (if (`Storage.GetStorage_Activated_Headset_Images`)
      (`self.ActivateCamera`))
    (else
      ;[1 1 1] If VR is used, store reference to VR-Headset, enable tick and hide headset
      (bind _returnvalue_2 (`GameplayStatics.GetActorOfClass` "/Game/Blueprints/BP_JacoArm/BP_VR_Pawn.BP_VR_Pawn_C"))
      (if (and (!= _returnvalue_2 null) (`HeadMountedDisplayFunctionLibrary.IsHeadMountedDisplayEnabled`))
        (set `self.HMD_Reference` (`/Game/Blueprints/BP_JacoArm/BP_VR_Pawn.VRCamera` _returnvalue_2))
        (`self.SetActorTickEnabled` true)
        (`SceneComponent.SetVisibility` (`self.GoogleGlass`) false false)))))

(event `self.ReceiveTick`
  (params (DeltaSeconds :type "Float (single-precision)"))
  ;[1 1 1] Tick Deactivated by default. Only if VR is used, position this actor at user's head
  (`SceneComponent.K2_SetWorldTransform` (`self.StaticMeshComponent`) (`SceneComponent.K2_GetComponentToWorld` (`self.HMD_Reference`)) false true))

(fn `ActivateCamera`
  (`ActorComponent.Activate` (`self.RGB_cam`) false))

(fn `Error Storing Image to Disk`
  (params (bSuccess :type Boolean))
  (if (not bSuccess)
    (`KismetSystemLibrary.PrintString` "Error: Error storing image to disk in WheelchairUser_Head" true true (struct :`R` 1.0 :`A` 1.0) 2000000.0)))

(fn `StoreImage`
  (params (path :type String))
  (bind _returnvalue (`Storage.GetStoragePath`))
  (`ImageWriteBlueprintLibrary.ExportToDisk` (`SceneCaptureComponent2D.TextureTarget` (`self.RGB_cam`)) (`KismetStringLibrary.Concat_StrStr` _returnvalue path (`self.Headset_Image_Filenames`)) (make `ImageWriteOptions` "JPG" (`|CreateDelegate` :!event `Error Storing Image to Disk`) 0 true false)))

(fn `UserConstructionScript`)