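; Gizmo actor for replays that attaches to the Jaco robot arm's end effector and derives the adaptive axis from the arm's observed movement.
; Each tick it records the EE pose and finger closure, then turns the latest delta into a remapped location, rotation and gripper vector.
; Motions above a threshold are normalised, averaged over recent samples, blended with the previous result and written to PlayerPawn's AdaptiveSet before parent Tick runs.
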(event EventBeginPlay
  (|CallParentFunction)
  (Variables|Default|SetArrowMaterial "/Game/WHS_HCI_Study/Material/M_Beam_Color.M_Beam_Color"))

(event EventTick
  (params (DeltaSeconds :type Float%20%28single-precision%29))
  (Utilities|FlowControl|Sequence
    (:then_0
      (Utilities|FlowControl|DoOnce false
        (:Completed
          (|CallParentFunction)
          (Transformation|AttachActorToActor (Variables|Default|GetJaco) "EE" "SnapToTarget" "SnapToTarget" "SnapToTarget" true)
          (Transformation|SetActorRelativeRotation "0,-90.000000, 0"))))
    (:then_1
      (|SetAdaptiveAxisBasedOnMovement))
    (:then_2
      (|CallParentFunction DeltaSeconds))))

(fn ConstructionScript
  (|CallParentFunction))

(fn NormaliseAdaptive
  (params (in :type Adaptive%20Axis%20Structure))
  (bind (_location _rotation _gripper) (Utilities|Struct|BreakAdaptiveAxis in))
  (bind _returnvalue (|(sqrt((((((((a*a)+(b*b))+(c*c))+(d*d))+(e*e))+(f*f))+(g*g)))) (.x _location) (.y _location) (.z _location) (.roll _rotation) (.pitch _rotation) (.yaw _rotation) _gripper))
  (return (Utilities|Struct|MakeAdaptiveAxis (Math|Vector|MakeVector (Math|Float|SafeDivide (.x _location) _returnvalue) (Math|Float|SafeDivide (.y _location) _returnvalue) (Math|Float|SafeDivide (.z _location) _returnvalue)) (Math|Rotator|MakeRotator (Math|Float|SafeDivide (.roll _rotation) _returnvalue) (Math|Float|SafeDivide (.pitch _rotation) _returnvalue) (Math|Float|SafeDivide (.yaw _rotation) _returnvalue)) (Math|Float|SafeDivide _gripper _returnvalue)) _returnvalue))

(fn CalculateAverageAxis
  (params (maxElements :type Integer))
  (bind _directions (Variables|Default|GetDirections))
  (bind _returnvalue (Utilities|Array|LastIndex _directions))
  (for _index (range (Math|Integer|Clamp(Integer) (- _returnvalue maxElements) 0 _returnvalue) _returnvalue)
    (LocalVariables|SetLocalSummant (CallFunction|Add (LocalVariables|GetLocalSummant) (Utilities|Array|Get(acopy) (Variables|Default|GetDirections) _index))))
  (return (CallFunction|Divide (LocalVariables|GetLocalSummant) (Math|Integer|Min(Integer) maxElements (Utilities|Array|Length _directions)))))

(fn Add
  (params (A :type Adaptive%20Axis%20Structure) (B :type Adaptive%20Axis%20Structure))
  (bind (_location _rotation _gripper) (Utilities|Struct|BreakAdaptiveAxis B))
  (bind (_location_2 _rotation_2 _gripper_2) (Utilities|Struct|BreakAdaptiveAxis A))
  (return (Utilities|Struct|MakeAdaptiveAxis (+ _location_2 _location) (Math|Rotator|MakeRotator (+ (.roll _rotation_2) (.roll _rotation)) (+ (.pitch _rotation_2) (.pitch _rotation)) (+ (.yaw _rotation_2) (.yaw _rotation))) (+ _gripper_2 _gripper))))

(fn Divide
  (params (A :type Adaptive%20Axis%20Structure) (B :type Integer))
  (bind (_location _rotation _gripper) (Utilities|Struct|BreakAdaptiveAxis A))
  (bind _returnvalue (Math|Conversions|ToFloat(Integer) B))
  (return (Utilities|Struct|MakeAdaptiveAxis (/ _location B) (Math|Rotator|MakeRotator (/ (.roll _rotation) _returnvalue) (/ (.pitch _rotation) _returnvalue) (/ (.yaw _rotation) _returnvalue)) (/ _gripper _returnvalue))))

(fn GetLastMotion
  (bind _fingervs (Variables|Default|GetFingerVs))
  (bind _poses (Variables|Default|GetPoses))
  (bind _returnvalue (Utilities|Array|LastIndex _poses))
  (bind _returnvalue_2 (Utilities|Array|LastIndex _poses))
  (bind _returnvalue_3 (- _returnvalue_2 1))
  (bind _output (Utilities|Array|Get(acopy) _poses _returnvalue))
  (bind _returnvalue_4 (Math|Transform|InvertTransform _output))
  (bind _output_2 (Utilities|Array|Get(acopy) _poses _returnvalue_3))
  (bind _returnvalue_5 (Math|Transform|ComposeTransforms _output_2 _returnvalue_4))
  (return (Utilities|Struct|MakeAdaptiveAxis (Math|Vector|MakeVector (.y (.location _returnvalue_5)) (* -1 (.x (.location _returnvalue_5))) (* -1 (.z (.location _returnvalue_5)))) (Math|Rotator|MakeRotator (.pitch (.rotation _returnvalue_5)) (* -1 (.roll (.rotation _returnvalue_5))) (* -1 (.yaw (.rotation _returnvalue_5)))) (* (- (Utilities|Array|Get(acopy) _fingervs _returnvalue) (Utilities|Array|Get(acopy) _fingervs _returnvalue_3)) 5e+01))))