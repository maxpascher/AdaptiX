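; BP_VideoCam is a scene capture camera actor that records video as a numbered PNG image sequence.
; If a file path is set and Record is on, it enables ticking, tags itself to tick during replays, and exports its capture render target every frame.
; With SnapToHead on, its first tick attaches it to the BP_WheelchairUser_Head actor at a configurable relative transform.
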(event `self.ReceiveBeginPlay`
  (if (`KismetStringLibrary.IsEmpty` (`self.FilePath`))
    (`KismetSystemLibrary.PrintString` "Video not rendered as file path was not defined" true true (struct :`R` 1.0 :`B` 0.496706 :`A` 1.0) 20000000.0)
    (else
      (`self.SetActorTickEnabled` (`self.Record`))
      (if (`self.Record`)
        (`KismetArrayLibrary.Array_Add` (`self.Tags`) "TickDuringReplay")))))

(event `self.ReceiveTick`
  (params (DeltaSeconds :type "Float (single-precision)"))
  (`|ExecutionSequence`
    (:`then_0`
      (`/Engine/EditorBlueprintResources/StandardMacros.DoOnce` false
        (:`Completed`
          (if (`self.SnapToHead`)
            (bind _returnvalue (`GameplayStatics.GetActorOfClass` "/Game/Blueprints/BP_WheelchairUser/ressources/BP_WheelchairUser_Head.BP_WheelchairUser_Head_C"))
            (`self.K2_AttachToActor` _returnvalue "None" "SnapToTarget" "SnapToTarget" "SnapToTarget")
            (`self.K2_SetActorRelativeTransform` (`self.RelativeTransformToHead`) false true)))))
    (:`then_1`
      (`KismetRenderingLibrary.ExportRenderTarget` (`SceneCaptureComponent2D.TextureTarget` (`self.CaptureComponent2D`)) (`self.FilePath`) (`KismetStringLibrary.Concat_StrStr` (`KismetStringLibrary.Conv_IntToString` (`self.ImageCounter`)) ".png"))
      (`/Engine/EditorBlueprintResources/StandardMacros.IncrementInt` (`self.ImageCounter`)))))

(fn `UserConstructionScript`)