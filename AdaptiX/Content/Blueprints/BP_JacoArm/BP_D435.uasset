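; BP_D435 is a simulated D435 camera that renders and saves RGB, depth and segmentation images.
; BeginPlay creates low- or high-res render targets and activates the captures when image storage and replay are both enabled.
; Segmentation writes SegmentTable IDs into custom depth stencils by actor tag, with component tags overriding per mesh.
; StoreImages exports each camera to disk, saving float depth separately from the 8-bit images.
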(event `self.ReceiveBeginPlay`
  (bind _rgb_cam (`self.RGB_Cam`))
  (bind _depth_cam (`self.Depth_Cam`))
  (bind _segment_cam (`self.Segment_Cam`))
  ;[1 1 1] BeginPlay
  (bind _returnvalue (`Storage.GetImagesInHighRes`))
  (`self.SetCameraTarget` (`self.RGB_Cam`) true _returnvalue)
  (`self.SetCameraTarget` (`self.Depth_Cam`) false _returnvalue)
  (`self.SetCameraTarget` (`self.Segment_Cam`) true _returnvalue)
  (`ActorComponent.Deactivate` (`self.ViewpointCamera`))
  (bind _returnvalue_2 (`Storage.GetStorage_Activated_Images`))
  (if (and _returnvalue_2 (`Storage.GetPlayReplay`))
    (`self.ActivateCameras`))
  (set `self.output_Filenames` (`|MakeMap` _rgb_cam (`KismetStringLibrary.Concat_StrStr` (`self.outFile_prefix`) (`self.RGB_Filename_Suffix`)) _depth_cam (`KismetStringLibrary.Concat_StrStr` (`self.outFile_prefix`) (`self.Depth_Filename_Suffix`)) _segment_cam (`KismetStringLibrary.Concat_StrStr` (`self.outFile_prefix`) (`self.Segment_:Filename_Suffix`))))
  (set `self.output_Fileformats` (`|MakeMap` _rgb_cam "JPG" _depth_cam "PNG" _segment_cam "PNG" :!valuetype "EDesiredImageFormat Enum"))
  (`self.SetSegmentation IDs`))

(fn `ActivateCameras`
  (for _array_element (`|MakeArray` (`self.RGB_Cam`) (`self.Depth_Cam`) (`self.Segment_Cam`))
    (`ActorComponent.Activate` _array_element false)
    (set `SceneCaptureComponent.bCaptureEveryFrame` true _array_element)))

(fn `Error Storing Image to Disk`
  (params (bSuccess :type Boolean))
  (if (not bSuccess)
    (`KismetSystemLibrary.PrintString` "Error: Error storing image to disk in BP_D435" true true (struct :`R` 1.0 :`A` 1.0) 2000000.0)))

(fn `SetSegmentation IDs`
  ;[1 1 1] Set Segmentation IDs
  (bind _outactors (`GameplayStatics.GetAllActorsOfClass` "/Script/Engine.Actor"))
  (for _array_element _outactors
    (bind _returnvalue (`self.K2_GetComponentsByClass` _array_element "/Script/Engine.MeshComponent"))
    ;;[1 1 1] Set Standard Value to 0
    (`PrimitiveComponent.SetRenderCustomDepth` _returnvalue true)
    (`PrimitiveComponent.SetCustomDepthStencilValue` _returnvalue 0)
    ;;[1 1 1] Set Custom Value
    (for _array_element_2 (`Actor.Tags` _array_element)
      (bind _returnvalue_2 (`|GetDataTableRow` "/Game/Structs/SegmentTable.SegmentTable" _array_element_2)
        (:`then`
          (`PrimitiveComponent.SetCustomDepthStencilValue` _returnvalue (`.SegmentID_6_D9878BF5477144A3CA0B628152D8823A` (break `/Game/Structs/Struct_Segment` _returnvalue_2)))
          (break))))
    ;;[1 1 1] Enable Componentwise Segments
    (for _array_element_3 _returnvalue
      (for _array_element_4 (`ActorComponent.ComponentTags` _array_element_3)
        (bind _returnvalue_3 (`|GetDataTableRow` "/Game/Structs/SegmentTable.SegmentTable" _array_element_4)
          (:`then`
            (`PrimitiveComponent.SetCustomDepthStencilValue` _array_element_3 (`.SegmentID_6_D9878BF5477144A3CA0B628152D8823A` (break `/Game/Structs/Struct_Segment` _returnvalue_3)))
            (break)))))))

(fn `StoreImages`
  (params (path :type String))
  (bind _returnvalue (`Storage.GetStoragePath`))
  (for _array_element (`|MakeArray` (`self.RGB_Cam`) (`self.Depth_Cam`) (`self.Segment_Cam`))
    (bind _texturetarget (`SceneCaptureComponent2D.TextureTarget` _array_element))
    (switch `ETextureRenderTargetFormat` (`TextureRenderTarget2D.RenderTargetFormat` _texturetarget)
      (:`RTF_RGBA8`
        (bind _returnvalue_2 (`KismetStringLibrary.Concat_StrStr` _returnvalue path))
        (bind _value (`BlueprintMapLibrary.Map_Find` (`self.output_Filenames`) _array_element))
        (`ImageWriteBlueprintLibrary.ExportToDisk` _texturetarget (`KismetStringLibrary.Concat_StrStr` _returnvalue_2 _value) (make `ImageWriteOptions` (`BlueprintMapLibrary.Map_Find` (`self.output_Fileformats`) _array_element) (`|CreateDelegate` :!event `Error Storing Image to Disk`) 0 true false)))
      (:`RTF_RGBA16f`
        (`KismetRenderingLibrary.ExportRenderTarget` _texturetarget _returnvalue_2 _value) ; Depth needs to be stored differently, as it is float
      ))))

(fn `UserConstructionScript`
  (`ActorComponent.SetAutoActivate` (`self.ViewpointCamera`) (`self.EnableViewpointCamera`)))