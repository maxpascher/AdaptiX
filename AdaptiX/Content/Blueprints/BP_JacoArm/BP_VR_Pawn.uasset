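; Player pawn for VR or desktop that teleoperates a Jaco robot arm linked to the right controller mesh.
; BeginPlay sets up cameras and a wrist or screen HUD for camera feeds; input axes move the controller and gripper.
; For adaptive control, MachineLearningRemote sends D435 RGB, depth and segment images as JSON to a Python CNN.
; Returned directions become selectable pairs of input axes; the pawn also triggers GameMode recording.
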(fn `Adaptive Movement`
  (params (AxisValue :type "Float (double-precision)") (Axis :type "/Game/Structs/AdaptiveAxis Structure"))
  (bind (_location _rotation _gripper) (break `/Game/Structs/AdaptiveAxis` Axis))
  (bind _jaco (`self.Jaco`))
  (`SceneComponent.K2_AddLocalTransform` (`self.RightHandMotionController`) (`KismetMathLibrary.MakeTransform` (* (* _location AxisValue) (`self.Vel_Trans`)) (* (* _rotation AxisValue) (`self.Vel_Rot`))) true false)
  (if (!= _jaco null)
    (`/Game/Blueprints/BP_JacoArm/Jaco.Grasp` _jaco (* _gripper AxisValue))))

(fn `SendInputToCNN`
  (bind _jaco (`self.Jaco`))
  (if (!= _jaco null)
    (bind _asbp_d435 (cast `/Game/Blueprints/BP_JacoArm/BP_D435` (`ChildActorComponent.ChildActor` (`/Game/Blueprints/BP_JacoArm/Jaco.CameraAbove` _jaco))))
    (`MachineLearningBaseComponent.SendStringInput` (`self.MachineLearningRemote`) (`KismetStringLibrary.Concat_StrStr` "{" "\"rgb\":" (`Storage.Conv_RenderTargetTextureToJSON` (`SceneCaptureComponent2D.TextureTarget` (`/Game/Blueprints/BP_JacoArm/BP_D435.RGB_Cam` _asbp_d435))) ", " "\"depth\":" (`Storage.Conv_RenderTargetTextureToJSON` (`SceneCaptureComponent2D.TextureTarget` (`/Game/Blueprints/BP_JacoArm/BP_D435.Depth_Cam` _asbp_d435)) true) ", " "\"segments\":" (`Storage.Conv_RenderTargetTextureToJSON` (`SceneCaptureComponent2D.TextureTarget` (`/Game/Blueprints/BP_JacoArm/BP_D435.Segment_Cam` _asbp_d435)) true) "}") "calculateCNN")))

(fn `ToggleAdaptiveAxesVisualisation`
  (locals (VisualiseAxis :type Boolean :default false))
  (for _array_element (`|MakeArray` (`self.AdaptiveDirectionArrow1`) (`self.AdaptiveDirectionArrow0`))
    (bind _output_get (set `local.VisualiseAxis` (not (`SceneComponent.IsVisible` _array_element))))
    (`self.SetActorTickEnabled` (`ChildActorComponent.ChildActor` _array_element) _output_get)
    (`SceneComponent.SetVisibility` _array_element _output_get false)))

(fn `UserConstructionScript`)