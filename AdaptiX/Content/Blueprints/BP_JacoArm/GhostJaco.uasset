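; GhostJaco is a physics-simulated Jaco robot arm with a three-finger gripper, posed through its animation Blueprint.
; BeginPlay builds physics constraints at the EE socket; ConnectToMotionController binds the wrist to a motion controller, optionally with soft drives.
; SetCompletePose applies supplied joint and finger states, while Grasp input incrementally opens the fingers.
; Gripper closing, pinch detection, object attach/release and collision disabling are stubbed, their logic left unconnected.
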(event `self.ReceiveBeginPlay`
  (bind _graspedobjectphysicsconstraint (`self.GraspedObjectPhysicsConstraint`))
  (bind _motioncontrollerconnector (`self.MotionControllerConnector`))
  (bind _returnvalue (`AddComponent|NODE_AddPhysicsConstraintComponent-1` :`bManualAttachment` true))
  (bind _output_get (set `self.MotionControllerConnector` _returnvalue))
  (`SceneComponent.K2_AttachToComponent` _output_get (`self.SkeletalMeshComponent`) "EE" "SnapToTarget" "SnapToTarget" "SnapToTarget" true)
  (`PhysicsConstraintComponent.SetDisableCollision` (`self.MotionControllerConnector`) true)
  (`PhysicsConstraintComponent.SetLinearXLimit` _motioncontrollerconnector "LCM_Locked" 0.0)
  (`PhysicsConstraintComponent.SetLinearYLimit` _motioncontrollerconnector "LCM_Locked" 0.0)
  (`PhysicsConstraintComponent.SetLinearZLimit` _motioncontrollerconnector "LCM_Locked" 0.0)
  (`PhysicsConstraintComponent.SetAngularSwing1Limit` _motioncontrollerconnector "ACM_Locked" 0.0)
  (`PhysicsConstraintComponent.SetAngularSwing2Limit` _motioncontrollerconnector "ACM_Locked" 0.0)
  (`PhysicsConstraintComponent.SetAngularTwistLimit` _motioncontrollerconnector "ACM_Locked" 0.0)
  (bind _returnvalue_2 (`AddComponent|NODE_AddPhysicsConstraintComponent-2` :`bManualAttachment` true))
  (bind _output_get_2 (set `self.GraspedObjectPhysicsConstraint` _returnvalue_2))
  (`SceneComponent.K2_AttachToComponent` _output_get_2 (`self.SkeletalMeshComponent`) "EE" "SnapToTarget" "SnapToTarget" "SnapToTarget" true)
  (`PhysicsConstraintComponent.SetDisableCollision` (`self.GraspedObjectPhysicsConstraint`) true)
  (`PhysicsConstraintComponent.SetLinearXLimit` _graspedobjectphysicsconstraint "LCM_Free" 0.0)
  (`PhysicsConstraintComponent.SetLinearYLimit` _graspedobjectphysicsconstraint "LCM_Free" 0.0)
  (`PhysicsConstraintComponent.SetLinearZLimit` _graspedobjectphysicsconstraint "LCM_Free" 0.0)
  (`PhysicsConstraintComponent.SetAngularSwing1Limit` _graspedobjectphysicsconstraint "ACM_Free" 0.0)
  (`PhysicsConstraintComponent.SetAngularSwing2Limit` _graspedobjectphysicsconstraint "ACM_Free" 0.0)
  (`PhysicsConstraintComponent.SetAngularTwistLimit` _graspedobjectphysicsconstraint "ACM_Free" 0.0)
  (if (not (`self.EnableElbowConstraint`))
    (`PhysicsConstraintComponent.BreakConstraint` (`self.HighElbowConstraint`)))
  (`SceneComponent.SetHiddenInGame` (`self.Bracelet`) (not (`self.ShowCameraInGame`)) false)
  (`SceneComponent.SetHiddenInGame` (`self.CameraAbove`) (not (`self.ShowCameraInGame`)) false)
  (`PrimitiveComponent.SetSimulatePhysics` (`self.SkeletalMeshComponent`) true) ; Needs to be defined here to allow alternative spawns
  (`PrimitiveComponent.SetConstraintMode` (`self.SkeletalMeshComponent`) "Default")
  (`PrimitiveComponent.SetConstraintMode` (`self.SkeletalMeshComponent`) "Default")
  (bind _asjaco_anim_blueprint (cast `/Game/Blueprints/BP_JacoArm/JacoResources/Jaco_AnimBlueprint` (`SkeletalMeshComponent.GetAnimInstance` (`self.SkeletalMeshComponent`))))
  (set `self.Animation Blueprint` _asjaco_anim_blueprint))

(event `self.ReceiveTick`
  (params (DeltaSeconds :type "Float (single-precision)")))

(fn `BoxColliding`
  (params (collider :type "BoxComponent Object Reference"))
  (returns (isPinching :type Boolean) (pinchedObject :type "StaticMeshActor Object Reference"))
  (locals (foundActor :type "StaticMeshActor Object Reference") (collisionFound :type Boolean)))

(fn `Connect to Motion Controller`
  (params (MotionController :type "StaticMeshComponent Object Reference") (HideController :type Boolean :default true) (softLocation :type Boolean :default true) (softRotation :type Boolean :default true))
  (bind _motioncontrollerconnector (`self.MotionControllerConnector`))
  (if HideController
    (`SceneComponent.SetVisibility` MotionController false false) ; Hide Controller
  )
  (`PhysicsConstraintComponent.SetConstrainedComponents` _motioncontrollerconnector (`self.SkeletalMeshComponent`) "joint7" MotionController "None")
  (`PhysicsConstraintComponent.SetConstraintReferenceFrame` _motioncontrollerconnector "Frame2" (`KismetMathLibrary.MakeTransform` (0.0 0.0 0.0) (struct :`Roll` 90.0))) ; Align origins independant of motion controller orientation
  (if softLocation
    ;[1 1 1] SoftLocation with motor
    (`PhysicsConstraintComponent.SetLinearXLimit` _motioncontrollerconnector "LCM_Free" 0.0)
    (`PhysicsConstraintComponent.SetLinearYLimit` _motioncontrollerconnector "LCM_Free" 0.0)
    (`PhysicsConstraintComponent.SetLinearZLimit` _motioncontrollerconnector "LCM_Free" 0.0)
    (`PhysicsConstraintComponent.SetLinearDriveParams` _motioncontrollerconnector 500.0 300.0 0.0)
    (`PhysicsConstraintComponent.SetLinearPositionDrive` _motioncontrollerconnector true true true)
    (`PhysicsConstraintComponent.SetLinearVelocityDrive` _motioncontrollerconnector true true true))
  (if softRotation
    ;[1 1 1] SoftRotation with motor
    (`PhysicsConstraintComponent.SetAngularSwing1Limit` _motioncontrollerconnector "ACM_Free" 0.0)
    (`PhysicsConstraintComponent.SetAngularSwing2Limit` _motioncontrollerconnector "ACM_Free" 0.0)
    (`PhysicsConstraintComponent.SetAngularTwistLimit` _motioncontrollerconnector "ACM_Free" 0.0)
    (`PhysicsConstraintComponent.SetAngularDriveMode` _motioncontrollerconnector "SLERP")
    (`PhysicsConstraintComponent.SetAngularDriveParams` _motioncontrollerconnector 5000.0 100.0 0.0)
    (`PhysicsConstraintComponent.SetAngularVelocityDriveSLERP` _motioncontrollerconnector true)
    (`PhysicsConstraintComponent.SetOrientationDriveSLERP` _motioncontrollerconnector true))
  (if (`self.ConnectOnlyWrist`)
    (`SkeletalMeshComponent.SetConstraintProfile` (`self.SkeletalMeshComponent`) "UserConstraint_5" "Hand" false)))

(fn `DisableCollisionAndPhysics`)

(fn `GetEEPose`
  (returns (EEPose :type "Transform Structure"))
  (return (`KismetMathLibrary.ComposeTransforms` (`SceneComponent.K2_GetComponentToWorld` (`self.MotionControllerConnector`)) (`KismetMathLibrary.InvertTransform` (`SceneComponent.K2_GetComponentToWorld` (`self.SkeletalMeshComponent`))))))

(fn `Grasp`
  (params (graspVelocity :type "Float (double-precision)"))
  (locals (ObjectToGrasp :type "StaticMeshActor Object Reference"))
  (bind _returnvalue (`KismetMathLibrary.FClamp` graspVelocity -1.0))
  (bind _returnvalue_2 (> (`KismetMathLibrary.Abs` _returnvalue) (`self.Min Finger Value`)))
  (bind _returnvalue_3 (select `bool` _returnvalue_2 :`true` _returnvalue))
  (if _returnvalue_2
    (if (not (> _returnvalue 0.0))
      (for _index (range 1 4)
        (`self.Move and Set Finger` _index _returnvalue_3)
        (`self.Move And Set Finger Tip` _index _returnvalue_3))
      (if (and (!= (`self.GraspedObject`) null) (or (and (== (`self.Finger1State`) 0.0) (== (`self.FingerTip1State`) 0.0)) (and (not (`self.BoxColliding` (`self.FingerTip1_Box`))) (not (`self.BoxColliding` (`self.Finger1_Box`))))))
        (`self.Release Grasped Object`)))))

(fn `Move and Set Finger`
  (params (FingerNumber :type Integer) (graspInput :type "Float (double-precision)"))
  (bind _returnvalue (`KismetMathLibrary.FClamp` (+ (* graspInput (`self.FingerVelocity`)) (select `int` (- FingerNumber 1) :`0` (`self.Finger1State`) :`1` (`self.Finger2State`) :`2` (`self.Finger3State`)))))
  (switch `int` FingerNumber
    (:`Default`
      (`KismetSystemLibrary.PrintString` "Error: FingerIndex in MoveFinger needs to be >0 and <4" true true (struct :`R` 1.0 :`A` 1.0) 200000.0))
    (:`1`
      (set `self.Finger1State` _returnvalue)
      (`self.SetFinger` FingerNumber (select `int` (- FingerNumber 1) :`0` (`self.Finger1State`) :`1` (`self.Finger2State`) :`2` (`self.Finger3State`)) :!label _label))
    (:`2`
      (set `self.Finger2State` _returnvalue)
      (goto _label))
    (:`3`
      (set `self.Finger3State` _returnvalue)
      (goto _label))))

(fn `Move And Set Finger Tip`
  (params (FingerNumber :type Integer) (graspInput :type "Float (double-precision)"))
  (bind _returnvalue (`KismetMathLibrary.FClamp` (+ (* graspInput (`self.FingerVelocity`)) (select `int` (- FingerNumber 1) :`0` (`self.FingerTip1State`) :`1` (`self.FingerTip2State`) :`2` (`self.FingerTip3State`)))))
  (switch `int` FingerNumber
    (:`Default`
      (`KismetSystemLibrary.PrintString` "Error: FingerIndex in MoveFinger needs to be >0 and <4" true true (struct :`R` 1.0 :`A` 1.0) 200000.0))
    (:`1`
      (set `self.FingerTip1State` _returnvalue)
      (`self.Set Finger Tip` FingerNumber (select `int` (- FingerNumber 1) :`0` (`self.FingerTip1State`) :`1` (`self.FingerTip2State`) :`2` (`self.FingerTip3State`)) :!label _label))
    (:`2`
      (set `self.FingerTip2State` _returnvalue)
      (goto _label))
    (:`3`
      (set `self.FingerTip3State` _returnvalue)
      (goto _label))))

(fn `PrintEEPose`
  (`KismetSystemLibrary.PrintString` (`KismetStringLibrary.Conv_TransformToString` (`self.GetEEPose`)))
  (return))

(fn `Release Grasped Object`)

(fn `Set Finger Tip`
  (params (FingerNumber :type Integer) (FingerTipState :type "Float (double-precision)"))
  (bind _animation_blueprint (`self.Animation Blueprint`))
  (bind _returnvalue (* FingerTipState (`self.FingerTipRange`) -1.0))
  (switch `int` FingerNumber
    (:`Default`
      (`KismetSystemLibrary.PrintString` "Error: FingerIndex in SetFinger needs to be >0 and <4" true true (struct :`R` 1.0 :`A` 1.0) 200000.0))
    (:`1`
      (set `/Game/Blueprints/BP_JacoArm/JacoResources/Jaco_AnimBlueprint.FingerTip1Angle` _returnvalue _animation_blueprint))
    (:`2`
      (set `/Game/Blueprints/BP_JacoArm/JacoResources/Jaco_AnimBlueprint.FingerTip2Angle` _returnvalue _animation_blueprint))
    (:`3`
      (set `/Game/Blueprints/BP_JacoArm/JacoResources/Jaco_AnimBlueprint.FingerTip3Angle` _returnvalue _animation_blueprint))))

(fn `SetCompletePose`
  (params (jointPoses :type "Array of Transform Structure") (finger1State :type "Float (double-precision)") (fingerTip1State :type "Float (double-precision)") (finger2State :type "Float (double-precision)") (fingerTip2State :type "Float (double-precision)") (finger3State :type "Float (double-precision)") (fingerTip3State :type "Float (double-precision)"))
  (bind _animation_blueprint (`self.Animation Blueprint`))
  (`SceneComponent.K2_SetWorldTransform` (`self.SkeletalMeshComponent`) (`|GetArrayItem` jointPoses) false true)
  (set `/Game/Blueprints/BP_JacoArm/JacoResources/Jaco_AnimBlueprint.Joints` jointPoses _animation_blueprint)
  (set `/Game/Blueprints/BP_JacoArm/JacoResources/Jaco_AnimBlueprint.NonFingerJoints_enabled` true _animation_blueprint)
  (`self.SetFinger` 1 finger1State)
  (`self.SetFinger` 2 finger2State)
  (`self.SetFinger` 3 finger3State)
  (`self.Set Finger Tip` 1 fingerTip1State)
  (`self.Set Finger Tip` 2 fingerTip2State)
  (`self.Set Finger Tip` 3 fingerTip3State))

(fn `SetFinger`
  (params (FingerNumber :type Integer) (FingerState :type "Float (double-precision)"))
  (bind _returnvalue (- FingerNumber 1))
  (bind _animation_blueprint (`self.Animation Blueprint`))
  (bind _returnvalue_2 (* FingerState (`self.FingerRange`) -1.0))
  (switch `int` FingerNumber
    (:`Default`
      (`KismetSystemLibrary.PrintString` "Error: FingerIndex in SetFinger needs to be >0 and <4" true true (struct :`R` 1.0 :`A` 1.0) 200000.0))
    (:`1`
      (bind _output_get (set `/Game/Blueprints/BP_JacoArm/JacoResources/Jaco_AnimBlueprint.Finger1Angle` _returnvalue_2 _animation_blueprint))
      (`SceneComponent.K2_SetRelativeRotation` (select `int` _returnvalue :`0` (`self.Finger1`) :`1` (`self.Finger2`) :`2` (`self.Finger3`)) (`KismetMathLibrary.MakeRotator` 0.0 (* -1 (select `int` _returnvalue :`0` _output_get :`1` (stale _output_get_2) :`2` (stale _output_get_3)))) false false :!label _label))
    (:`2`
      (bind _output_get_2 (set `/Game/Blueprints/BP_JacoArm/JacoResources/Jaco_AnimBlueprint.Finger2Angle` _returnvalue_2 _animation_blueprint))
      (goto _label))
    (:`3`
      (bind _output_get_3 (set `/Game/Blueprints/BP_JacoArm/JacoResources/Jaco_AnimBlueprint.Finger3Angle` _returnvalue_2 _animation_blueprint))
      (goto _label))))

(fn `UserConstructionScript`)