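; Rubber fork actor that picks up food by snapping it to its tip.
; When ForkTipSphere overlaps an actor tagged Food and the tip is empty, that actor attaches to the Tip socket with physics simulation off.
; Its collision object type changes to Jaco's channel to avoid colliding with Jaco's GraspedObjectCollider.
; A held reference whose actor is no longer attached to the fork clears on the next overlap, allowing another pickup.
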(event `self.ForkTipSphere.OnComponentBeginOverlap`
  (params (OverlappedComponent :type "PrimitiveComponent Object Reference") (OtherActor :type "Actor Object Reference") (OtherComp :type "PrimitiveComponent Object Reference") (OtherBodyIndex :type Integer) (bFromSweep :type Boolean) (SweepResult :type "HitResult Structure (by ref)"))
  ;[1 1 1] Check if Tip is Empty
  (if (== (`self.FoodGrasped`) null)
    ;[1 1 1] Check if is Food
    (if (`self.ActorHasTag` OtherActor "Food") :!label _label
      ;[1 1 1] Attach to Tip
      (`self.K2_AttachToComponent` OtherActor (`self.StaticMeshComponent`) "Tip" "SnapToTarget" "KeepWorld" "KeepWorld" true)
      (bind _output_get (set `self.FoodGrasped` OtherActor))
      (`PrimitiveComponent.SetSimulatePhysics` (`self.GetComponentByClass` _output_get "/Script/Engine.PrimitiveComponent") false)
      (`PrimitiveComponent.SetCollisionObjectType` (`self.GetComponentByClass` (`self.FoodGrasped`) "/Script/Engine.PrimitiveComponent") "ECC_GameTraceChannel1") ; Set the Food to be of type Jaco to avoid collision with Jaco's GraspedObjectCollider
    )
    (else
      ;[1 1 1] If Tip has Actor that is no longer attached to the fork, remove reference
      (if (!= (`self.GetAttachParentActor` (`self.FoodGrasped`)) self)
        (set `self.FoodGrasped` null)
        (goto _label)))))

(fn `UserConstructionScript`)