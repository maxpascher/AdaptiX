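; Physics door that the Jaco arm opens by its handle, with meshes and materials randomised at BeginPlay.
; An invisible-handle style proxy drives the visible handle's roll each tick.
; While grasped, the proxy is unhinged, Jaco is constrained to an arc, and the non-simulated door follows the proxy's yaw once open or unlatched.
; On release, constraints swap back and the door swings on its physics hinge or snaps shut.
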(event `self.ReceiveBeginPlay`
  (bind _handleproxymeshcomponent (`self.HandleProxyMeshComponent`))
  (bind _returnvalue (`GameplayStatics.GetActorOfClass` "/Game/Blueprints/BP_JacoArm/Jaco.Jaco_C"))
  (set `self.Jaco` _returnvalue)
  (bind _asstatic_mesh_actor (cast `StaticMeshActor` (`ChildActorComponent.ChildActor` (`self.Door`))))
  (set `self.DoorActor` _asstatic_mesh_actor)
  (set `self.DoorMeshComponent` (`StaticMeshActor.StaticMeshComponent` _asstatic_mesh_actor))
  (bind _asstatic_mesh_actor_2 (cast `StaticMeshActor` (`ChildActorComponent.ChildActor` (`self.HandleProxy`))))
  (set `self.HandleProxyActor` _asstatic_mesh_actor_2)
  (set `self.HandleProxyMeshComponent` (`StaticMeshActor.StaticMeshComponent` _asstatic_mesh_actor_2))
  (bind _asstatic_mesh_actor_3 (cast `StaticMeshActor` (`ChildActorComponent.ChildActor` (`self.Handle`))))
  (bind _output_get (set `self.HandleActor` _asstatic_mesh_actor_3))
  (set `self.HandleMeshComponent` (`StaticMeshActor.StaticMeshComponent` _output_get))
  (`StaticMeshComponent.SetStaticMesh` (`self.DoorMeshComponent`) (`KismetArrayLibrary.Array_Random` (`self.Door Meshes`)))
  (`StaticMeshComponent.SetStaticMesh` (`self.HandleMeshComponent`) (`KismetArrayLibrary.Array_Random` (`self.Handle Meshes`)))
  (`PrimitiveComponent.SetMaterial` (`self.DoorMeshComponent`) 0 (`KismetArrayLibrary.Array_Random` (`self.Door Materials`)))
  (`PrimitiveComponent.SetMaterial` (`self.HandleMeshComponent`) 0 (`KismetArrayLibrary.Array_Random` (`self.Handle Materials`)))
  (`PrimitiveComponent.SetMaterial` (`self.StaticMeshComponent`) 0 (`KismetArrayLibrary.Array_Random` (`self.Frame Materials`)))
  (for _array_element (`|MakeArray` (`self.HandleProxyMeshComponent`) (`self.HandleMeshComponent`) (`self.HandleProxyHinge`) :!type "SceneComponent Object Reference")
    (`SceneComponent.K2_AttachToComponent` _array_element (`self.DoorMeshComponent`) "Handle" "SnapToTarget" "SnapToTarget" "SnapToTarget" true))
  (`PrimitiveComponent.SetSimulatePhysics` _handleproxymeshcomponent true)
  (`PrimitiveComponent.SetEnableGravity` _handleproxymeshcomponent false)
  (set `self.HandleYawRotationOffset` (- (`self.GetHandleProxyRelativeYawRotation`) (`self.InitialDoorOpening`))) ; Initially store offset to be used in handleRotation Function
  (`PhysicsConstraintComponent.SetConstrainedComponents` (`self.DoorHinge`) (`self.DoorMeshComponent`) "None" (`self.StaticMeshComponent`) "None") ; Door Hinge Constraint
  (`PhysicsConstraintComponent.SetAngularSwing1Limit` (`self.DoorHinge`) "ACM_Limited" (`self.MaxDoorRotation_Swing`))
  (`PhysicsConstraintComponent.SetConstraintReferenceFrame` (`self.DoorHinge`) "Frame1" (`KismetMathLibrary.MakeTransform` (0.0 0.0 0.0) (`KismetMathLibrary.MakeRotator` 0.0))) ; Revert Initial opening angle value
  (`SceneComponent.K2_AttachToComponent` (`self.Jaco-on-arc-Constraint`) (`self.DoorMeshComponent`) "Handle" "SnapToTarget" "SnapToTarget" "SnapToTarget" true))

(event `self.ReceiveTick`
  (params (DeltaSeconds :type "Float (single-precision)"))
  (bind _handleproxyhinge (`self.HandleProxyHinge`))
  (bind _returnvalue_roll (`KismetMathLibrary.BreakRotator` (`KismetMathLibrary.InverseTransformRotation` (`SceneComponent.GetSocketTransform` (`self.StaticMeshComponent`) "Door" "RTS_World") (`SceneComponent.K2_GetComponentRotation` (`self.HandleProxyMeshComponent`)))))
  (`SceneComponent.K2_SetRelativeRotation` (`self.HandleMeshComponent`) (`KismetMathLibrary.MakeRotator` (`KismetMathLibrary.FClamp` _returnvalue_roll -15.0 60.0)) false false)
  (if (== (`self.GetAttachParentActor` (`self.HandleProxyActor`)) (`self.Jaco`))
    (`PrimitiveComponent.SetSimulatePhysics` (`self.DoorMeshComponent`) false)
    (`SceneComponent.K2_AttachToComponent` (`self.DoorMeshComponent`) (`self.StaticMeshComponent`) "Door" "SnapToTarget" "KeepWorld" "KeepWorld" true)
    (if (or (> (`self.Get Door Rotation`) 0.5) (`self.IsHandleRolledEnoughToOpenDoor`))
      (`self.K2_SetActorRelativeRotation` (`self.DoorActor`) (`KismetMathLibrary.MakeRotator` 0.0 0.0 (* -1 (`KismetMathLibrary.FClamp` (`self.GetHandleProxyRelativeYawRotation`) 0.0 (`self.MaxDoorRotation_ProxyPull`)))) true false)
      (else
        (`SceneComponent.K2_SetRelativeRotation` :`self` (`self.DoorMeshComponent`))))
    (`|ExecutionSequence`
      (:`then_0`
        (`/Engine/EditorBlueprintResources/StandardMacros.DoOnce` false :!label _label
          (:`Completed`
            (`PhysicsConstraintComponent.BreakConstraint` (`self.HandleProxyHinge`))
            (`PhysicsConstraintComponent.SetConstrainedComponents` (`self.Jaco-on-arc-Constraint`) (`SkeletalMeshActor.SkeletalMeshComponent` (`self.Jaco`)) "joint7" (`self.DoorMeshComponent`) "None"))))
      (:`then_1`
        (goto _label_2 :!via `Reset`)))
    (else
      (`PrimitiveComponent.SetSimulatePhysics` (`self.DoorMeshComponent`) (or (and (> (`self.GetHandleProxyRelativeYawRotation`) 1.0) (> (`self.Get Door Rotation`) 0.01)) (and (`self.IsHandleRolledEnoughToOpenDoor`) (>= (`self.Get Door Rotation`) 0.0))))
      (if (not (`SceneComponent.IsSimulatingPhysics` (`self.DoorMeshComponent`) "None"))
        (`SceneComponent.K2_AttachToComponent` (`self.DoorMeshComponent`) (`self.StaticMeshComponent`) "Door" "SnapToTarget" "SnapToTarget" "KeepWorld" true))
      (`|ExecutionSequence`
        (:`then_0`
          (`/Engine/EditorBlueprintResources/StandardMacros.DoOnce` false :!label _label_2
            (:`Completed`
              (`PhysicsConstraintComponent.SetConstrainedComponents` _handleproxyhinge (`self.HandleProxyMeshComponent`) "None" (`self.DoorMeshComponent`) "None") ; Proxy Handle Hinge Constraint
              (`PhysicsConstraintComponent.SetConstraintReferenceFrame` _handleproxyhinge "Frame1" (`KismetMathLibrary.MakeTransform` (0.0 0.0 0.0))) ; Make sure the constrained is positioned such that horizontal is zero
              (`PhysicsConstraintComponent.BreakConstraint` (`self.Jaco-on-arc-Constraint`)))))
        (:`then_1`
          (goto _label :!via `Reset`))))))

(fn `Get Door Rotation`
  (returns (DoorRotation :type "Float (double-precision)"))
  (bind (_returnvalue_roll _returnvalue_pitch _returnvalue_yaw) (`KismetMathLibrary.BreakRotator` (`KismetMathLibrary.InverseTransformRotation` (`SceneComponent.GetSocketTransform` (`self.StaticMeshComponent`) "Door" "RTS_World") (`SceneComponent.K2_GetComponentRotation` (`self.DoorMeshComponent`)))))
  (return (* -1 _returnvalue_yaw)))

(fn `GetHandleProxyRelativeYawRotation`
  (returns (ReturnValue_Yaw :type "Float (double-precision)"))
  (bind (_returnvalue_roll _returnvalue_pitch _returnvalue_yaw) (`KismetMathLibrary.BreakRotator` (`KismetMathLibrary.Conv_VectorToRotator` (`KismetMathLibrary.InverseTransformLocation` (`SceneComponent.GetSocketTransform` (`self.StaticMeshComponent`) "Door" "RTS_World") (`SceneComponent.K2_GetComponentLocation` (`self.HandleProxyMeshComponent`))))))
  (bind _returnvalue (- (* -1 _returnvalue_yaw) (`self.HandleYawRotationOffset`)))
  (return (`KismetMathLibrary.SelectFloat` (+ _returnvalue 360.0) _returnvalue (< _returnvalue -45.0))))

(fn `IsHandleRolledEnoughToOpenDoor`
  (returns (DoorCanBeOpened :type Boolean))
  (bind _relativerotation_roll (`KismetMathLibrary.BreakRotator` (`SceneComponent.RelativeRotation` (`self.HandleMeshComponent`))))
  (return (>= _relativerotation_roll (`self.MinHandleRollForDoorOpening`))))

(fn `UserConstructionScript`
  (`SceneComponent.K2_SetRelativeRotation` (`self.Door`) (`KismetMathLibrary.MakeRotator` 0.0 0.0 (* -1 (`self.InitialDoorOpening`))) false true))