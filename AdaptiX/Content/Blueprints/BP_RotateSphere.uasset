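; BP_RotateSphere is a small sphere that follows the BP_D435 RGB camera outside replays and indicates its angular sector around a reference point.
; Each tick it copies the camera's location and computes the angle around Origin, offset by half StepLength.
; "Color" is set by rotating the mesh, either in four discrete sectors (red, blue, green, black) or blended continuously.
; Space resets Origin to the sphere's current location.
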(event `self.ReceiveBeginPlay`
  (bind _recording (`self.RunningReplay`))
  (if (not _recording)
    (bind _outactors (`GameplayStatics.GetAllActorsOfClass` "/Game/Blueprints/BP_JacoArm/BP_D435.BP_D435_C"))
    (set `self.Camera` (`|GetArrayItem` _outactors))
    (`self.EnableInput` (`GameplayStatics.GetPlayerController` 0))))

(event `self.ReceiveTick`
  (params (DeltaSeconds :type "Float (single-precision)"))
  (bind _recording (`self.RunningReplay`))
  (if (not _recording)
    (`SceneComponent.K2_SetWorldLocation` (`self.StaticMeshComponent`) (`SceneComponent.K2_GetComponentLocation` (`/Game/Blueprints/BP_JacoArm/BP_D435.RGB_Cam` (`self.Camera`))) false true)
    (`self.SetColorBasedOnPosition`)))

(event `Key|SpaceBar`
  (params (Key :type "Key Structure"))
  ;[1 1 1] Press Space to set new Origin
  (:`Pressed`
    (bind _output_get (set `self.Origin` (`SceneComponent.K2_GetComponentLocation` (`self.StaticMeshComponent`))))
    (`KismetSystemLibrary.PrintString` (`KismetStringLibrary.Concat_StrStr` "New Origin Set at " (`KismetStringLibrary.Conv_VectorToString` _output_get)))))

(fn `GetAngle`
  (returns (ReturnValue :type "Float (double-precision)"))
  (bind _steplength (`self.StepLength`))
  (bind (_returnvalue_x _returnvalue_y) (`KismetMathLibrary.BreakVector` (- (`SceneComponent.K2_GetComponentLocation` (`self.StaticMeshComponent`)) (+ (`self.Origin`) (`KismetMathLibrary.MakeVector` (* _steplength 0.5) (* _steplength -0.5))))))
  (return (`KismetMathLibrary.DegAtan2` _returnvalue_x _returnvalue_y)))

(fn `RunningReplay`
  (returns (Recording :type Boolean))
  (bind _asbp_gm_storage (cast `/Game/Blueprints/BP_JacoArm/BP_GM_Storage` (`GameplayStatics.GetGameMode`))
    (:`then`
      (return (`/Game/Blueprints/BP_JacoArm/BP_GM_Storage.ReplayRunning` _asbp_gm_storage)))
    (:`CastFailed`
      (return false))))

(fn `SetColor`
  (params (Color :type "Vector Structure"))
  (bind _staticmeshcomponent (`self.StaticMeshComponent`))
  (`SceneComponent.K2_SetWorldRotation` _staticmeshcomponent (`KismetMathLibrary.MakeRotator` Color_X Color_Y Color_Z) false true)
  (`SceneComponent.SetWorldScale3D` _staticmeshcomponent (0.05 0.05 0.05)))

(fn `SetColorBasedOnPosition`
  (bind _returnvalue (`self.GetAngle`))
  (bind _returnvalue_2 (`self.GetAngle`))
  (bind _returnvalue_3 (>= _returnvalue 90.0))
  (bind _returnvalue_4 (>= _returnvalue_2 -45.0))
  (bind _returnvalue_5 (>= _returnvalue_2 45.0))
  (bind _returnvalue_6 (>= _returnvalue_2 135.0))
  (bind _returnvalue_7 (<= _returnvalue_2 -135.0))
  (if (`self.DiscreteColors`)
    (if (and _returnvalue_4 (not _returnvalue_5))
      (`self.SetColor` (0.0 -90.0 0.0)) ; Red
      (elif (and _returnvalue_5 (not _returnvalue_6))
        (`self.SetColor` (0.0 0.0 0.0)) ; Blau
        (elif (or _returnvalue_6 _returnvalue_7)
          (`self.SetColor` (90.0 0.0 0.0)) ; Grün
          (elif (and (not _returnvalue_7) (not _returnvalue_4))
            (`self.SetColor` (-90.0 0.0 0.0)) ; Schwarz
            (else
              (`self.SetColor` (0.0 45.0 245.0)) ; Eierschale
              (`KismetSystemLibrary.PrintString` "Unknown Region!" true true (struct :`R` 1.0 :`A` 1.0)))))))
    (elif (and (>= _returnvalue 0.0) (not _returnvalue_3))
      (`self.SetColor` (`KismetMathLibrary.MakeVector` 0.0 (+ -90.0 _returnvalue))) ; Red (-90) to Blue(0), 0<= angle <= 90
      (elif _returnvalue_3
        (`self.SetColor` (`KismetMathLibrary.MakeVector` (+ _returnvalue -90.0))) ; Blue (0) to Green (90), 90 <angle <=180
        (elif (<= _returnvalue -90.0)
          (`self.SetColor` (`KismetMathLibrary.MakeVector` (+ 270.0 _returnvalue))) ; Green (90) to Black(180)  -180<=angle<=-90
          (else
            (`self.SetColor` (`KismetMathLibrary.MakeVector` 0.0 (+ _returnvalue -90.0))) ; Black (-180) to Red(-90)  -90<=angles <=0
          ))))))

(fn `UserConstructionScript`)