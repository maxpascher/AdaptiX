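; Blue care cup prop that accepts a loose lid and becomes a single cup-with-lid actor.
; Each Tick scans actors overlapping its Sphere for a static mesh matching LidProxy's mesh, then snaps it to the Lid socket, keeping its yaw.
; The lid loses physics and collision, while LidProxy takes its transform and material and enables collision in its place.
; Tick then switches off, so only one lid attaches.
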(event `self.ReceiveTick`
  (params (DeltaSeconds :type "Float (single-precision)"))
  (bind _lid_proxy (`self.Lid_Proxy`))
  (for _array_element (`PrimitiveComponent.GetOverlappingActors` (`self.Sphere`) null)
    (bind _asstatic_mesh_actor (cast `StaticMeshActor` _array_element))
    ;[1 1 1] Only add Lid if the static mesh aligns with the one stored in the proxy
    (if (and (== (`self.GetAttachParentActor` _asstatic_mesh_actor) null) (== (`StaticMeshComponent.StaticMesh` (`StaticMeshActor.StaticMeshComponent` _asstatic_mesh_actor)) (`StaticMeshComponent.StaticMesh` (`self.Lid_Proxy`))))
      ;[1 1 1] Snap Lid to Socket, but keeping the yaw rotation
      (`self.K2_AttachToActor` _asstatic_mesh_actor self "Lid" "SnapToTarget" "KeepWorld" "SnapToTarget" true)
      (`self.K2_SetActorRelativeRotation` _asstatic_mesh_actor (`KismetMathLibrary.MakeRotator` 0.0 0.0 (.yaw (.rotation (`SceneComponent.GetRelativeTransform` (`Actor.RootComponent` _asstatic_mesh_actor))))) false false)
      (bind _staticmeshcomponent (`StaticMeshActor.StaticMeshComponent` _asstatic_mesh_actor))
      ;[1 1 1] Disable Lid Actor
      (`PrimitiveComponent.SetSimulatePhysics` _staticmeshcomponent false)
      (`PrimitiveComponent.SetCollisionEnabled` _staticmeshcomponent "NoCollision")
      ;[1 1 1] Enable Lid Proxy to let the Cup with Lid be a complete Actor
      (`SceneComponent.K2_SetRelativeTransform` _lid_proxy (`SceneComponent.GetRelativeTransform` _staticmeshcomponent) false true)
      (`PrimitiveComponent.SetCollisionEnabled` _lid_proxy "QueryAndPhysics")
      (`PrimitiveComponent.SetMaterial` _lid_proxy 0 (`PrimitiveComponent.GetMaterial` _staticmeshcomponent 0))
      ;[1 1 1] Disable Tick of this actor
      (`self.SetActorTickEnabled` false)
      (break))))

(fn `UserConstructionScript`)