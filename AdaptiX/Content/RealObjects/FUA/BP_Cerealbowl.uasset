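; BP_Cerealbowl is a cereal bowl that fills itself with loose, physics-driven cereal pieces tagged as Food.
; The construction script adds one StaticMeshActor child actor component per NumCerealsInReservoir, using the SM_Cereal mesh.
; Each piece gets a random-hue Color material parameter at fixed saturation and value, and is movable with physics simulation and overlap events enabled.
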(fn `UserConstructionScript`
  (for _ (range 1 (+ (`self.NumCerealsInReservoir`) 1))
    (bind _returnvalue (`AddComponent|NODE_AddChildActorComponent-1`))
    (`ChildActorComponent.SetChildActorClass` _returnvalue "/Script/Engine.StaticMeshActor")
    (bind _childactor (`ChildActorComponent.ChildActor` _returnvalue))
    (set `Actor.Tags` (`|MakeArray` "Food" :!type "Name") _childactor)
    (bind _asstatic_mesh_actor (cast `StaticMeshActor` _childactor))
    (bind _staticmeshcomponent (`StaticMeshActor.StaticMeshComponent` _asstatic_mesh_actor))
    (`StaticMeshComponent.SetStaticMesh` _staticmeshcomponent "/Game/RealObjects/FUA/resources/SM_Cereal.SM_Cereal")
    (`MeshComponent.SetVectorParameterValueOnMaterials` _staticmeshcomponent "Color" (`KismetMathLibrary.Conv_LinearColorToVector` (`KismetMathLibrary.HSVToRGB` (* 360 (`KismetMathLibrary.RandomFloat`)) 0.8 0.5)))
    (`SceneComponent.SetMobility` _staticmeshcomponent "Movable")
    (`PrimitiveComponent.SetSimulatePhysics` _staticmeshcomponent true)
    (set `PrimitiveComponent.bGenerateOverlapEvents` true _staticmeshcomponent)))